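; Parent sound trigger that plays a configurable sound when the first-person player character overlaps its box.
; An optional prerequisite task gates playback by checking its row name against completed tasks in the player's task list widget.
; Playback is either 2D or through the Audio component configured at BeginPlay, optionally only once.
; Each play sets HasPlayed and calls SoundPlayed, an empty event hook.
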(event OnComponentBeginOverlap(BoxTrigger)
  (params (OverlappedComponent :type Primitive%20Component%20Object%20Reference) (OtherActor :type Actor%20Object%20Reference) (OtherComp :type Primitive%20Component%20Object%20Reference) (OtherBodyIndex :type Integer) (bFromSweep :type Boolean) (SweepResult :type Hit%20Result%20Structure%20%28by%20ref%29))
  (bind _asbp_first_person_character (Utilities|Casting|CastToBP_FirstPersonCharacter OtherActor))
  (bind _prerequisitetask (Variables|Default|GetPrerequisiteTask)
    (:then
      (if (Utilities|Array|ContainsItem (Variables|/Game/TaskSystem/WBP_TaskList.WBP_TaskList_C|GetCompletedTasks (Variables|/Game/FirstPerson/Blueprints/BP_FirstPersonCharacter.BP_FirstPersonCharacter_C|GetWBP_TaskList _asbp_first_person_character)) (.TaskRowName (Utilities|GetClassDefaults _prerequisitetask)))
        (Variables|Default|SetHasCompletedTask? true)
        (if (Variables|Default|GetPlayOnce?) :!label _label
          (if (not (Variables|Default|GetHasPlayed?))
            (if (Variables|Default|Get2DSound?)
              (Audio|PlaySound2D (Variables|Default|GetSoundToPlay) (Variables|Default|GetVolumeMultiplier) (Variables|Default|GetPitchMultiplier) 0.0 0 0)
              (Variables|Default|SetHasPlayed? true)
              (CallFunction|SoundPlayed)
              (else
                (Audio|Components|Audio|Play (Variables|Default|GetAudio) 0.0)
                (Variables|Default|SetHasPlayed? true)
                (CallFunction|SoundPlayed))))
          (elif (Variables|Default|Get2DSound?)
            (Audio|PlaySound2D (Variables|Default|GetSoundToPlay) (Variables|Default|GetVolumeMultiplier) (Variables|Default|GetPitchMultiplier) 0.0 0 0)
            (Variables|Default|SetHasPlayed? true)
            (CallFunction|SoundPlayed)
            (else
              (Audio|Components|Audio|Play (Variables|Default|GetAudio) 0.0)
              (Variables|Default|SetHasPlayed? true)
              (CallFunction|SoundPlayed))))))
    (:else
      (goto _label))))

(event Custom|SoundPlayed)

(event EventBeginPlay
  (bind _audio (Variables|Default|GetAudio))
  (Audio|Components|Audio|SetSound (Variables|Default|GetAudio) (Variables|Default|GetSoundToPlay))
  (Audio|Components|Audio|SetVolumeMultiplier _audio (Variables|Default|GetVolumeMultiplier) :!class /Script/Engine.AudioComponent)
  (Audio|Components|Audio|SetPitchMultiplier _audio (Variables|Default|GetPitchMultiplier)))

(fn ConstructionScript)