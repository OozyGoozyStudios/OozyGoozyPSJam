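; Base interactable Blueprint for objects the first-person player uses or picks up to advance task-list objectives.
; Overlapping the player capsule flags proximity and, if the associated task is listed, reveals a construction-script duplicate mesh carrying an outline material.
; Interacted checks that task and any required or consumable equipped item, showing a prompt if missing.
; Success plays sound, increments or completes the task, and can add pickups to player equipment.
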(event OnComponentBeginOverlap(OverlapBox)
  (params (OverlappedComponent :type Primitive%20Component%20Object%20Reference) (OtherActor :type Actor%20Object%20Reference) (OtherComp :type Primitive%20Component%20Object%20Reference) (OtherBodyIndex :type Integer) (bFromSweep :type Boolean) (SweepResult :type Hit%20Result%20Structure%20%28by%20ref%29))
  (if (not (Variables|Default|GetHasBeenInteracted?))
    (bind _asbp_first_person_character (Utilities|Casting|CastToBP_FirstPersonCharacter OtherActor))
    (if (== OtherComp (Variables|/Script/Engine.Character|GetCapsuleComponent _asbp_first_person_character))
      (Variables|/Game/FirstPerson/Blueprints/BP_FirstPersonCharacter.BP_FirstPersonCharacter_C|SetNearInteractable? _asbp_first_person_character true)
      (bind _hastask_ (CallFunction|EnsureHasTask))
      (if _hastask_
        (CallFunction|ChangeStencilVisibility true)))))

(event OnComponentEndOverlap(OverlapBox)
  (params (OverlappedComponent :type Primitive%20Component%20Object%20Reference) (OtherActor :type Actor%20Object%20Reference) (OtherComp :type Primitive%20Component%20Object%20Reference) (OtherBodyIndex :type Integer))
  (bind _asbp_first_person_character (Utilities|Casting|CastToBP_FirstPersonCharacter OtherActor))
  (if (== OtherComp (Variables|/Script/Engine.Character|GetCapsuleComponent _asbp_first_person_character))
    (Variables|/Game/FirstPerson/Blueprints/BP_FirstPersonCharacter.BP_FirstPersonCharacter_C|SetNearInteractable? _asbp_first_person_character false)
    (Default|RemoveInteractionWidget _asbp_first_person_character)
    (CallFunction|ChangeStencilVisibility false)))

(event Custom|Interacted
  (bind _hastask_ (CallFunction|EnsureHasTask))
  (if _hastask_
    (if (Variables|Default|GetRequiresObject?)
      (if (Variables|Default|GetConsumesObject?)
        (if (Variables|Default|GetUnlocked?)
          (CallFunction|PlayInteractedSound)
          (else
            (bind (_isholdingconsumable_ _playercharacter _equipmenttoremove) (CallFunction|CheckPlayerHoldingConsumable))
            (if _isholdingconsumable_
              (Default|RemoveEquipment _playercharacter _equipmenttoremove)
              (CallFunction|EquipmentConsumed)
              (CallFunction|TaskUpdated)
              (CallFunction|PlayInteractedSound)
              (elif (not (Variables|Default|GetUnlocked?))
                (CallFunction|MissingConsumable)))))
        (else
          (bind _isholdingrequired_ (CallFunction|CheckPlayerHoldingRequired))
          (if _isholdingrequired_
            (CallFunction|TaskUpdated)
            (CallFunction|PlayInteractedSound)
            (if (Variables|Default|GetIsPickup?)
              (CallFunction|GetPickedUp))
            (else
              (CallFunction|MissingConsumable)))))
      (else
        (CallFunction|PlayInteractedSound)
        (if (not (Variables|Default|GetCompleted?))
          (Variables|Default|SetHasBeenInteracted? true)
          (CallFunction|TaskUpdated)
          (if (Variables|Default|GetIsPickup?)
            (CallFunction|GetPickedUp)))))))

(event Custom|GetPickedUp
  (bind _defaultsceneroot (Variables|Default|GetDefaultSceneRoot))
  ;[1 1 1] Picks up interactable, adds it to character equipment array, and removes it from level
  (Collision|SetCollisionEnabled (Variables|Default|GetInteractableMesh) "NoCollision")
  (bind _asbp_first_person_character (Utilities|Casting|CastToBP_FirstPersonCharacter (Game|GetPlayerCharacter 0)))
  (Default|AddEquipment _asbp_first_person_character (Variables|Default|GetPickupRef))
  (if (Variables|Default|GetPickUpWholeObject?)
    (Components|MoveComponentTo _defaultsceneroot (- (Transformation|GetWorldLocation (Variables|/Script/Engine.Character|GetCapsuleComponent _asbp_first_person_character)) (Transformation|GetWorldLocation _defaultsceneroot)) "0, 0, 0" false true 2.0 false)
    (Actor|DestroyActor self)))

(event Custom|TaskUpdated
  (bind _associatedtask (Variables|Default|GetAssociatedTask))
  ;[1 1 1] Completes Task from Task List (AssociatedTask must be set in Class Defaults)
  (if (Utilities|IsValidClass _associatedtask)
    (if (.IsIncrementalTask? (Utilities|GetClassDefaults _associatedtask))
      (bind _asbp_first_person_character (Utilities|Casting|CastToBP_FirstPersonCharacter (Game|GetPlayerCharacter 0)))
      (Default|IncrementTask (Variables|/Game/FirstPerson/Blueprints/BP_FirstPersonCharacter.BP_FirstPersonCharacter_C|GetWBP_TaskList _asbp_first_person_character) (Variables|Default|GetAssociatedTask))
      (else
        (Variables|Default|SetCompleted? true)
        (bind _asbp_first_person_character_2 (Utilities|Casting|CastToBP_FirstPersonCharacter (Game|GetPlayerCharacter 0)))
        (Default|CompleteTask (Variables|/Game/FirstPerson/Blueprints/BP_FirstPersonCharacter.BP_FirstPersonCharacter_C|GetWBP_TaskList _asbp_first_person_character_2) (Variables|Default|GetAssociatedTask))))))

(event Custom|EquipmentConsumed)

(fn ConstructionScript
  (bind _interactablemesh (Variables|Default|GetInteractableMesh))
  (if (or (Variables|Default|GetIsPickup?) (Variables|Default|GetStencilOverride?))
    (bind _returnvalue (AddComponent|AddStaticMeshComponent false (Transformation|GetRelativeTransform _interactablemesh)))
    (bind _output_get (Variables|Default|SetStencilMesh _returnvalue))
    (Components|StaticMesh|SetStaticMesh _output_get (Variables|/Script/Engine.StaticMeshComponent|GetStaticMesh _interactablemesh))
    (for (_ _array_index) (Rendering|Material|GetMaterials (Variables|Default|GetStencilMesh))
      (Rendering|Material|SetMaterial (Variables|Default|GetStencilMesh) _array_index "/Game/Interactables/MI_InteractableOutline.MI_InteractableOutline")
      (Rendering|SetVisibility _output_get false false))))

(fn CheckPlayerHoldingConsumable
  (bind _asbp_first_person_character (Utilities|Casting|CastToBP_FirstPersonCharacter (Game|GetPlayerCharacter 0)))
  (return (== (Utilities|GetClass (Variables|/Game/FirstPerson/Blueprints/BP_FirstPersonCharacter.BP_FirstPersonCharacter_C|GetCurrentlyEquippedItem _asbp_first_person_character)) (Variables|Default|GetObjectRequired)) _asbp_first_person_character (Variables|/Game/FirstPerson/Blueprints/BP_FirstPersonCharacter.BP_FirstPersonCharacter_C|GetCurrentlyEquippedItem _asbp_first_person_character)))

(fn PlayInteractedSound
  (Audio|PlaySoundatLocation (Variables|Default|GetInteractedSound) (Transformation|GetWorldLocation (Variables|Default|GetDefaultSceneRoot)) "0, 0, 0" 1.0 1.0 0.0 0 0 0 0)
  (if (Variables|Default|GetAddAltSound?)
    (bind _altinteractedsound (Variables|Default|GetAltInteractedSound)
      (:then
        (Audio|PlaySound2D _altinteractedsound 1.0 1.0 0.0 0 0))
      (:else))))

(fn MissingConsumable
  (bind _asbp_first_person_character (Utilities|Casting|CastToBP_FirstPersonCharacter (Game|GetPlayerCharacter 0)))
  (Default|CreateMissingConsumableWidget _asbp_first_person_character (Variables|Default|GetMissingObjectPrompt)))

(fn EnsureHasTask
  (LocalVariables|SetHasTask false)
  (Variables|Default|GetAssociatedTask
    (:then
      (bind _asbp_first_person_character (Utilities|Casting|CastToBP_FirstPersonCharacter (Game|GetPlayerCharacter 0)))
      (for _array_element (Variables|/Game/TaskSystem/WBP_TaskList.WBP_TaskList_C|GetTaskList (Variables|/Game/FirstPerson/Blueprints/BP_FirstPersonCharacter.BP_FirstPersonCharacter_C|GetWBP_TaskList _asbp_first_person_character))
        (if (== (Utilities|GetClass _array_element) (Variables|Default|GetAssociatedTask))
          (LocalVariables|SetHasTask true)))
      (return (LocalVariables|GetHasTask)))
    (:else
      (return true))))

(fn CheckPlayerHoldingRequired
  (bind _asbp_first_person_character (Utilities|Casting|CastToBP_FirstPersonCharacter (Game|GetPlayerCharacter 0)))
  (return (== (Utilities|GetClass (Variables|/Game/FirstPerson/Blueprints/BP_FirstPersonCharacter.BP_FirstPersonCharacter_C|GetCurrentlyEquippedItem _asbp_first_person_character)) (Variables|Default|GetObjectRequired)) _asbp_first_person_character))

(fn ChangeStencilVisibility
  (params (Visible? :type Boolean))
  (bind _stencilmesh (Variables|Default|GetStencilMesh)
    (:then
      (Rendering|SetVisibility _stencilmesh Visible? false))
    (:else)))