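; Coal pile interactable that runs the parent's interaction logic and plays a shoveling sound at its mesh when used.
; Assigning a new task clears its completed and interacted flags and refills the pickup quantity.
; A pickup path marked deprecated, still called on equipment consumption, decrements quantity, gives the player equipment, marks the pile interacted when empty, and can move and destroy it.
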(event Custom|SetNewAssociatedTask
  (params (NewTask :type WBP%20Individual%20Task%20Class%20Reference))
  (Variables|Default|SetAssociatedTask NewTask)
  (Variables|Default|SetCompleted? false)
  (Variables|Default|SetHasBeenInteracted? false)
  (Variables|Default|SetPickupQuantity 3))

(event EventBeginPlay)

(event Collision|EventActorBeginOverlap
  (params (OtherActor :type Actor%20Object%20Reference)))

(event EventTick
  (params (DeltaSeconds :type Float%20%28single-precision%29)))

(event EventGetPickedUp
  (bind _defaultsceneroot (Variables|Default|GetDefaultSceneRoot))
  ;[1 1 1] Deprecated (Coal is no longer an equipment pickup)
  (if (> (Variables|Default|GetPickupQuantity) 0)
    (bind _output_get (Variables|Default|SetPickupQuantity (- (Variables|Default|GetPickupQuantity) 1)))
    (if (> _output_get 0)
      _
      (else
        (Variables|Default|SetHasBeenInteracted? true)))
    (bind _asbp_first_person_character (Utilities|Casting|CastTo (Game|GetPlayerCharacter 0)))
    (CallFunction|AddEquipment _asbp_first_person_character (Variables|Default|GetPickupRef))
    (if (Variables|Default|GetPickUpWholeObject?)
      (Components|MoveComponentTo _defaultsceneroot (- (Transformation|GetWorldLocation (Variables|/Script/Engine.Character|GetCapsuleComponent _asbp_first_person_character)) (Transformation|GetWorldLocation _defaultsceneroot)) "0, 0, 0" false true 2.0 false)
      (Actor|DestroyActor self))))

(event EventInteracted
  (|CallParentFunction)
  (Audio|PlaySoundatLocation "/Game/Sounds/Pickup_SFX/S_shoveling_coal_B_Cue.S_shoveling_coal_B_Cue" (Transformation|GetWorldLocation (Variables|Default|GetInteractableMesh)) "0, 0, 0" 1.0 1.0 0.0 0 0 0 0))

(event EventEquipmentConsumed
  (CallFunction|GetPickedUp))

(fn ConstructionScript
  (|CallParentFunction))