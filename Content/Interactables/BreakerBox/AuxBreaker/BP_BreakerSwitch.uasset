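; BP_BreakerSwitch is an interactable, color-named breaker switch from the auxiliary breaker box.
; Interacting toggles SwitchOn, broadcasts the new state through the Flipped dispatcher, and plays a switch sound pitched slightly lower when off.
; The construction script builds the interaction prompt from BreakerColorName, and TaskComplete sets HasBeenInteracted.
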(event Custom|TaskComplete
  (Variables|Default|SetHasBeenInteracted? true))

(event EventBeginPlay)

(event Collision|EventActorBeginOverlap
  (params (OtherActor :type Actor%20Object%20Reference)))

(event EventTick
  (params (DeltaSeconds :type Float%20%28single-precision%29)))

(event EventInteracted
  (bind _output_get (Variables|Default|SetSwitchOn? (not (Variables|Default|GetSwitchOn?))))
  (Default|CallFlipped _output_get)
  (Audio|PlaySoundatLocation "/Game/Sounds/S_breaker_switch.S_breaker_switch" (Transformation|GetWorldLocation (Variables|Default|GetDefaultSceneRoot)) "0, 0, 0" 1.0 (Math|Float|SelectFloat 1.0 0.9 (Variables|Default|GetSwitchOn?)) 0.0 0 0 0 0))

(fn ConstructionScript
  (|CallParentFunction)
  (Variables|Default|SetInteractionPrompt (Utilities|Text|ToText(String) (Utilities|String|Append "Flip " (Utilities|String|ToString(Name) (Variables|Default|GetBreakerColorName)) " Switch"))))