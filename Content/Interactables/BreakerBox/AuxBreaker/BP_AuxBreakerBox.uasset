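; Auxiliary breaker box puzzle with four colored switches and an insertable fuse.
; On BeginPlay it binds to the Flipped events of its child-actor switches, each of which rotates a mesh bone and rechecks the combination.
; Red, yellow and blue on with black off completes every switch task, calls TaskUpdated and hides the stencil mesh.
; The fuse holder's event sets FuseInstalled and shows the fuse, independently of the switch check.
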(event EventBeginPlay
  (bind _breakerboxmesh (Variables|Default|GetBreakerBoxMesh))
  (bind _offrotation (Variables|Default|GetOffRotation))
  (Utilities|FlowControl|Sequence
    (:then_0
      ;[1 1 1] Set All Switches To Off
      (Components|PoseableMesh|SetBoneRotationbyName _breakerboxmesh "Switch_1" _offrotation "WorldSpace")
      (Components|PoseableMesh|SetBoneRotationbyName _breakerboxmesh "Switch_2" _offrotation "WorldSpace")
      (Components|PoseableMesh|SetBoneRotationbyName _breakerboxmesh "Switch_3" _offrotation "WorldSpace")
      (Components|PoseableMesh|SetBoneRotationbyName _breakerboxmesh "Switch_4" _offrotation "WorldSpace"))
    (:then_1
      (|BindSwitchFlippedEvents :!label _label))
    (:then_2
      (goto _label execute2))
    (:then_3
      (goto _label execute3))
    (:then_4
      (goto _label execute4))
    (:then_5
      (|BindFuseHolderEvents))))

(fn ConstructionScript
  (|CallParentFunction)
  (Rendering|SetVisibility (Variables|Default|GetFuse) (Variables|Default|GetFuseInstalled?) false))

(fn BlueFlipped
  (params (SwitchOn? :type Boolean))
  (Variables|Default|SetBlueOn? SwitchOn?)
  (Components|PoseableMesh|SetBoneRotationbyName (Variables|Default|GetBreakerBoxMesh) "Switch_3" (Math|Rotator|SelectRotator (Variables|Default|GetOnRotation) (Variables|Default|GetOffRotation) SwitchOn?) "WorldSpace")
  (CallFunction|CheckSwitchCompliance))

(fn YellowFlipped
  (params (SwitchOn? :type Boolean))
  (Variables|Default|SetYellowOn? SwitchOn?)
  (Components|PoseableMesh|SetBoneRotationbyName (Variables|Default|GetBreakerBoxMesh) "Switch_4" (Math|Rotator|SelectRotator (Variables|Default|GetOnRotation) (Variables|Default|GetOffRotation) SwitchOn?) "WorldSpace")
  (CallFunction|CheckSwitchCompliance))

(fn BlackFlipped
  (params (SwitchOn? :type Boolean))
  (Variables|Default|SetBlackOn? SwitchOn?)
  (Components|PoseableMesh|SetBoneRotationbyName (Variables|Default|GetBreakerBoxMesh) "Switch_2" (Math|Rotator|SelectRotator (Variables|Default|GetOnRotation) (Variables|Default|GetOffRotation) SwitchOn?) "WorldSpace")
  (CallFunction|CheckSwitchCompliance))

(fn RedFlipped
  (params (SwitchOn? :type Boolean))
  (Variables|Default|SetRedOn? SwitchOn?)
  (Components|PoseableMesh|SetBoneRotationbyName (Variables|Default|GetBreakerBoxMesh) "Switch_1" (Math|Rotator|SelectRotator (Variables|Default|GetOnRotation) (Variables|Default|GetOffRotation) SwitchOn?) "WorldSpace")
  (CallFunction|CheckSwitchCompliance))

(fn CheckSwitchCompliance
  (if (Math|Boolean|ANDBoolean (Variables|Default|GetRedOn?) (not (Variables|Default|GetBlackOn?)) (Variables|Default|GetYellowOn?) (Variables|Default|GetBlueOn?))
    (Default|TaskComplete (Variables|Default|GetBlue))
    (Default|TaskComplete (Variables|Default|GetYellow))
    (Default|TaskComplete (Variables|Default|GetRed))
    (Default|TaskComplete (Variables|Default|GetBlack))
    (CallFunction|TaskUpdated)
    (bind _stencilmesh (Variables|Default|GetStencilMesh)
      (:then
        (Rendering|SetVisibility _stencilmesh false false))
      (:else))))

(event Custom|Red_FlippedEvent
  (params (SwitchOn? :type Boolean))
  (CallFunction|RedFlipped SwitchOn?))

(event Custom|BlueFlipped_Event
  (params (SwitchOn? :type Boolean))
  (CallFunction|BlueFlipped SwitchOn?))

(event Custom|Yellow_FlippedEvent
  (params (SwitchOn? :type Boolean))
  (CallFunction|YellowFlipped SwitchOn?))

(event Custom|Black_FlippedEvent
  (params (SwitchOn? :type Boolean))
  (CallFunction|BlackFlipped SwitchOn?))

(event Custom|FuseInserted_Event
  (Variables|Default|SetFuseInstalled? true)
  (Rendering|SetVisibility (Variables|Default|GetFuse) true false))