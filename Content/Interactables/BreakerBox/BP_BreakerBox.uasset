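; Breaker box interactable that flips its switch and plays the audio sequence for power coming back on.
; On interaction it runs parent logic, plays the switch sound and calls OnState, which rotates the switch and later starts a power ambience.
; It also starts ambience at the BP_Generator found by class lookup, then plays delayed 2D emergency-systems and boss sounds.
; OffState only rotates the switch back.
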(event Custom|OnState
  (Transformation|SetRelativeRotation (Variables|Default|GetBreakerSwitch) (Variables|Default|GetOnInteractedState) false false)
  (Utilities|FlowControl|Delay 3.35)
  (Audio|PlaySoundatLocation "/Game/Sounds/Ambience/S_power_ambience_Cue.S_power_ambience_Cue" (Transformation|GetWorldLocation (Variables|Default|GetInteractableMesh)) "0, 0, 0" 1.0 1.0 0.0 0 0 0 0))

(event Custom|OffState
  (Transformation|SetRelativeRotation (Variables|Default|GetBreakerSwitch) (Variables|Default|GetOffInteractedState) false false))

(event EventBeginPlay)

(event Collision|EventActorBeginOverlap
  (params (OtherActor :type Actor%20Object%20Reference)))

(event EventTick
  (params (DeltaSeconds :type Float%20%28single-precision%29)))

(event EventInteracted
  (|CallParentFunction)
  (Audio|PlaySoundatLocation "/Game/Sounds/S_breaker_switch.S_breaker_switch" (Transformation|GetWorldLocation (Variables|Default|GetInteractableMesh)) "0, 0, 0" 1.0 1.0 0.0 0 0 0 0)
  (CallFunction|OnState)
  (bind _returnvalue (Actor|GetActorOfClass "/Game/Interactables/Generator/BP_Generator.BP_Generator_C"))
  (bind _output_get (Variables|Default|SetGenerator _returnvalue))
  (Audio|PlaySoundatLocation "/Game/Sounds/Ambience/S_generator_ambience_Cue.S_generator_ambience_Cue" (Transformation|GetWorldLocation (Variables|/Game/Interactables/BP_ParentInteractable.BP_ParentInteractable_C|GetInteractableMesh _output_get)) "0, 0, 0" 1.0 1.0 0.0 0 0 0 0)
  (Utilities|FlowControl|Delay 1.0)
  (Audio|PlaySound2D "/Game/Sounds/General_SFX/S_emergency_systems_online.S_emergency_systems_online" 1.0 1.0 0.0 0 0)
  (Utilities|FlowControl|Delay 16.0)
  (Audio|PlaySound2D "/Game/Sounds/VoiceActing/Boss/S_Boss_6.S_Boss_6" 1.0 1.0 0.0 0 0))

(fn ConstructionScript
  (|CallParentFunction))