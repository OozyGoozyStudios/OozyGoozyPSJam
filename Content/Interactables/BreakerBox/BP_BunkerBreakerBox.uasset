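; Interactable bunker breaker box that switches to its on state when used, with switch, emergency-systems and delayed power ambience sounds.
; Interacted runs the parent logic and OnState, which rotates the switch mesh and sets BreakerOn.
; OffState reverses both but is not called here, and ActorLoaded restores the switch rotation from BreakerOn.
; An unconnected chain for playing ambience at BP_Generator never runs.
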(event Custom|OnState
  (Transformation|SetRelativeRotation (Variables|Default|GetBreakerSwitch) (Variables|Default|GetOnInteractedState) false false)
  (Variables|Default|SetBreakerOn? true)
  (Utilities|FlowControl|Delay 3.35)
  (Audio|PlaySoundatLocation "/Game/Sounds/Ambience/S_power_ambience_Cue.S_power_ambience_Cue" (Transformation|GetWorldLocation (Variables|Default|GetInteractableMesh)) "0, 0, 0" 1.0 1.0 0.0 0 0 0 0))

(event Custom|OffState
  (Transformation|SetRelativeRotation (Variables|Default|GetBreakerSwitch) (Variables|Default|GetOffInteractedState) false false)
  (Variables|Default|SetBreakerOn? false))

(event EventBeginPlay)

(event Collision|EventActorBeginOverlap
  (params (OtherActor :type Actor%20Object%20Reference)))

(event EventTick
  (params (DeltaSeconds :type Float%20%28single-precision%29)))

(event EventInteracted
  (|CallParentFunction)
  (Audio|PlaySoundatLocation "/Game/Sounds/S_breaker_switch.S_breaker_switch" (Transformation|GetWorldLocation (Variables|Default|GetInteractableMesh)) "0, 0, 0" 1.0 1.0 0.0 0 0 0 0)
  (CallFunction|OnState)
  (Utilities|FlowControl|Delay 1.0)
  (Audio|PlaySound2D "/Game/Sounds/General_SFX/S_emergency_systems_online.S_emergency_systems_online" 1.0 1.0 0.0 0 0))

(event EventActorLoaded
  (if (Variables|Default|GetBreakerOn?)
    (Transformation|SetRelativeRotation (Variables|Default|GetBreakerSwitch) (Variables|Default|GetOnInteractedState) false false)
    (else
      (Transformation|SetRelativeRotation (Variables|Default|GetBreakerSwitch) (Variables|Default|GetOffInteractedState) false false))))

(fn ConstructionScript
  (|CallParentFunction))