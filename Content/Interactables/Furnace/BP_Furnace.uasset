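; BP_Furnace is an interactable furnace that the player fuels with coal using a shovel.
; Each consumed piece of equipment below the coal limit adds coal and re-arms the interaction.
; Each addition brightens the floor's dynamic-material emissive, and the first three each power on a child-actor light and ease the flame plane to a new position.
; The third coal also removes the empty shovel from the player.
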(event Custom|CoalAdded
  (bind _flameplane (Variables|Default|GetFlamePlane))
  (bind _relativerotation (Variables|/Script/Engine.SceneComponent|GetRelativeRotation _flameplane))
  (bind _output_get (Variables|Default|SetCoalCount (+ (Variables|Default|GetCoalCount) 1)))
  (CallFunction|IncreaseEmissive)
  (switch int _output_get
    (:1
      (CallFunction|TurnonOffLight (Variables|Default|GetLight1) true)
      (CallFunction|GetPickedUp)
      (Components|MoveComponentTo _flameplane (Variables|Default|GetFlameLoc1) _relativerotation true false 1.0 false))
    (:2
      (CallFunction|TurnonOffLight (Variables|Default|GetLight2) true)
      (CallFunction|GetPickedUp)
      (Components|MoveComponentTo _flameplane (Variables|Default|GetFlameLoc2) _relativerotation true false 1.0 false))
    (:3
      (CallFunction|RemoveShovelfromPlayer)
      (CallFunction|TurnonOffLight (Variables|Default|GetLight3) true)
      (Components|MoveComponentTo _flameplane (Variables|Default|GetFlameLoc3) _relativerotation true true 1.0 false))))

(event EventBeginPlay
  (Variables|Default|SetFlameLocStart (Variables|/Script/Engine.SceneComponent|GetRelativeLocation (Variables|Default|GetFlamePlane)))
  (bind _returnvalue (Rendering|Material|CreateDynamicMaterialInstance "/Game/MaterialsTexturesVFX/VFX/Fireball/M_FurnaceFloor_Inst.M_FurnaceFloor_Inst" "None" "None" :!class /Script/Engine.KismetMaterialLibrary))
  (bind _output_get (Variables|Default|SetDMI_FurnaceFloor _returnvalue))
  (Rendering|Material|SetMaterial (Variables|Default|GetInteractableMesh) 1 _output_get)
  (CallFunction|TurnonOffLight (Variables|Default|GetLight1) false)
  (CallFunction|TurnonOffLight (Variables|Default|GetLight2) false)
  (CallFunction|TurnonOffLight (Variables|Default|GetLight3) false))

(event EventInteracted
  (|CallParentFunction)
  (Audio|PlaySoundatLocation "/Game/Sounds/General_SFX/S_fueling_furnace_Cue.S_fueling_furnace_Cue" (Transformation|GetWorldLocation (Variables|Default|GetInteractableMesh)) "0, 0, 0" 1.0 1.0 0.0 0 0 0 0))

(event EventEquipmentConsumed
  (if (< (Variables|Default|GetCoalCount) (Variables|Default|GetMaxCoalNeeded))
    (CallFunction|CoalAdded)
    (Variables|Default|SetHasBeenInteracted? false)
    (else
      (Variables|Default|SetHasBeenInteracted? true))))

(fn ConstructionScript)

(fn IncreaseEmissive
  (bind _output_get (Variables|Default|SetEmissiveMultiplier (+ (Variables|Default|GetEmissiveMultiplier) 0.75)))
  (Rendering|Material|SetScalarParameterValue (Variables|Default|GetDMI_FurnaceFloor) "EmissiveMultiplier" _output_get :!class /Script/Engine.MaterialInstanceDynamic))

(fn TurnonOffLight
  (params (Light :type Child%20Actor%20Component%20Object%20Reference) (PowerOn? :type Boolean))
  (bind _asbp_parent_light (Utilities|Casting|CastToBP_ParentLight (Variables|/Script/Engine.ChildActorComponent|GetChildActor Light)))
  (if PowerOn?
    (Default|Poweron _asbp_parent_light)
    (else
      (Default|PowerOff _asbp_parent_light))))

(fn RemoveShovelfromPlayer
  (bind _asbp_first_person_character (Utilities|Casting|CastToBP_FirstPersonCharacter (Game|GetPlayerCharacter 0)))
  (Default|RemoveEquipmentExternal _asbp_first_person_character "/Game/Interactables/EquipmentPickups/Shovel/BP_EmptyShovelPickup.BP_EmptyShovelPickup_C"))