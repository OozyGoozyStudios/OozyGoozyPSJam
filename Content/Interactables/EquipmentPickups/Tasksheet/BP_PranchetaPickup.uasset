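; Clipboard (prancheta) equipment pickup that shows the player's task list on an in-world widget.
; On BeginPlay it links that widget to the character's TaskManager and HUD task list, then copies in existing Gated tasks.
; Using it disables player movement and eases the clipboard from ItemSocket to PranchetaSocket through a self-retriggering timer interp instead of Tick.
; Ending use eases it back, then restores walking.
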(event EventBeginPlay
  (bind _asbp_first_person_character (Utilities|Casting|CastToBP_FirstPersonCharacter (Game|GetPlayerCharacter 0)))
  (bind _output_get (Variables|Default|SetAs%20BP%20First%20Person%20Character _asbp_first_person_character))
  (Variables|Default|SetWBP_TaskList (Variables|/Game/FirstPerson/Blueprints/BP_FirstPersonCharacter.BP_FirstPersonCharacter_C|GetWBP_TaskList _output_get))
  (Widget|SetVisibility (Variables|/Game/FirstPerson/Blueprints/BP_FirstPersonCharacter.BP_FirstPersonCharacter_C|GetWBP_TaskList _output_get) "Visible")
  (bind _aswbp_prancheta_task_list (Utilities|Casting|CastToWBP_PranchetaTaskList (UserInterface|GetWidget (Variables|Default|GetWBP_PhysicalTasks)))
    (:then
      (Variables|Default|SetAs%20WBP%20Prancheta%20Task%20List _aswbp_prancheta_task_list)
      (Variables|/Game/TaskSystem/WBP_PranchetaTaskList.WBP_PranchetaTaskList_C|SetTaskManagerRef _aswbp_prancheta_task_list (Variables|/Game/FirstPerson/Blueprints/BP_FirstPersonCharacter.BP_FirstPersonCharacter_C|GetTaskManager _output_get))
      (Default|StorePranchetaWidgetRef (Variables|/Game/FirstPerson/Blueprints/BP_FirstPersonCharacter.BP_FirstPersonCharacter_C|GetWBP_TaskList _output_get) _aswbp_prancheta_task_list))
    (:CastFailed
      _))
  (CallFunction|SetRelativeTransforms)
  (CallFunction|AddExistingTaskstoList))

(event Collision|EventActorBeginOverlap
  (params (OtherActor :type Actor%20Object%20Reference))
  (|CallParentFunction OtherActor) ; This node is disabled and will not be called.\nDrag off pins to build functionality.
)

(event EventTick
  (params (DeltaSeconds :type Float%20%28single-precision%29))
  (|CallParentFunction DeltaSeconds) ; This node is disabled and will not be called.\nDrag off pins to build functionality.
)

(event EventUseEquipment
  (Variables|Default|SetBeingUsed? true)
  (Variables|Default|SetCurrentTransform (Transformation|GetActorTransform))
  (Pawn|Components|CharacterMovement|SetMovementMode (Variables|/Script/Engine.Character|GetCharacterMovement (Variables|Default|GetAs%20BP%20First%20Person%20Character)) "MOVE_None" 0)
  (CallFunction|InterpTransform))

(event EventUseEquipmentEnd
  (Variables|Default|SetBeingUsed? false)
  (Variables|Default|SetCurrentTransform (Transformation|GetActorTransform))
  (CallFunction|InterpTransform))

(fn ConstructionScript
  (|CallParentFunction))

(fn SetRelativeTransforms
  (bind _as_bp_first_person_character (Variables|Default|GetAs%20BP%20First%20Person%20Character))
  (bind _mesh (Variables|/Script/Engine.Character|GetMesh _as_bp_first_person_character))
  (Variables|Default|SetUsedTransform (Transformation|GetSocketTransform _mesh "PranchetaSocket" "RTS_World"))
  (Variables|Default|SetItemSocketTransform (Transformation|GetSocketTransform _mesh "ItemSocket" "RTS_World")))

(fn InterpTransform
  (bind _as_bp_first_person_character (Variables|Default|GetAs%20BP%20First%20Person%20Character))
  (bind _tolerance (LocalVariables|GetTolerance))
  (bind _tolerance_2 (LocalVariables|GetTolerance))
  (bind _as_bp_first_person_character_2 (Variables|Default|GetAs%20BP%20First%20Person%20Character))
  (bind _mesh (Variables|/Script/Engine.Character|GetMesh _as_bp_first_person_character_2))
  (bind _mesh_2 (Variables|/Script/Engine.Character|GetMesh _as_bp_first_person_character))
  (bind _returnvalue (Transformation|GetSocketTransform _mesh_2 "ItemSocket" "RTS_World"))
  (bind _returnvalue_2 (Transformation|GetSocketTransform _mesh "PranchetaSocket" "RTS_World"))
  (if (Variables|Default|GetBeingUsed?)
    (if (Class|KismetMathLibrary|NearlyEqualTransformTransform (Variables|Default|GetCurrentTransform) _returnvalue_2 _tolerance_2 _tolerance_2 _tolerance_2)
      (return)
      (else
        (Variables|Default|SetCurrentTransform (Class|KismetMathLibrary|TInterpto (Variables|Default|GetCurrentTransform) _returnvalue_2 (Utilities|Time|GetWorldDeltaSeconds) (LocalVariables|GetInterpSpeed)))
        (Transformation|SetActorTransform (Class|KismetMathLibrary|TInterpto (Variables|Default|GetCurrentTransform) _returnvalue_2 (Utilities|Time|GetWorldDeltaSeconds) (LocalVariables|GetInterpSpeed)))
        (Utilities|Time|SetTimerbyFunctionName 0 "InterpTransform" 0.01)))
    (elif (Class|KismetMathLibrary|NearlyEqualTransformTransform (Variables|Default|GetCurrentTransform) _returnvalue _tolerance _tolerance _tolerance)
      (Pawn|Components|CharacterMovement|SetMovementMode (Variables|/Script/Engine.Character|GetCharacterMovement (Variables|Default|GetAs%20BP%20First%20Person%20Character)) "MOVE_Walking" 0)
      (return)
      (else
        (Variables|Default|SetCurrentTransform (Class|KismetMathLibrary|TInterpto (Variables|Default|GetCurrentTransform) _returnvalue (Utilities|Time|GetWorldDeltaSeconds) (LocalVariables|GetInterpSpeed)))
        (Transformation|SetActorTransform (Class|KismetMathLibrary|TInterpto (Variables|Default|GetCurrentTransform) _returnvalue (Utilities|Time|GetWorldDeltaSeconds) (LocalVariables|GetInterpSpeed)))
        (Utilities|Time|SetTimerbyFunctionName 0 "InterpTransform" 0.01)))))

(fn Equipped
  (|CallParentFunction)
  (Transformation|SetActorTransform (Transformation|GetSocketTransform (Variables|/Script/Engine.Character|GetMesh (Variables|Default|GetAs%20BP%20First%20Person%20Character)) "ItemSocket" "RTS_World")))

(fn Unequipped
  (|CallParentFunction)
  (Transformation|SetActorTransform (Transformation|GetSocketTransform (Variables|/Script/Engine.Character|GetMesh (Variables|Default|GetAs%20BP%20First%20Person%20Character)) "ItemSocket" "RTS_World"))
  (Pawn|Components|CharacterMovement|SetMovementMode (Variables|/Script/Engine.Character|GetCharacterMovement (Variables|Default|GetAs%20BP%20First%20Person%20Character)) "MOVE_Walking" 0))

(fn CreateTutorialWidget
  (Variables|Default|GetTutorialWidget
    (:then)
    (:else
      (bind _returnvalue (UserInterface|CreateWidget "/Game/Interactables/EquipmentPickups/WBP_TutorialWidget.WBP_TutorialWidget_C" 0 "Tab" "View Tasks At Any Time" true true))
      (bind _output_get (Variables|Default|SetTutorialWidget _returnvalue))
      (UserInterface|Viewport|AddtoViewport _output_get 0))))

(fn AddExistingTaskstoList
  (for _array_element (Variables|/Game/TaskSystem/WBP_TaskList.WBP_TaskList_C|GetTaskList (Variables|Default|GetWBP_TaskList))
    (switch Utilities|FlowControl|Switch|SwitchonE_TaskDistinction (Variables|/Game/TaskSystem/WBP_IndividualTask.WBP_IndividualTask_C|GetTaskDistinction _array_element)
      (:NewEnumerator0
        (Default|AddTask (Variables|Default|GetAs%20WBP%20Prancheta%20Task%20List) (Variables|/Game/TaskSystem/WBP_IndividualTask.WBP_IndividualTask_C|GetTaskRowName _array_element))))))