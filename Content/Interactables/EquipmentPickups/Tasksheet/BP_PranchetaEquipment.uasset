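; Clipboard ("prancheta") equipment that shows the task list when used by the player.
; On BeginPlay it caches the first-person player character and sets that character's task list widget visible.
; UseEquipment adds the widget to the viewport if it is not already there, then calls its Used function, leaving the display behavior to the widget.
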(event EventBeginPlay
  (bind _asbp_first_person_character (Utilities|Casting|CastToBP_FirstPersonCharacter (Game|GetPlayerCharacter 0)))
  (bind _output_get (Variables|Default|SetAs%20BP%20First%20Person%20Character _asbp_first_person_character))
  (Widget|SetVisibility (Variables|/Game/FirstPerson/Blueprints/BP_FirstPersonCharacter.BP_FirstPersonCharacter_C|GetWBP_TaskList _output_get) "Visible"))

(event Collision|EventActorBeginOverlap
  (params (OtherActor :type Actor%20Object%20Reference))
  (|CallParentFunction OtherActor) ; This node is disabled and will not be called.\nDrag off pins to build functionality.
)

(event EventTick
  (params (DeltaSeconds :type Float%20%28single-precision%29))
  (|CallParentFunction DeltaSeconds) ; This node is disabled and will not be called.\nDrag off pins to build functionality.
)

(event EventUseEquipment
  (bind _as_bp_first_person_character (Variables|Default|GetAs%20BP%20First%20Person%20Character))
  (bind _wbp_tasklist (Variables|/Game/FirstPerson/Blueprints/BP_FirstPersonCharacter.BP_FirstPersonCharacter_C|GetWBP_TaskList _as_bp_first_person_character))
  (if (UserInterface|Viewport|IsinViewport _wbp_tasklist)
    (Default|Used _wbp_tasklist)
    (else
      (UserInterface|Viewport|AddtoViewport _wbp_tasklist 0)
      (Default|Used _wbp_tasklist))))

(fn ConstructionScript
  (|CallParentFunction))