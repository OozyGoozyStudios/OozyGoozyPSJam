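; Torch equipment pickup that extends a parent light pickup with a spotlight.
; The spotlight starts at zero intensity on BeginPlay, and the SetIntensity override passes the requested intensity to it after calling the parent.
; The ToggleLight override runs the parent logic, then plays a 2D OnSound if LightOn is false.
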(event EventBeginPlay
  (Rendering|Components|Light|SetIntensity (Variables|Default|GetSpotLight) 0.0))

(event Collision|EventActorBeginOverlap
  (params (OtherActor :type Actor%20Object%20Reference))
  (|CallParentFunction OtherActor) ; This node is disabled and will not be called.\nDrag off pins to build functionality.
)

(event EventTick
  (params (DeltaSeconds :type Float%20%28single-precision%29))
  (|CallParentFunction DeltaSeconds) ; This node is disabled and will not be called.\nDrag off pins to build functionality.
)

(fn ConstructionScript
  (|CallParentFunction))

(fn ToggleLight
  (|CallParentFunction)
  (if (not (Variables|Default|GetLightOn?))
    (Audio|PlaySound2D (Variables|Default|GetOnSound) 1.0 0.8 0.0 0 0)))

(fn SetIntensity
  (params (Intensity :type Float%20%28double-precision%29))
  (|CallParentFunction Intensity)
  (Rendering|Components|Light|SetIntensity (Variables|Default|GetSpotLight) Intensity))