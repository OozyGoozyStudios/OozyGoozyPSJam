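; Base equippable flashlight that, while equipped, rotates its root each tick to follow the first-person character's camera pitch and mesh yaw.
; ToggleLight switches between base and zero intensity, and can schedule a delayed tutorial widget before the light's first use.
; A 2D hiss sound plays when lit, fades on switch-off or unequip, and resumes on re-equip.
; SetIntensity and CreateTutorialWidget are empty stubs.
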(event EventBeginPlay
  (bind _returnvalue (Actor|GetActorOfClass "/Game/FirstPerson/Blueprints/BP_FirstPersonCharacter.BP_FirstPersonCharacter_C"))
  (Variables|Default|SetBP_FirstPersonCharacter _returnvalue))

(event EventTick
  (params (DeltaSeconds :type Float%20%28single-precision%29))
  (|CallParentFunction DeltaSeconds)
  (if (Variables|Default|GetEquipped?)
    (bind _bp_firstpersoncharacter (Variables|Default|GetBP_FirstPersonCharacter)
      (:then
        (Transformation|SetWorldRotation (Variables|Default|GetDefaultSceneRoot) (Math|Rotator|MakeRotator (* (.pitch (Transformation|GetWorldRotation (Variables|/Script/PSJamJan.PSJamJanCharacter|GetFirstPersonCameraComponent _bp_firstpersoncharacter))) -1.0) 0.0 (.yaw (Transformation|GetWorldRotation (Variables|/Script/Engine.Character|GetMesh _bp_firstpersoncharacter)))) false false))
      (:else
        (bind _returnvalue (Actor|GetActorOfClass "/Game/FirstPerson/Blueprints/BP_FirstPersonCharacter.BP_FirstPersonCharacter_C"))
        (Variables|Default|SetBP_FirstPersonCharacter _returnvalue)))))

(fn ConstructionScript
  (|CallParentFunction))

(fn ToggleLight
  (if (Variables|Default|GetLightOn?)
    (Variables|Default|SetLightOn? false)
    (CallFunction|SetIntensity 0.0)
    (CallFunction|StopSounds)
    (else
      (if (Variables|Default|GetHasBeenTurnedOn?)
        _
        (elif (Variables|Default|GetHasTutorialWidget?)
          (Variables|Default|GetTutorialWidget
            (:then)
            (:else
              (Utilities|Time|SetTimerbyFunctionName 0 "CreateTutorialWidget" 1.0)))))
      (Variables|Default|SetLightOn? true)
      (Variables|Default|SetCurrentIntensity (Variables|Default|GetBaseIntensity))
      (CallFunction|SetIntensity (Variables|Default|GetCurrentIntensity))
      (CallFunction|PlayonNoise))))

(fn SetIntensity
  (params (Intensity :type Float%20%28double-precision%29)))

(fn StopSounds
  (bind _flashlightonaudio (Variables|Default|GetFlashlightOnAudio)
    (:then
      (Audio|Components|Audio|FadeOut _flashlightonaudio 0.1 0.0 "Linear" :!class /Script/Engine.AudioComponent))
    (:else)))

(fn CreateTutorialWidget)

(fn PlayonNoise
  (bind _flashlightonaudio (Variables|Default|GetFlashlightOnAudio)
    (:then
      (if (Audio|Components|Audio|IsPlaying _flashlightonaudio)
        _
        (else
          (CallFunction|PlayHiss)))
      (Variables|Default|SetHasBeenTurnedOn? true))
    (:else
      (CallFunction|PlayHiss))))

(fn PlayHiss
  (bind _onsound (Variables|Default|GetOnSound)
    (:then
      (bind _returnvalue (Audio|SpawnSound2D _onsound 1.0 1.0 0.0 0))
      (bind _output_get (Variables|Default|SetFlashlightOnAudio _returnvalue))
      (Audio|Components|Audio|Play _output_get 0.0))
    (:else)))

(fn Equipped
  (|CallParentFunction)
  (Variables|Default|SetEquipped? true)
  (if (Variables|Default|GetLightOn?)
    (CallFunction|PlayHiss)))

(fn Unequipped
  (|CallParentFunction)
  (Variables|Default|SetEquipped? false)
  (CallFunction|StopSounds))