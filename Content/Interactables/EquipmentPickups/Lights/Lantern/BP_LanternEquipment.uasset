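; Lantern equipment pickup: a child light whose intensity drains as oil burns, with a hiss whose volume follows brightness.
; While lit, Tick subtracts from intensity and updates the point light, playing an overload sound once below a threshold.
; RefillOil raises intensity through a self-repeating timer, but its call after UseEquipment's checks is unwired and never runs.
; A refuel tutorial widget is created, but its timed removal function is empty.
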(event Custom|TimerEvent)

(event EventBeginPlay
  (CallFunction|IsLighton)
  (CallFunction|PlayHiss)
  (CallFunction|UpdateSoundProperties))

(event EventUseEquipment
  (if (Variables|Default|GetbLightOn?)
    (if (not (Variables|Default|GetbBurningDown?))
      (if (Variables|Default|GetIsFilling?)
        _))))

(event EventTick
  (params (DeltaSeconds :type Float%20%28single-precision%29))
  (if (Math|Boolean|ANDBoolean (> (Variables|Default|GetCurrentIntensity_0) 0.0) (Variables|Default|GetbLightOn?) (not (Utilities|Time|IsTimerActivebyHandle (Variables|Default|GetLightTimerHandle))))
    (bind _returnvalue (Utilities|Time|SetTimerbyEvent (delegate Custom|TimerEvent) (Variables|Default|GetLightTimer) true))
    (bind _output_get (Variables|Default|SetLightTimerHandle _returnvalue))
    (CallFunction|SubtractfromLight)
    (CallFunction|TimerEvent)
    (Utilities|Time|ClearandInvalidateTimerbyHandle _output_get)
    (CallFunction|IsLighton)
    (if (not (Variables|Default|GetIsFilling?))
      (if (< (Variables|Default|GetCurrentIntensity_0) (Variables|Default|GetThresholdIntensity))
        (Variables|Default|SetbBurningDown? false)
        (Utilities|FlowControl|DoOnce true
          (:Completed
            (Audio|PlaySound2D "/Game/Sounds/General_SFX/Lantern/S_lantern_overload.S_lantern_overload" 1.0 1.0 0.0 0 0)))))))

(fn ConstructionScript)

(fn IsLighton
  (bind _currentintensity_0 (Variables|Default|GetCurrentIntensity_0))
  (if (Variables|Default|GetbLightOn?)
    (CallFunction|SetIntensity _currentintensity_0)
    (if (<= _currentintensity_0 0.0)
      (Variables|Default|SetbLightOn? false))
    (else
      (CallFunction|SetIntensity 0.0))))

(fn SubtractfromLight
  (Variables|Default|SetCurrentIntensity_0 (- (Variables|Default|GetCurrentIntensity_0) (Variables|Default|GetDimAmount)))
  (CallFunction|UpdateSoundProperties))

(fn StartStopDimTimer
  (params (TimerHandle :type Timer%20Handle%20Structure))
  (if (Variables|Default|GetbLightOn?)
    (Utilities|Time|UnpauseTimerbyHandle TimerHandle)
    (else
      (Utilities|Time|PauseTimerbyHandle TimerHandle))))

(fn UpdateSoundProperties
  (bind _lanternhiss (Variables|Default|GetLanternHiss)
    (:then
      (Audio|Components|Audio|SetVolumeMultiplier _lanternhiss (Math|Float|MapRangeClamped (Variables|Default|GetCurrentIntensity_0) 0.0 4e+02 0.0 0.7) :!class /Script/Engine.AudioComponent))
    (:else)))

(fn PlayOverload
  (Audio|PlaySoundatLocation "/Game/Sounds/General_SFX/Lantern/S_lantern_overload.S_lantern_overload" (Transformation|GetWorldLocation (Variables|Default|GetLanternGlass)) "0, 0, 0" 3.0 1.0 0.0 0 0 0 0))

(fn RemoveTutorialWidget)

(fn RefillOil
  (if (< (Variables|Default|GetCurrentIntensity_0) (Variables|Default|GetMaxIntensity_0))
    (Variables|Default|SetIsFilling? true)
    (Variables|Default|SetCurrentIntensity_0 (+ (Variables|Default|GetCurrentIntensity_0) (Variables|Default|GetRefuelStepAmount)))
    (Utilities|Time|SetTimerbyFunctionName 0 "RefillOil" 0.02)
    (else
      (Variables|Default|SetIsFilling? false)
      (Variables|Default|SetbBurningDown? true)
      (return))))

(fn SetIntensity
  (params (Intensity :type Float%20%28double-precision%29))
  (|CallParentFunction Intensity)
  (Rendering|Components|Light|SetIntensity (Variables|Default|GetPointLight) Intensity))

(fn ToggleLight
  (|CallParentFunction))

(fn CreateTutorialWidget
  (|CallParentFunction)
  (bind _returnvalue (UserInterface|CreateWidget "/Game/Interactables/EquipmentPickups/Tutorials/WBP_TutorialWidget.WBP_TutorialWidget_C" 0 (Utilities|Array|MakeArray "L" "LeftMouseButton") "Fuel Lantern and Increase Brightness"))
  (Variables|Default|SetTutorialWidget _returnvalue)
  (UserInterface|Viewport|AddtoViewport _returnvalue 0)
  (Utilities|Time|SetTimerbyFunctionName 0 "RemoveTutorialWidget" 5.0))