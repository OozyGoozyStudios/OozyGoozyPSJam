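; TeleLumen equipment pickup: a handheld device that swaps between a flashlight and an anomaly receiver.
; The character's anomaly updates drive a state-colored blinking LED and timer-interpolated screen glitch.
; Using the receiver in range freezes movement and starts tuning through its HUD widget.
; An opened anomaly tints the screen and plays its sound, with an envelope follower pulsing screen emissive, then completes and restores walking.
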(event OnEnvelopeFollowerUpdate(EnvelopeFollowerListener)
  (params (EnvelopeValue :type Float%20%28single-precision%29))
  (Rendering|Material|SetScalarParameterValue (Variables|Screen|GetDMI_TeleLumenScreen) "EmissiveScalar" (+ (* EnvelopeValue 5e+01) 0.05) :!class /Script/Engine.MaterialInstanceDynamic))

(event Custom|AnomalyUpdate_Event
  (params (EnteredAnomaly? :type Boolean) (AnomalyRef :type BP%20Parent%20Audio%20Anomaly%20Object%20Reference))
  (Variables|LED|SetBlinkLED? EnteredAnomaly?)
  (if EnteredAnomaly?
    (Variables|Default|SetCurrentAnomaly AnomalyRef)
    (Variables|Default|SetE_ReceiverState "NewEnumerator1")
    (else
      (Variables|Default|SetCurrentAnomaly 0)
      (Variables|Default|SetE_ReceiverState "NewEnumerator0")))
  (CallFunction|SetLEDColor false)
  (CallFunction|ChangeAlertState (Variables|LED|GetBlinkLED?)))

(event Custom|StartAnomalyEvent
  (Pawn|Components|CharacterMovement|SetMovementMode (Variables|/Script/Engine.Character|GetCharacterMovement (Variables|Default|GetPlayerCharacterRef)) "MOVE_None" 0)
  (Default|AnomalyEnd (Variables|Default|GetAs%20WBP%20Alert%20Triangle))
  (Variables|Default|SetE_ReceiverState "NewEnumerator4")
  (CallFunction|SetLEDColor false)
  (Utilities|FlowControl|Delay 0.5)
  (Default|StartAnomalyEvent (Variables|Default|GetAs%20WBP%20Receiver%20HUD)))

(event Custom|OpenAnomaly
  (bind _currentanomaly (Variables|Default|GetCurrentAnomaly))
  (Variables|Default|SetE_ReceiverState "NewEnumerator2")
  (CallFunction|SetLEDColor false)
  (Variables|LED|SetBlinkLED? false)
  (Variables|LED|SetLEDOn? true)
  (Variables|Default|SetAnomalyOpened? true)
  (Variables|Screen|SetTargetScreenColor (Variables|/Game/LevelPrototyping/Blueprints/AudioAnomalies/BP_ParentAudioAnomaly.BP_ParentAudioAnomaly_C|GetAnomalyColor _currentanomaly))
  (CallFunction|InterpScreenColor)
  (CallFunction|EstablishEnvelopeFollower (Variables|/Game/LevelPrototyping/Blueprints/AudioAnomalies/BP_ParentAudioAnomaly.BP_ParentAudioAnomaly_C|GetSoundToPlay _currentanomaly))
  (Utilities|FlowControl|Delay 0.2)
  (Audio|Components|Audio|Play (Variables|Default|GetAnomalySource) 0.0)
  (Utilities|FlowControl|Delay (Variables|/Game/LevelPrototyping/Blueprints/AudioAnomalies/BP_ParentAudioAnomaly.BP_ParentAudioAnomaly_C|GetSoundLength _currentanomaly))
  (CallFunction|CloseAnomaly))

(event Custom|CloseAnomaly
  (bind _playercharacterref (Variables|Default|GetPlayerCharacterRef))
  (Variables|Default|SetE_ReceiverState "NewEnumerator0")
  (CallFunction|SetLEDColor false)
  (Class|SourceEffectEnvelopeFollowerPreset|UnregisterEnvelopeFollowerListener (Variables|Default|GetEnvFollowerPreset) (Variables|Default|GetEnvelopeFollowerListener))
  (Variables|Default|SetAnomalyOpened? false)
  (Variables|Screen|SetTargetScreenColor (Variables|Screen|GetDefaultScreenColor))
  (CallFunction|InterpScreenColor)
  (Variables|/Game/LevelPrototyping/Blueprints/AudioAnomalies/BP_ParentAudioAnomaly.BP_ParentAudioAnomaly_C|SetHasBeenCompleted? (Variables|Default|GetCurrentAnomaly) true)
  (Default|EndAnomaly _playercharacterref (Variables|Default|GetCurrentAnomaly))
  (Pawn|Components|CharacterMovement|SetMovementMode (Variables|/Script/Engine.Character|GetCharacterMovement _playercharacterref) "MOVE_Walking" 0)
  (Rendering|Material|SetScalarParameterValue (Variables|Screen|GetDMI_TeleLumenScreen) "EmissiveScalar" 0.05 :!class /Script/Engine.MaterialInstanceDynamic)
  (Default|UserPassiveMode (Variables|Default|GetAs%20WBP%20Receiver%20HUD)))

(event EventBeginPlay
  (|CallParentFunction)
  (bind _returnvalue (Actor|GetActorOfClass "/Game/FirstPerson/Blueprints/BP_FirstPersonCharacter.BP_FirstPersonCharacter_C"))
  (Variables|Default|SetPlayerCharacterRef _returnvalue)
  (EventDispatchers|AssignAnomalyUpdate _returnvalue (delegate Custom|AnomalyUpdate_Event))
  (CallFunction|SetFlashlightVar)
  (CallFunction|SetReceiverVar)
  (CallFunction|SetAlertVar)
  (Variables|Default|SetLightOn? false)
  (CallFunction|SetIntensity 0.0)
  (Variables|Default|SetDynamicIntensity (Variables|Default|GetBaseIntensity))
  (Variables|LED|SetCurrentLEDColor (Variables|LED|GetLED_Red))
  (CallFunction|BlinkLED))

(event EventSwapScreen
  (|CallParentFunction)
  (if (not (Variables|Default|GetAnomalyOpened?))
    (if (Variables|Screen|GetCanSwapScreen?)
      (Audio|PlaySound2D "/Game/Sounds/General_SFX/TeleLumen/S_telelumen_screen_switch.S_telelumen_screen_switch" 0.3 1.0 0.0 0 0)
      (switch Utilities|FlowControl|Switch|SwitchonE_TeleLumenMode (Variables|Screen|GetTeleLumenMode)
        (:NewEnumerator0
          (Variables|Screen|SetCanSwapScreen? false)
          (Rendering|SetVisibility (Variables|Default|GetFlashLightScreen) false false)
          (Utilities|FlowControl|Delay 0.25)
          (bind _output_get (Variables|Screen|SetTeleLumenMode "NewEnumerator1"))
          (Default|CallModeChange _output_get)
          (Variables|Screen|SetCanSwapScreen? true))
        (:NewEnumerator1
          (Variables|Screen|SetCanSwapScreen? false)
          (bind _output_get_2 (Variables|Screen|SetTeleLumenMode "NewEnumerator0"))
          (Default|CallModeChange _output_get_2)
          (Utilities|FlowControl|Delay 0.25)
          (Rendering|SetVisibility (Variables|Default|GetFlashLightScreen) (Variables|Default|GetLightOn?) false)
          (Variables|Screen|SetCanSwapScreen? true))))))

(event EventTick
  (params (DeltaSeconds :type Float%20%28single-precision%29))
  (|CallParentFunction DeltaSeconds))

(event EventUseEquipment
  (if (Math|Boolean|ANDBoolean (Utilities|IsValid (Variables|Default|GetCurrentAnomaly)) (Utilities|Enum|Equal(Enum) (Variables|Screen|GetTeleLumenMode) "NewEnumerator1") (Utilities|Enum|Equal(Enum) (Variables|Default|GetE_ReceiverState) "NewEnumerator1"))
    (CallFunction|StartAnomalyEvent)))

(fn ConstructionScript
  (|CallParentFunction)
  (|EstablishDMIs))

(fn Equipped
  (|CallParentFunction)
  (switch Utilities|FlowControl|Switch|SwitchonE_TeleLumenMode (Variables|Screen|GetTeleLumenMode)
    (:NewEnumerator0
      (Rendering|SetVisibility (Variables|Default|GetFlashLightScreen) (Variables|Default|GetLightOn?) false))
    (:NewEnumerator1
      (Rendering|SetVisibility (Variables|Default|GetFlashLightScreen) false false))))

(fn Scrub
  (params (InputValue :type Float%20%28double-precision%29))
  (|CallParentFunction InputValue)
  (switch Utilities|FlowControl|Switch|SwitchonE_TeleLumenMode (Variables|Screen|GetTeleLumenMode)
    (:NewEnumerator0
      (Default|GetScrubbed (Variables|Default|GetAs%20WBP%20Flashlight%20HUD) InputValue))))

(fn SetFlashlightVar
  (bind _spotlight (Variables|Default|GetSpotLight))
  (bind _aswbp_flashlight_hud (Utilities|Casting|CastToWBP_FlashlightHUD (UserInterface|GetWidget (Variables|Default|GetFlashLightScreen)))
    (:then
      (bind _output_get (Variables|Default|SetAs%20WBP%20Flashlight%20HUD _aswbp_flashlight_hud))
      (Variables|/Game/Interactables/EquipmentPickups/Lights/TeleLumen/RadioLight/UI/Flashlight/WBP_FlashlightHUD.WBP_FlashlightHUD_C|SetSpotlightRef _output_get _spotlight)
      (Variables|/Game/Interactables/EquipmentPickups/Lights/TeleLumen/RadioLight/UI/Flashlight/WBP_FlashlightHUD.WBP_FlashlightHUD_C|SetTeleLumenRef _output_get self)
      (Variables|/Game/Interactables/EquipmentPickups/Lights/TeleLumen/RadioLight/UI/Flashlight/WBP_FlashlightHUD.WBP_FlashlightHUD_C|SetDefaultSpotlightIntensity _output_get (Variables|/Script/Engine.LightComponentBase|GetIntensity _spotlight))
      (Variables|/Game/Interactables/EquipmentPickups/Lights/TeleLumen/RadioLight/UI/Flashlight/WBP_FlashlightHUD.WBP_FlashlightHUD_C|SetDefaultAttenuationRadius _output_get (Variables|/Script/Engine.LocalLightComponent|GetAttenuationRadius _spotlight)))
    (:CastFailed
      (Development|PrintString "Failed to Cast to WBP_FlashlightHUD --Event BeginPlay-- BP_TeleLumenPickup"))))

(fn SetAlertVar
  (Variables|Default|GetAs%20WBP%20Alert%20Triangle
    (:then
      _)
    (:else
      (bind _aswbp_alert_triangle (Utilities|Casting|CastToWBP_AlertTriangle (UserInterface|GetWidget (Variables|Default|GetAlertScreen))))
      (Variables|Default|SetAs%20WBP%20Alert%20Triangle _aswbp_alert_triangle)
      (Variables|/Game/Interactables/EquipmentPickups/Lights/TeleLumen/RadioLight/UI/Alert/WBP_AlertTriangle.WBP_AlertTriangle_C|SetTeleLumenRef _aswbp_alert_triangle self)
      (Default|BindtoTeleLumen _aswbp_alert_triangle)))
  (return))

(fn SetReceiverVar
  (bind _aswbp_pulsing_receiver (Utilities|Casting|CastToWBP_PulsingReceiver (UserInterface|GetWidget (Variables|Default|GetReceiverScreen))))
  (Variables|Default|SetAs%20WBP%20Receiver%20HUD _aswbp_pulsing_receiver)
  (Variables|/Game/Interactables/EquipmentPickups/Lights/TeleLumen/RadioLight/UI/Receiver_mk2/WBP_PulsingReceiver.WBP_PulsingReceiver_C|SetTeleLumenRef _aswbp_pulsing_receiver self)
  (Default|TeleLumenRefSet _aswbp_pulsing_receiver))

(fn SetIntensity
  (params (Intensity :type Float%20%28double-precision%29))
  (|CallParentFunction Intensity)
  (if (Variables|Default|GetLightOn?)
    (Rendering|Components|Light|SetIntensity (Variables|Default|GetSpotLight) Intensity)
    (Rendering|SetVisibility (Variables|Default|GetFlashLightScreen) true false)
    (else
      (Rendering|Components|Light|SetIntensity (Variables|Default|GetSpotLight) 0.0)
      (Rendering|SetVisibility (Variables|Default|GetFlashLightScreen) false false))))

(fn ToggleLight
  (switch Utilities|FlowControl|Switch|SwitchonE_TeleLumenMode (Variables|Screen|GetTeleLumenMode)
    (:NewEnumerator0
      (if (Variables|Default|GetLightOn?)
        (Variables|Default|SetLightOn? false)
        (CallFunction|SetIntensity 0.0)
        (CallFunction|StopSounds)
        ;[1 1 1] Play Off Sound
        (Audio|PlaySound2D (Variables|Default|GetOnSound) 1.0 0.8 0.0 0 0)
        (else
          (if (Variables|Default|GetHasBeenTurnedOn?)
            _
            (elif (Variables|Default|GetHasTutorialWidget?)
              (Variables|Default|GetTutorialWidget
                (:then)
                (:else
                  (Utilities|Time|SetTimerbyFunctionName 0 "CreateTutorialWidget" 1.0)))))
          (Variables|Default|SetLightOn? true)
          (Rendering|SetVisibility (Variables|Default|GetFlashLightScreen) (Variables|Default|GetLightOn?) false)
          (CallFunction|SetIntensity (Variables|Default|GetDynamicIntensity))
          (CallFunction|PlayonNoise))))))

(fn SetLEDColor
  (params (OverrideColor? :type Boolean) (ColorOverride :type Linear%20Color%20Structure))
  (if OverrideColor?
    (Rendering|Material|SetVectorParameterValue (Variables|LED|GetDMI_LED) "LightColor" ColorOverride :!class /Script/Engine.MaterialInstanceDynamic)
    (else
      (switch Utilities|FlowControl|Switch|SwitchonE_ReceiverState (Variables|Default|GetE_ReceiverState)
        (:NewEnumerator0
          (Variables|LED|SetCurrentLEDColor (Variables|LED|GetLED_Red)))
        (:NewEnumerator1
          (Variables|LED|SetCurrentLEDColor (Variables|LED|GetLED_Yellow)))
        (:NewEnumerator4
          (Variables|LED|SetCurrentLEDColor (Variables|LED|GetLED_Blue)))
        (:NewEnumerator2
          (Variables|LED|SetCurrentLEDColor (Variables|LED|GetLED_Green)))
        (:NewEnumerator3
          (Variables|LED|SetCurrentLEDColor "")))
      (CallFunction|BlinkLED))))

(fn BlinkLED
  (bind _s_telelumen_ping (Variables|Default|GetS_telelumen_ping))
  (if (Variables|LED|GetBlinkLED?)
    (if (Variables|LED|GetLEDOn?)
      (Rendering|Material|SetVectorParameterValue :self (Variables|LED|GetDMI_LED) :ParameterName "LightColor" :!class /Script/Engine.MaterialInstanceDynamic)
      (Variables|LED|SetLEDOn? false)
      (Utilities|Time|SetTimerbyFunctionName 0 "Blink LED" 0.75)
      (else
        (Rendering|Material|SetVectorParameterValue (Variables|LED|GetDMI_LED) "LightColor" (Variables|LED|GetCurrentLEDColor) :!class /Script/Engine.MaterialInstanceDynamic)
        (Variables|LED|SetLEDOn? true)
        (if (Audio|Components|Audio|IsPlaying _s_telelumen_ping)
          _
          (else
            (Audio|Components|Audio|Play _s_telelumen_ping 0.0)))
        (Utilities|Time|SetTimerbyFunctionName 0 "Blink LED" 0.5)))
    (else
      (Audio|Components|Audio|Stop (Variables|Default|GetS_telelumen_ping))
      (Rendering|Material|SetVectorParameterValue (Variables|LED|GetDMI_LED) "LightColor" (Variables|LED|GetCurrentLEDColor) :!class /Script/Engine.MaterialInstanceDynamic))))

(fn ChangeAlertState
  (params (Active? :type Boolean))
  (Variables|Screen|SetScreenGlitched? Active?)
  (CallFunction|InterpGlitchState))

(fn InterpScreenColor
  (if (Variables|Default|GetAnomalyOpened?)
    (if (== (Variables|Screen|GetCurrentScreenColor) (Variables|Screen|GetTargetScreenColor))
      (return)
      (else
        (Rendering|Material|SetVectorParameterValue (Variables|Screen|GetDMI_TeleLumenScreen) "ScreenColor" (Class|KismetMathLibrary|CInterpto (Variables|Screen|GetCurrentScreenColor) (Variables|Screen|GetTargetScreenColor) (Utilities|Time|GetWorldDeltaSeconds) 3.0) :!class /Script/Engine.MaterialInstanceDynamic)
        (Variables|Screen|SetCurrentScreenColor (Class|KismetMathLibrary|CInterpto (Variables|Screen|GetCurrentScreenColor) (Variables|Screen|GetTargetScreenColor) (Utilities|Time|GetWorldDeltaSeconds) 3.0))
        (Utilities|Time|SetTimerbyFunctionName 0 "Interp Screen Color" 0.01)))
    (elif (== (Variables|Screen|GetCurrentScreenColor) (Variables|Screen|GetDefaultScreenColor))
      (return)
      (else
        (Rendering|Material|SetVectorParameterValue (Variables|Screen|GetDMI_TeleLumenScreen) "ScreenColor" (Class|KismetMathLibrary|CInterpto (Variables|Screen|GetCurrentScreenColor) (Variables|Screen|GetDefaultScreenColor) (Utilities|Time|GetWorldDeltaSeconds) 3.0) :!class /Script/Engine.MaterialInstanceDynamic)
        (Variables|Screen|SetCurrentScreenColor (Class|KismetMathLibrary|CInterpto (Variables|Screen|GetCurrentScreenColor) (Variables|Screen|GetDefaultScreenColor) (Utilities|Time|GetWorldDeltaSeconds) 3.0))
        (Utilities|Time|SetTimerbyFunctionName 0 "Interp Screen Color" 0.01)))))

(fn EstablishEnvelopeFollower
  (params (SoundToPlay :type Sound%20Cue%20Object%20Reference))
  ;[1 1 1] Make sure the Sound Cue file has SEPC_TeleLumen under Effects->Source->SoundEffectChain
  (Audio|Components|Audio|SetSound (Variables|Default|GetAnomalySource) SoundToPlay)
  (Class|SourceEffectEnvelopeFollowerPreset|RegisterEnvelopeFollowerListener (Variables|Default|GetEnvFollowerPreset) (Variables|Default|GetEnvelopeFollowerListener)))

(fn InterpGlitchState
  (if (Variables|Screen|GetScreenGlitched?)
    (if (Math|Float|NearlyEqual(Float) (Variables|Screen|GetCurrentGlitchAmplitude) 1.0 0.001)
      (return)
      (else
        (Variables|Screen|SetCurrentGlitchAmplitude (Math|Interpolation|FInterptoConstant (Variables|Screen|GetCurrentGlitchAmplitude) 1.0 (Utilities|Time|GetWorldDeltaSeconds) 2.25))
        (Rendering|Material|SetScalarParameterValue (Variables|Screen|GetDMI_TeleLumenScreen) "Glitched" (Math|Interpolation|FInterptoConstant (Variables|Screen|GetCurrentGlitchAmplitude) 1.0 (Utilities|Time|GetWorldDeltaSeconds) 2.25) :!class /Script/Engine.MaterialInstanceDynamic)
        (Utilities|Time|SetTimerbyFunctionName 0 "Interp Glitch State" 0.01)))
    (elif (Math|Float|NearlyEqual(Float) (Variables|Screen|GetCurrentGlitchAmplitude) 0.0 0.001)
      (return)
      (else
        (Variables|Screen|SetCurrentGlitchAmplitude (Math|Interpolation|FInterptoConstant (Variables|Screen|GetCurrentGlitchAmplitude) 0.0 (Utilities|Time|GetWorldDeltaSeconds) 4.5))
        (Rendering|Material|SetScalarParameterValue (Variables|Screen|GetDMI_TeleLumenScreen) "Glitched" (Math|Interpolation|FInterptoConstant (Variables|Screen|GetCurrentGlitchAmplitude) 0.0 (Utilities|Time|GetWorldDeltaSeconds) 4.5) :!class /Script/Engine.MaterialInstanceDynamic)
        (Utilities|Time|SetTimerbyFunctionName 0 "Interp Glitch State" 0.01)))))

(fn Unequipped
  (|CallParentFunction)
  ;[1 1 1] Play Off Sound if light if on
  (if (Variables|Default|GetLightOn?)
    (Audio|PlaySound2D (Variables|Default|GetOnSound) 1.0 0.8 0.0 0 0)))