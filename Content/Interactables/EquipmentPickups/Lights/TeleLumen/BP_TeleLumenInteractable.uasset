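; TeleLumen light pickup interactable that shows a blinking LED with a ping sound.
; On BeginPlay it puts a dynamic LED material on the interactable mesh and starts BlinkLED, which re-arms itself by timer to alternate black and the current LED color, playing the ping on each lit phase.
; When blinking is off, the LED holds its color and a separately referenced ping component is stopped.
; An Act 3 check via BP_TaskManager is left unconnected.
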(event EventBeginPlay
  (|CallParentFunction)
  (bind _returnvalue (Rendering|Material|CreateDynamicMaterialInstance "/Game/Interactables/EquipmentPickups/Lights/TeleLumen/RadioLight/M_TeleLumenLED.M_TeleLumenLED" "None" "None" :!class /Script/Engine.KismetMaterialLibrary))
  (Variables|Default|SetDMI_LED _returnvalue)
  (Rendering|Material|SetMaterial (Variables|Default|GetInteractableMesh) 2 (Variables|Default|GetDMI_LED))
  (Variables|Default|SetBlinkLED? true)
  (CallFunction|BlinkLED))

(fn ConstructionScript
  (|CallParentFunction))

(fn BlinkLED
  (bind _s_telelumen_ping1 (Variables|Default|GetS_telelumen_ping1))
  (if (Variables|Default|GetBlinkLED?)
    (if (Variables|Default|GetLEDOn?)
      (Rendering|Material|SetVectorParameterValue :self (Variables|Default|GetDMI_LED) :ParameterName "LightColor" :!class /Script/Engine.MaterialInstanceDynamic)
      (Variables|Default|SetLEDOn? false)
      (Utilities|Time|SetTimerbyFunctionName 0 "Blink LED" 0.75)
      (else
        (Rendering|Material|SetVectorParameterValue (Variables|Default|GetDMI_LED) "LightColor" (Variables|Default|GetCurrentLEDColor) :!class /Script/Engine.MaterialInstanceDynamic)
        (Variables|Default|SetLEDOn? true)
        (Components|Activation|Activate _s_telelumen_ping1 false)
        (if (Audio|Components|Audio|IsPlaying _s_telelumen_ping1)
          _
          (else
            (Audio|Components|Audio|Play _s_telelumen_ping1 0.0)))
        (Utilities|Time|SetTimerbyFunctionName 0 "Blink LED" 0.5)))
    (else
      (Audio|Components|Audio|Stop (Variables|Default|GetS_telelumen_ping))
      (Rendering|Material|SetVectorParameterValue (Variables|Default|GetDMI_LED) "LightColor" (Variables|Default|GetCurrentLEDColor) :!class /Script/Engine.MaterialInstanceDynamic))))