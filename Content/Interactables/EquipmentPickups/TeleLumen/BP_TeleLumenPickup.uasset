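; TeleLumen equipment pickup: a handheld device with a spotlight and two widget screens, one for the flashlight and one for the walkie.
; BeginPlay caches both HUD widgets and hands the spotlight and its defaults to the flashlight HUD.
; SwapScreen toggles screens behind a short delay lock, and Scrub input reaches only the flashlight HUD while that screen is active.
; Tick rotates the root from player camera pitch and mesh yaw.
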(event EventBeginPlay
  (bind _returnvalue (Actor|GetActorOfClass "/Game/FirstPerson/Blueprints/BP_FirstPersonCharacter.BP_FirstPersonCharacter_C"))
  (Variables|Default|SetPlayerCharacter _returnvalue)
  (Rendering|SetVisibility (Variables|Default|GetWalkieScreen) false false)
  (CallFunction|SetFlashlightVar)
  (CallFunction|SetWalkieVar))

(event EventSwapScreen
  (|CallParentFunction)
  (if (Variables|Default|GetCanSwapScreen?)
    (if (Variables|Default|GetOnFlashlightScreen?)
      (Variables|Default|SetCanSwapScreen? false)
      (Rendering|SetVisibility (Variables|Default|GetFlashLightScreen) false false)
      (Variables|Default|SetOnFlashlightScreen? false)
      (Utilities|FlowControl|Delay 0.25)
      (Rendering|SetVisibility (Variables|Default|GetWalkieScreen) true false)
      (Variables|Default|SetCanSwapScreen? true)
      (else
        (Variables|Default|SetCanSwapScreen? false)
        (Rendering|SetVisibility (Variables|Default|GetWalkieScreen) false false)
        (Variables|Default|SetOnFlashlightScreen? true)
        (Utilities|FlowControl|Delay 0.25)
        (Rendering|SetVisibility (Variables|Default|GetFlashLightScreen) true false)
        (Variables|Default|SetCanSwapScreen? true)))))

(event EventTick
  (params (DeltaSeconds :type Float%20%28single-precision%29))
  (bind _playercharacter (Variables|Default|GetPlayerCharacter))
  (|CallParentFunction DeltaSeconds)
  (Transformation|SetWorldRotation (Variables|Default|GetDefaultSceneRoot) (Math|Rotator|MakeRotator (* (.pitch (Transformation|GetWorldRotation (Variables|/Script/PSJamJan.PSJamJanCharacter|GetFirstPersonCameraComponent _playercharacter))) -1.0) 0.0 (.yaw (Transformation|GetWorldRotation (Variables|/Script/Engine.Character|GetMesh _playercharacter)))) false false))

(fn ConstructionScript
  (bind _telelumenmesh (Variables|Default|GetTeleLumenMesh))
  (|CallParentFunction)
  (bind _returnvalue (Rendering|Material|CreateDynamicMaterialInstance _telelumenmesh 1 "/Game/Interactables/EquipmentPickups/TeleLumen/RadioLight/M_FlashlightScreen.M_FlashlightScreen" "None" :!class /Script/Engine.PrimitiveComponent))
  (Rendering|Material|SetMaterial _telelumenmesh 1 _returnvalue))

(fn Equipped
  (|CallParentFunction))

(fn Scrub
  (params (InputValue :type Float%20%28double-precision%29))
  (|CallParentFunction InputValue)
  (if (Variables|Default|GetOnFlashlightScreen?)
    (Default|GetScrubbed (Variables|Default|GetAs%20WBP%20Flashlight%20HUD) InputValue)))

(fn SetFlashlightVar
  (bind _spotlight (Variables|Default|GetSpotLight))
  (bind _aswbp_flashlight_hud (Utilities|Casting|CastToWBP_FlashlightHUD (UserInterface|GetWidget (Variables|Default|GetFlashLightScreen)))
    (:then
      (bind _output_get (Variables|Default|SetAs%20WBP%20Flashlight%20HUD _aswbp_flashlight_hud))
      (Variables|/Game/Interactables/EquipmentPickups/TeleLumen/RadioLight/WBP_FlashlightHUD.WBP_FlashlightHUD_C|SetSpotlightRef _output_get _spotlight)
      (Variables|/Game/Interactables/EquipmentPickups/TeleLumen/RadioLight/WBP_FlashlightHUD.WBP_FlashlightHUD_C|SetDefaultSpotlightIntensity _output_get (Variables|/Script/Engine.LightComponentBase|GetIntensity _spotlight))
      (Variables|/Game/Interactables/EquipmentPickups/TeleLumen/RadioLight/WBP_FlashlightHUD.WBP_FlashlightHUD_C|SetDefaultAttenuationRadius _output_get (Variables|/Script/Engine.LocalLightComponent|GetAttenuationRadius _spotlight)))
    (:CastFailed
      (Development|PrintString "Failed to Cast to WBP_FlashlightHUD --Event BeginPlay-- BP_TeleLumenPickup"))))

(fn SetWalkieVar
  (bind _aswbp_walkie_hud (Utilities|Casting|CastToWBP_WalkieHUD (UserInterface|GetWidget (Variables|Default|GetWalkieScreen)))
    (:then
      (Variables|Default|SetAs%20WBP%20Walkie%20HUD _aswbp_walkie_hud))
    (:CastFailed
      (Development|PrintString "Failed to Cast to WBP_WalkieHUD --Event BeginPlay-- BP_TeleLumenPickup"))))