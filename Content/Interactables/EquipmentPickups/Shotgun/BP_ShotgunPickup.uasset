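; Shotgun equipment pickup that, while equipped, follows the first-person character's mesh yaw and camera pitch each Tick.
; UseEquipment is DoOnce-gated: when equipped, it fires a debug-drawn camera line trace, spends ammo and waits before resetting, otherwise playing a no-ammo sound.
; The trace result is unused, and Shoot does not check ammo.
; Reloading adds shells one at a time through a self-rescheduling LoadShell timer until MaxAmmo.
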(event Custom|Reload%20Weapon
  (CallFunction|Reload))

(event EventBeginPlay
  (bind _returnvalue (Actor|GetActorOfClass "/Game/FirstPerson/Blueprints/BP_FirstPersonCharacter.BP_FirstPersonCharacter_C"))
  (Variables|Default|SetBP_FirstPersonCharacter _returnvalue))

(event Collision|EventActorBeginOverlap
  (params (OtherActor :type Actor%20Object%20Reference))
  (|CallParentFunction OtherActor) ; This node is disabled and will not be called.\nDrag off pins to build functionality.
)

(event EventTick
  (params (DeltaSeconds :type Float%20%28single-precision%29))
  (|CallParentFunction DeltaSeconds)
  (if (Variables|Default|GetEquipped?)
    (bind _bp_firstpersoncharacter (Variables|Default|GetBP_FirstPersonCharacter)
      (:then
        (Utilities|HandleObjectRotation _bp_firstpersoncharacter _bp_firstpersoncharacter :!label _label))
      (:else
        (goto _label execute2)))))

(event EventUseEquipment
  (Utilities|FlowControl|DoOnce false :!label _label
    (:Completed
      (if (Variables|Default|GetEquipped?)
        (CallFunction|Shoot)
        (Variables|Default|SetIsShooting? true)
        (Utilities|FlowControl|Delay 2.0)
        (Variables|Default|SetIsShooting? false)
        (goto _label Reset)
        (else
          (Audio|PlaySoundatLocation "/Game/Sounds/General_SFX/Shotgun/S_shotgun_no_ammo.S_shotgun_no_ammo" (Transformation|GetWorldLocation (Variables|Default|GetShotgun)) "0, 0, 0" 1.0 1.0 0.0 0 0 0 0)
          (goto _label Reset))))))

(fn ConstructionScript
  (|CallParentFunction))

(fn Reload
  (Utilities|ReloadHandler)
  (if (Variables|Default|GetCanReload?)
    (CallFunction|LoadShell)))

(fn Shoot
  (bind _bp_firstpersoncharacter (Variables|Default|GetBP_FirstPersonCharacter))
  (bind _firstpersoncameracomponent (Variables|/Script/PSJamJan.PSJamJanCharacter|GetFirstPersonCameraComponent _bp_firstpersoncharacter))
  (bind _returnvalue (Transformation|GetWorldLocation _firstpersoncameracomponent))
  ;[0.07292 0.07292 0.07292] Use Ammo
  (Math|Integer|DecrementInt (Variables|Default|GetAmmo)
    (:%20%20
      ;[0.07292 0.07292 0.07292] Play Gun Shot Sound
      (Audio|PlaySoundatLocation "/Game/Sounds/General_SFX/Shotgun/S_shotgun_shoot_and_cock.S_shotgun_shoot_and_cock" (Transformation|GetWorldLocation (Variables|Default|GetFirePoint)) "0, 0, 0" 1.0 1.0 0.0 0 0 0 0)
      ;[0.07292 0.07292 0.07292] Firing Line Trace
      (Collision|LineTraceByChannel _returnvalue (+ _returnvalue (* (Math|Vector|GetForwardVector _firstpersoncameracomponent) (Variables|Default|GetGunRange))) "TraceTypeQuery1" false 0 "ForDuration" true "(R=1.000000,G=0.000000,B=0.000000,A=1.000000)" "(R=0.000000,G=1.000000,B=0.000000,A=1.000000)" 2.0))))

(fn LoadShell
  (Variables|Default|SetCanReload? false)
  (Variables|Default|SetIsReloading? true)
  (Variables|Default|SetAmmo (+ (Variables|Default|GetAmmo) 1))
  (Audio|PlaySoundatLocation "/Game/Sounds/General_SFX/Shotgun/S_shotgun_reload_cue.S_shotgun_reload_cue" (Transformation|GetWorldLocation (Variables|Default|GetShotgun)) "0, 0, 0" 1.0 1.0 0.0 0 0 0 0)
  (if (!= (Variables|Default|GetAmmo) (Variables|Default|GetMaxAmmo))
    (Utilities|Time|SetTimerbyFunctionName 0 "LoadShell" 0.75)
    (Development|PrintString (Utilities|String|ToString(Integer) (Variables|Default|GetAmmo)))
    (else
      (Variables|Default|SetIsReloading? false)
      (return))))