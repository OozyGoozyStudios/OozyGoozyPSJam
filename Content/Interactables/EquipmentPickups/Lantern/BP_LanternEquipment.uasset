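; Lantern equipment whose point light dims while lit, switches off when empty and is refueled by using it.
; Tick drives the dimming, and intensity sets both the light and the burning and glug sound volumes.
; Using it at max intensity starts a self-rescheduling burn-down lockout, during which further use only plays an overload sound.
; ToggleLight resets to base intensity when switching on and shows a brief fueling tutorial the first time.
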(event Custom|TimerEvent)

(event EventBeginPlay
  (CallFunction|IsLighton)
  (CallFunction|UpdateSoundProperties))

(event EventUseEquipment
  (if (Variables|Default|GetbLightOn?)
    (if (Variables|Default|GetbBurningDown?)
      (CallFunction|PlayOverload)
      (elif (< (Variables|Default|GetCurrentIntensity) (Variables|Default|GetMaxIntensity))
        (bind _output_get (Variables|Default|SetCurrentIntensity (+ (Variables|Default|GetCurrentIntensity) (Variables|Default|GetRechargePerClick))))
        (CallFunction|PlayGlug _output_get)
        (CallFunction|UpdateSoundProperties)
        (else
          (CallFunction|BurnDown))))))

(event EventTick
  (params (DeltaSeconds :type Float%20%28single-precision%29))
  (if (Math|Boolean|ANDBoolean (> (Variables|Default|GetCurrentIntensity) 0.0) (Variables|Default|GetbLightOn?) (not (Utilities|Time|IsTimerActivebyHandle (Variables|Default|GetLightTimerHandle))))
    (bind _returnvalue (Utilities|Time|SetTimerbyEvent (delegate Custom|TimerEvent) (Variables|Default|GetLightTimer) true))
    (bind _output_get (Variables|Default|SetLightTimerHandle _returnvalue))
    (CallFunction|SubtractfromLight)
    (CallFunction|TimerEvent)
    (Utilities|Time|ClearandInvalidateTimerbyHandle _output_get)
    (CallFunction|IsLighton)))

(fn ConstructionScript)

(fn SetIntensity
  (params (Intensity :type Float%20%28double-precision%29))
  (Rendering|Components|Light|SetIntensity (Variables|Default|GetPointLight) Intensity))

(fn ToggleLight
  (if (Variables|Default|GetbLightOn?)
    (Variables|Default|SetbLightOn? false)
    (CallFunction|SetIntensity 0.0)
    (else
      (if (Variables|Default|GetHasBeenTurnedOn?)
        _
        (else
          (bind _returnvalue (UserInterface|CreateWidget "/Game/Interactables/EquipmentPickups/WBP_TutorialWidget.WBP_TutorialWidget_C" 0 "LeftMouseButton" "Fuel Lantern" true))
          (Variables|Default|SetTutorialWidget _returnvalue)
          (UserInterface|Viewport|AddtoViewport _returnvalue 0)
          (Utilities|Time|SetTimerbyFunctionName 0 "RemoveTutorialWidget" 2.2)))
      (Variables|Default|SetbLightOn? true)
      (Variables|Default|SetCurrentIntensity (Variables|Default|GetBaseIntensity))
      (CallFunction|SetIntensity (Variables|Default|GetCurrentIntensity))
      (CallFunction|UpdateSoundProperties)
      (Variables|Default|SetHasBeenTurnedOn? true))))

(fn IsLighton
  (bind _currentintensity (Variables|Default|GetCurrentIntensity))
  (if (Variables|Default|GetbLightOn?)
    (CallFunction|SetIntensity _currentintensity)
    (if (<= _currentintensity 0.0)
      (Variables|Default|SetbLightOn? false))
    (else
      (CallFunction|SetIntensity 0.0))))

(fn SubtractfromLight
  (Variables|Default|SetCurrentIntensity (- (Variables|Default|GetCurrentIntensity) (Variables|Default|GetDimAmount)))
  (CallFunction|UpdateSoundProperties))

(fn StartStopDimTimer
  (params (TimerHandle :type Timer%20Handle%20Structure))
  (if (Variables|Default|GetbLightOn?)
    (Utilities|Time|UnpauseTimerbyHandle TimerHandle)
    (else
      (Utilities|Time|PauseTimerbyHandle TimerHandle))))

(fn BurnDown
  (if (Variables|Default|GetbBurningDown?)
    (Variables|Default|SetCurrentBurnLevel (+ (Variables|Default|GetCurrentBurnLevel) (Variables|Default|GetBurnStepAmount)))
    (if (>= (Variables|Default|GetCurrentBurnLevel) (Variables|Default|GetBurnDownMax))
      (CallFunction|EndBurnDown)
      (else
        (Utilities|Time|SetTimerbyFunctionName 0 "BurnDown" 0.1)))
    (else
      (Variables|Default|SetbBurningDown? true)
      (Variables|Default|SetCurrentBurnLevel 0.0)
      (Utilities|Time|SetTimerbyFunctionName 0 "BurnDown" 0.1))))

(fn EndBurnDown
  (Variables|Default|SetbBurningDown? false))

(fn UpdateSoundProperties
  (Audio|Components|Audio|SetVolumeMultiplier (Variables|Default|GetS_lantern_burning) (Math|Float|MapRangeClamped (Variables|Default|GetCurrentIntensity) 0.0 3.5e+02 0.0 1.5) :!class /Script/Engine.AudioComponent))

(fn PlayOverload
  (Audio|PlaySoundatLocation "/Game/Sounds/General_SFX/Lantern/S_lantern_overload.S_lantern_overload" (Transformation|GetWorldLocation (Variables|Default|GetLanternGlass)) "0, 0, 0" 2.0 1.0 0.0 0 0 0 0))

(fn PlayGlug
  (params (CurrentIntensity :type Float%20%28double-precision%29))
  (Audio|PlaySoundatLocation "/Game/Sounds/General_SFX/Lantern/Glugs/S_glug_Cue.S_glug_Cue" (Transformation|GetWorldLocation (Variables|Default|GetLanternGlass)) "0, 0, 0" (Math|Float|MapRangeClamped CurrentIntensity 1.5e+02 3.5e+02 0.5 2.0) 1.0 0.0 0 0 0 0))

(fn RemoveTutorialWidget
  (bind _tutorialwidget (Variables|Default|GetTutorialWidget)
    (:then
      (Default|CompleteTutorial _tutorialwidget))
    (:else)))