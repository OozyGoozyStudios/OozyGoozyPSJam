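; Base Blueprint for equipment pickups, defining the shared hooks for equipping, using and removing an item.
; Equipped and Unequipped show or hide the root component and its children, and Removed destroys the actor.
; UseEquipment, UseEquipmentEnd, Scrub and SwapScreen are empty stubs, and GetIncrementalText returns an empty string, leaving item-specific behavior undefined at this level.
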(event Custom|UseEquipment)

(event Custom|UseEquipmentEnd)

(event Collision|EventActorBeginOverlap
  (params (OtherActor :type Actor%20Object%20Reference)))

(event EventTick
  (params (DeltaSeconds :type Float%20%28single-precision%29)))

(fn ConstructionScript
  (|CallParentFunction))

(fn Equipped
  (Rendering|SetVisibility (Variables|Default|GetDefaultSceneRoot) true true))

(fn Unequipped
  (Rendering|SetVisibility (Variables|Default|GetDefaultSceneRoot) false true))

(fn Removed
  (Actor|DestroyActor))

(fn GetIncrementalText
  (return ""))

(fn Scrub
  (params (InputValue :type Float%20%28double-precision%29)))

(fn SwapScreen)