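; Equippable filled coffee cup pickup that the first-person character sips from until it is empty.
; UseEquipment moves the cup between the hand and mouth sockets using self-rescheduling timers with TInterpTo, while polled flags gate the next sip.
; Each sip lowers and rescales the fill line, hiding it once empty, and tells the character to refresh its equip widget text.
; GetIncrementalText builds the cup's label showing remaining sips.
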(event Custom|SipCoffee
  (Variables|Default|SetbCanSip? false)
  (CallFunction|BringCuptoMouth)
  (CallFunction|CheckCupatMouth))

(event Custom|CheckCupAtMouth
  (if (Variables|Default|GetCupAtMouth?)
    (Utilities|FlowControl|Delay 1.0)
    (CallFunction|ReturnCuptoHand)
    (CallFunction|CheckCupatHand)
    (else
      (Utilities|Time|SetTimerbyFunctionName 0 "CheckCupAtMouth" 0.1))))

(event Custom|CheckCupAtHand
  (if (Variables|Default|GetCupAtHand?)
    (Variables|Default|SetbCanSip? true)
    (else
      (Utilities|Time|SetTimerbyFunctionName 0 "CheckCupAtHand" 0.1))))

(event EventBeginPlay
  (bind _asbp_first_person_character (Utilities|Casting|CastToBP_FirstPersonCharacter (Game|GetPlayerCharacter 0)))
  (Variables|Default|SetAs%20BP%20First%20Person%20Character _asbp_first_person_character))

(event Collision|EventActorBeginOverlap
  (params (OtherActor :type Actor%20Object%20Reference))
  (|CallParentFunction OtherActor) ; This node is disabled and will not be called.\nDrag off pins to build functionality.
)

(event EventTick
  (params (DeltaSeconds :type Float%20%28single-precision%29))
  (|CallParentFunction DeltaSeconds) ; This node is disabled and will not be called.\nDrag off pins to build functionality.
)

(event EventUseEquipment
  (if (Variables|Default|GetbCanSip?)
    (if (not (Variables|Default|GetIsEmpty?))
      (CallFunction|SipCoffee))))

(fn ConstructionScript
  (|CallParentFunction))

(fn MoveCoffeeLine
  (Development|PrintString "Schlurp")
  (bind _output_get (Variables|Default|SetCurrentSipCount (+ (Variables|Default|GetCurrentSipCount) 1)))
  (if (>= _output_get (Variables|Default|GetMaxNumberSips))
    (Variables|Default|SetIsEmpty? true)
    (Variables|Default|SetbCanSip? false)
    (Rendering|SetVisibility (Variables|Default|GetFillLine) false false)
    (else
      (switch int _output_get
        (:1
          (Transformation|SetRelativeTransform (Variables|Default|GetFillLine) (Math|Transform|MakeTransform (Variables|Default|GetSip1Level) "0, 0, 0" (Variables|Default|GetSip1Scale)) false false))
        (:2
          (Transformation|SetRelativeTransform (Variables|Default|GetFillLine) (Math|Transform|MakeTransform (Variables|Default|GetSip2Level) "0, 0, 0" (Variables|Default|GetSip2Scale)) false false))
        (:3
          (Transformation|SetRelativeTransform (Variables|Default|GetFillLine) (Math|Transform|MakeTransform (Variables|Default|GetSip3Level) "0, 0, 0" (Variables|Default|GetSip3Scale)) false false)))))
  (Default|ChangeEquipWidgetText (Variables|Default|GetAs%20BP%20First%20Person%20Character))
  (return))

(fn BringCuptoMouth
  (bind _as_bp_first_person_character (Variables|Default|GetAs%20BP%20First%20Person%20Character))
  (bind _coffeecup (Variables|Default|GetCoffeeCup))
  (bind _returnvalue (Transformation|GetWorldTransform _coffeecup))
  (bind _mesh (Variables|/Script/Engine.Character|GetMesh _as_bp_first_person_character))
  (bind _returnvalue_2 (Transformation|GetSocketTransform _mesh "SipCoffeeSocket" "RTS_World"))
  (if (>= (Math|Vector|Distance(Vector) (.Location (Math|Transform|BreakTransform _returnvalue)) (.Location (Math|Transform|BreakTransform _returnvalue_2))) (Variables|Default|GetMinDistance))
    (Transformation|SetWorldTransform (Variables|Default|GetCoffeeCup) (Class|KismetMathLibrary|TInterpto _returnvalue _returnvalue_2 (Utilities|Time|GetWorldDeltaSeconds) 5.0) false false)
    (Utilities|Time|SetTimerbyFunctionName 0 "BringCupToMouth" 0.01)
    (else
      (CallFunction|MoveCoffeeLine)
      (Variables|Default|SetCupAtMouth? true))))

(fn ReturnCuptoHand
  (bind _as_bp_first_person_character (Variables|Default|GetAs%20BP%20First%20Person%20Character))
  (bind _coffeecup (Variables|Default|GetCoffeeCup))
  (bind _returnvalue (Transformation|GetWorldTransform _coffeecup))
  (bind _mesh (Variables|/Script/Engine.Character|GetMesh _as_bp_first_person_character))
  (bind _returnvalue_2 (Transformation|GetSocketTransform _mesh "ItemSocket" "RTS_World"))
  (if (>= (Math|Vector|Distance(Vector) (.Location (Math|Transform|BreakTransform _returnvalue)) (.Location (Math|Transform|BreakTransform _returnvalue_2))) (Variables|Default|GetMinDistance))
    (Transformation|SetWorldTransform (Variables|Default|GetCoffeeCup) (Class|KismetMathLibrary|TInterpto _returnvalue _returnvalue_2 (Utilities|Time|GetWorldDeltaSeconds) 5.0) false false)
    (Utilities|Time|SetTimerbyFunctionName 0 "ReturnCupToHand" 0.01)
    (Variables|Default|SetCupAtMouth? false)
    (else
      (Variables|Default|SetCupAtHand? true))))

(fn GetIncrementalText
  (bind _maxnumbersips (Variables|Default|GetMaxNumberSips))
  (switch int (Variables|Default|GetCurrentSipCount)
    (:0
      (bind _output_get (Variables|Default|SetIncrementalString "Full"))
      (Variables|Default|SetFullIncrementalString (Utilities|String|Append "Coffee Cup " "(" _output_get ")")))
    (:1
      (bind _output_get_2 (Variables|Default|SetIncrementalString (Utilities|String|Append (Utilities|String|ToString(Integer) (- _maxnumbersips (Variables|Default|GetCurrentSipCount))) "/" (Utilities|String|ToString(Integer) _maxnumbersips)) :!label _label))
      (Variables|Default|SetFullIncrementalString (Utilities|String|Append "Coffee Cup " "(" _output_get_2 ")")))
    (:2
      (goto _label))
    (:3
      (goto _label))
    (:4
      (bind _output_get_3 (Variables|Default|SetIncrementalString "Empty"))
      (Variables|Default|SetFullIncrementalString (Utilities|String|Append "Coffee Cup " "(" _output_get_3 ")"))))
  (return (Utilities|Text|ToText(String) (Variables|Default|GetFullIncrementalString))))