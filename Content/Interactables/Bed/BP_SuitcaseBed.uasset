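; Bed interactable that shows a suitcase once equipment is consumed on it.
; Consuming the equipment runs the parent logic, then sets SuitcasePlaced and reveals SuitcaseMesh.
; The construction script and ActorLoaded event both reapply mesh visibility from that flag, so editor and loaded states match it.
; The save interface's ComponentsToSave returns no components.
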(event EventBeginPlay)

(event Collision|EventActorBeginOverlap
  (params (OtherActor :type Actor%20Object%20Reference)))

(event EventTick
  (params (DeltaSeconds :type Float%20%28single-precision%29)))

(event EventActorLoaded
  (Rendering|SetVisibility (Variables|Default|GetSuitcaseMesh) (Variables|Default|GetSuitcasePlaced?) false))

(event EventEquipmentConsumed
  (|CallParentFunction)
  (Variables|Default|SetSuitcasePlaced? true)
  (Rendering|SetVisibility (Variables|Default|GetSuitcaseMesh) (Variables|Default|GetSuitcasePlaced?) false))

(fn ConstructionScript
  (|CallParentFunction)
  (Rendering|SetVisibility (Variables|Default|GetSuitcaseMesh) (Variables|Default|GetSuitcasePlaced?) false))

(fn ComponentstoSave
  (return))