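; BP_FakeTeleLumen is a TeleLumen prop whose screen, LED and spotlight light up when it becomes powered.
; The construction script creates dynamic material instances for the screen and LED and assigns them to the static mesh.
; TogglePower applies the Powered flag to their emissive scalars and the spotlight intensity on BeginPlay and on BecomePowered, which only switches power on.
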(event Custom|BecomePowered
  (Variables|Default|SetPowered? true)
  (CallFunction|TogglePower))

(event EventBeginPlay
  (CallFunction|TogglePower))

(fn ConstructionScript
  (CallFunction|SetupDMIs))

(fn SetupDMIs
  (bind _returnvalue (Rendering|Material|CreateDynamicMaterialInstance "/Game/Interactables/EquipmentPickups/Lights/TeleLumen/RadioLight/M_TeleLumenScreen.M_TeleLumenScreen" "None" "None" :!class /Script/Engine.KismetMaterialLibrary))
  (Variables|Default|SetDMI_Screen _returnvalue)
  (bind _returnvalue_2 (Rendering|Material|CreateDynamicMaterialInstance "/Game/Interactables/EquipmentPickups/Lights/TeleLumen/RadioLight/M_TeleLumenLED.M_TeleLumenLED" "None" "None" :!class /Script/Engine.KismetMaterialLibrary))
  (Variables|Default|SetDMI_LED _returnvalue_2)
  (Rendering|Material|SetMaterial (Variables|Default|GetStaticMesh) 1 (Variables|Default|GetDMI_Screen))
  (Rendering|Material|SetMaterial (Variables|Default|GetStaticMesh) 2 (Variables|Default|GetDMI_LED)))

(fn TogglePower
  (if (Variables|Default|GetPowered?)
    (Rendering|Material|SetScalarParameterValue (Variables|Default|GetDMI_Screen) "EmissiveScalar" 0.05 :!class /Script/Engine.MaterialInstanceDynamic)
    (Rendering|Material|SetScalarParameterValue (Variables|Default|GetDMI_LED) "EmissiveScalar" 5.0 :!class /Script/Engine.MaterialInstanceDynamic)
    (Rendering|Components|Light|SetIntensity (Variables|Default|GetSpotLight) 2e+03)
    (else
      (Rendering|Material|SetScalarParameterValue (Variables|Default|GetDMI_Screen) "EmissiveScalar" 0.0 :!class /Script/Engine.MaterialInstanceDynamic)
      (Rendering|Material|SetScalarParameterValue (Variables|Default|GetDMI_LED) "EmissiveScalar" 0.0 :!class /Script/Engine.MaterialInstanceDynamic)
      (Rendering|Components|Light|SetIntensity (Variables|Default|GetSpotLight) 0.0))))

(fn ComponentstoSave
  (return 0))