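; Scripted stand-in infrared button that fills by itself when IRPowerRestored fires, then opens the bunker power door.
; A looping timer interpolates progress, driving button color, thermal bar material and sound pitch until completion.
; TaskManager power, IR-sensor and optional override-ID events refresh its powered state and glow.
; Focus events are empty and their former hold-to-charge logic is disconnected, so looking at it does not start progress.
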(event Custom|IRSensorsActive_Event
  (Variables|Default|SetIsActivated? true)
  (CallFunction|PowerUpdateButton))

(event Custom|CheckForOutOfFocus
  (Utilities|Time|SetTimerbyFunctionName 0 "CheckForFocus" 1.0))

(event Custom|OverrideSensorID_Event
  (params (SensorID :type Integer))
  (if (== SensorID (Variables|Default|GetRemoteDoorID))
    (Variables|Default|SetHasReceivedOverride? true)
    (CallFunction|PowerUpdateButton)))

(event Custom|IRPowerRestored
  (CallFunction|IncrementFocusProgress))

(event Custom|FakeButtonCompleted
  (bind _s_infrared_completed (Variables|Default|GetS_Infrared_Completed))
  (Variables|Default|SetButtonCompleted? true)
  (Variables|Default|SetHasBeenInteracted? true)
  (Variables|Default|SetButtonFull? true)
  (Variables|Default|SetButtonDecrements? false)
  (Rendering|Material|SetVectorParameterValue (Variables|Default|GetDMI_ButtonEmissive) "ButtonColor" (Variables|Default|GetCompletedColor) :!class /Script/Engine.MaterialInstanceDynamic)
  (Rendering|Material|SetScalarParameterValue (Variables|Default|GetDMI_ThermalPanel) "TransitionValue" 1.0 :!class /Script/Engine.MaterialInstanceDynamic)
  (Components|Activation|Deactivate (Variables|Default|GetS_Infrared_Full))
  (Components|Activation|Activate _s_infrared_completed false)
  (Audio|Components|Audio|Play _s_infrared_completed 0.0)
  (bind _returnvalue (Actor|GetActorOfClass "/Game/Interactables/Door/BP_BunkerPowerDoor.BP_BunkerPowerDoor_C"))
  (Default|MakeDoorOpen _returnvalue true))

(event EventBeginPlay
  (Variables|Default|SetHasBeenInteracted? true)
  (Utilities|FlowControl|Delay 0.2)
  (Variables|Default|SetButtonProgress 0.0)
  (Collision|SetCollisionEnabled (Variables|Default|GetConeOverlapSKM) "QueryOnly")
  (bind _as_bp_first_person_character (CallFunction|StorePlayerCharacterRef))
  (bind _taskmanager (Variables|/Game/FirstPerson/Blueprints/BP_FirstPersonCharacter.BP_FirstPersonCharacter_C|GetTaskManager _as_bp_first_person_character)
    (:then
      (Variables|Default|SetIsActivated? (Variables|/Game/TaskSystem/BP_TaskManager.BP_TaskManager_C|GetIRSensorsActive? _taskmanager))
      (|BindToPowerUpdate _taskmanager _taskmanager)
      (EventDispatchers|AssignIRSensorsActive _taskmanager (delegate Custom|IRSensorsActive_Event))
      (CallFunction|PowerUpdateButton)
      (if (Variables|Default|GetRequiresOverride?)
        (EventDispatchers|AssignOverrideSensorID _taskmanager (delegate Custom|OverrideSensorID_Event))))
    (:else)))

(event EventActorLoaded
  (CallFunction|PowerUpdateButton)
  (if (Variables|Default|GetButtonCompleted?)
    (Rendering|Material|SetVectorParameterValue (Variables|Default|GetDMI_ButtonEmissive) "ButtonColor" (Variables|Default|GetCompletedColor) :!class /Script/Engine.MaterialInstanceDynamic)
    (Rendering|Material|SetScalarParameterValue (Variables|Default|GetDMI_ThermalPanel) "TransitionValue" 1.0 :!class /Script/Engine.MaterialInstanceDynamic)
    (else
      (Rendering|Material|SetVectorParameterValue (Variables|Default|GetDMI_ButtonEmissive) "ButtonColor" (Variables|Default|GetOffColor) :!class /Script/Engine.MaterialInstanceDynamic)
      (Rendering|Material|SetScalarParameterValue (Variables|Default|GetDMI_ThermalPanel) "TransitionValue" 0.0 :!class /Script/Engine.MaterialInstanceDynamic))))

(event EventInFocus)

(event EventOutFocus)

(fn ConstructionScript
  (bind _dmi_buttonemissive (Variables|Default|GetDMI_ButtonEmissive))
  (bind _buttonfull_ (Variables|Default|GetButtonFull?))
  (|CallParentFunction)
  (CallFunction|CheckDMIIsValid)
  (Rendering|Material|SetMaterial (Variables|Default|GetInteractableMesh) 0 _dmi_buttonemissive)
  (Rendering|Material|SetVectorParameterValue _dmi_buttonemissive "ButtonColor" (Math|Color|SelectColor (Variables|Default|GetOnColor) (Variables|Default|GetOffColor) _buttonfull_) :!class /Script/Engine.MaterialInstanceDynamic)
  (Rendering|Material|SetScalarParameterValue (Variables|Default|GetDMI_ThermalPanel) "TransitionValue" (Math|Float|SelectFloat 1.0 0.0 _buttonfull_) :!class /Script/Engine.MaterialInstanceDynamic))

(fn IncrementFocusProgress
  (if (not (Variables|Default|GetButtonCompleted?))
    (Components|Activation|Activate (Variables|Default|GetS_Infrared_Progess) false)
    (if (Math|Float|NearlyEqual(Float) (Variables|Default|GetButtonProgress) 1.0 (LocalVariables|GetTolerance))
      (CallFunction|FakeButtonCompleted)
      (return)
      (else
        (Variables|Default|SetButtonProgress (Math|Interpolation|FInterptoConstant (Variables|Default|GetButtonProgress) 1.0 (Utilities|Time|GetWorldDeltaSeconds) (LocalVariables|GetInterpSpeed)))
        (Rendering|Material|SetVectorParameterValue (Variables|Default|GetDMI_ButtonEmissive) "ButtonColor" (Math|Color|Lerp(LinearColor) (Variables|Default|GetOffColor) (Variables|Default|GetOnColor) (Variables|Default|GetButtonProgress)) :!class /Script/Engine.MaterialInstanceDynamic)
        (Rendering|Material|SetScalarParameterValue (Variables|Default|GetDMI_ThermalPanel) "TransitionValue" (Variables|Default|GetButtonProgress) :!class /Script/Engine.MaterialInstanceDynamic)
        (Audio|Components|Audio|SetPitchMultiplier (Variables|Default|GetS_Infrared_Progess) (Math|Float|MapRangeClamped (Variables|Default|GetButtonProgress) 0.0 1.0 1.0 2.0))
        (bind _returnvalue (Utilities|Time|SetTimerbyFunctionName 0 "Increment Focus Progress" 0.01))
        (Variables|Default|SetIncrementFocusProgress _returnvalue)))))

(fn StoreTelelumenRef
  (Variables|Default|GetTeleLumenRef
    (:then
      _)
    (:else
      (bind _returnvalue (Actor|GetActorOfClass "/Game/Interactables/EquipmentPickups/Lights/TeleLumen/BP_TeleLumenPickup.BP_TeleLumenPickup_C"))
      (Utilities|IsValid _returnvalue
        (:Is%20Valid
          (Variables|Default|SetTeleLumenRef _returnvalue)))))
  (return (Variables|Default|GetTeleLumenRef)))

(fn StorePlayerCharacterRef
  (Variables|Default|GetAs%20BP%20First%20Person%20Character
    (:then
      _)
    (:else
      (bind _asbp_first_person_character (Utilities|Casting|CastToBP_FirstPersonCharacter (Game|GetPlayerCharacter 0)))
      (Variables|Default|SetAs%20BP%20First%20Person%20Character _asbp_first_person_character)))
  (return (Variables|Default|GetAs%20BP%20First%20Person%20Character)))

(fn CheckforFocus
  (bind _buttoncompleted_ (Variables|Default|GetButtonCompleted?))
  (bind _buttonfull_ (Variables|Default|GetButtonFull?))
  (bind _infocus_ (Variables|Default|GetInFocus?))
  (bind _returnvalue (not _buttoncompleted_))
  (Development|PrintString (Utilities|String|Append "CheckForFocus:" "   " (Utilities|String|ToString(Boolean) _returnvalue) "   " (Utilities|String|ToString(Boolean) _buttonfull_) "   " (Utilities|String|ToString(Boolean) _infocus_)))
  (if _returnvalue
    (if _buttonfull_
      (if _infocus_
        (Utilities|Time|SetTimerbyFunctionName 0 "CheckForFocus" 0.5)))))

(fn CheckDMIIsValid
  (Variables|Default|GetDMI_ButtonEmissive
    (:then
      _)
    (:else
      (bind _returnvalue (Rendering|Material|CreateDynamicMaterialInstance (Rendering|Material|GetMaterial (Variables|Default|GetInteractableMesh) 0) "None" "None" :!class /Script/Engine.KismetMaterialLibrary))
      (Variables|Default|SetDMI_ButtonEmissive _returnvalue)
      (Rendering|Material|SetMaterial (Variables|Default|GetInteractableMesh) 0 (Variables|Default|GetDMI_ButtonEmissive))))
  (Variables|Default|GetDMI_ThermalPanel
    (:then
      _)
    (:else
      (bind _returnvalue_2 (Rendering|Material|CreateDynamicMaterialInstance (Rendering|Material|GetMaterial (Variables|Default|GetPanel_thermalbar) 0) "None" "None" :!class /Script/Engine.KismetMaterialLibrary))
      (Variables|Default|SetDMI_ThermalPanel _returnvalue_2)
      (Rendering|Material|SetMaterial (Variables|Default|GetPanel_thermalbar) 0 (Variables|Default|GetDMI_ThermalPanel))))
  (return))

(fn PowerUpdateButton
  (if (Variables|Default|GetRequiresOverride?)
    (if (Variables|Default|GetHasReceivedOverride?)
      (if (Variables|Default|GetIsActivated?) :!label _label
        (Rendering|Material|SetScalarParameterValue (Variables|Default|GetDMI_ButtonEmissive) "EmissiveMultiplier" 0.1 :!class /Script/Engine.MaterialInstanceDynamic)
        (Variables|Default|SetHasBeenInteracted? false)
        (Variables|Default|SetHasPower? true)
        (else
          (Rendering|Material|SetScalarParameterValue (Variables|Default|GetDMI_ButtonEmissive) "EmissiveMultiplier" 0.0 :!class /Script/Engine.MaterialInstanceDynamic :!label _label_2)
          (Variables|Default|SetHasBeenInteracted? true)
          (Variables|Default|SetHasPower? false)))
      (else
        (goto _label_2)))
    (else
      (goto _label))))

(event Custom|DynamicIntensityChanged_Event
  (params (NewDynamicIntensity :type Float%20%28double-precision%29))
  (if (not (Variables|Default|GetButtonCompleted?))
    (if (Variables|Default|GetInFocus?)
      (Utilities|Time|SetTimerbyFunctionName 0 "Increment Focus Progress" 0.01))))

(event Custom|PowerUpdate_Event
  (params (LightState :type E_LightStates%20Enum :default "NewEnumerator0"))
  (Variables|Default|SetLight%20State LightState)
  (CallFunction|PowerUpdateButton))

(fn ReturnFocusCenter
  (return (Transformation|GetWorldLocation (Variables|Default|GetInteractableMesh))))