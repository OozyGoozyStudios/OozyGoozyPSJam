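; Infrared button interactable that fills while the player faces it with enough TeleLumen intensity, then opens a remote door through the player's TaskManager.
; Self-rescheduling timers interpolate progress up or down, driving dynamic materials for button color and thermal bar.
; If set to decrement, it closes the door after a hold delay once focus is lost.
; A TaskManager completion event matching its door ID locks it in the completed state.
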(event Custom|ButtonFull
  (Utilities|FlowControl|DoOnce false
    (:Completed
      (Development|PrintString "Button Completed")
      (Variables|Default|SetCompleted? true)
      (Variables|Default|SetButtonFull? true)
      (Variables|Default|SetHasBeenInteracted? true)
      (bind _as_bp_first_person_character (CallFunction|StorePlayerCharacterRef))
      (bind _taskmanager (Variables|/Game/FirstPerson/Blueprints/BP_FirstPersonCharacter.BP_FirstPersonCharacter_C|GetTaskManager _as_bp_first_person_character)
        (:then
          (Default|OpenRemoteDoor _taskmanager (Variables|Default|GetRemoteDoorID))
          (if (and (Variables|Default|GetButtonDecrements?) (not (Variables|Default|GetButtonCompleted?)))
            (CallFunction|ButtonUncompleted)))
        (:else
          (Development|PrintString "TaskManager is not Valid --BP_InfraredButton-- Event Button Completed"))))))

(event Custom|ButtonUncompleted
  (Utilities|FlowControl|Delay (Variables|Default|GetTimeHoldBeforeDecrement))
  (|ButtonUncompletedOrder
    (:then2
      (Utilities|FlowControl|DoOnce false) ; enters at Reset
    )))

(event Custom|CheckForOutOfFocus
  (Utilities|Time|SetTimerbyFunctionName 0 "CheckForFocus" 1.0))

(event EventBeginPlay
  (Utilities|FlowControl|Delay 0.2)
  (Variables|Default|SetButtonProgress 0.0)
  (Collision|SetCollisionEnabled (Variables|Default|GetConeOverlapSKM) "QueryOnly")
  (bind _as_bp_first_person_character (CallFunction|StorePlayerCharacterRef))
  (bind _taskmanager (Variables|/Game/FirstPerson/Blueprints/BP_FirstPersonCharacter.BP_FirstPersonCharacter_C|GetTaskManager _as_bp_first_person_character)
    (:then
      (|AssignRemoteDoorIDComplete_Dispatcher_2 _taskmanager))
    (:else)))

(event EventActorLoaded
  (if (Variables|Default|GetButtonCompleted?)
    (Rendering|Material|SetVectorParameterValue (Variables|Default|GetDMI_ButtonEmissive) "ButtonColor" (Variables|Default|GetCompletedColor) :!class /Script/Engine.MaterialInstanceDynamic)
    (Rendering|Material|SetScalarParameterValue (Variables|Default|GetDMI_ThermalPanel) "TransitionValue" 1.0 :!class /Script/Engine.MaterialInstanceDynamic)
    (else
      (Rendering|Material|SetVectorParameterValue (Variables|Default|GetDMI_ButtonEmissive) "ButtonColor" (Variables|Default|GetOffColor) :!class /Script/Engine.MaterialInstanceDynamic)
      (Rendering|Material|SetScalarParameterValue (Variables|Default|GetDMI_ThermalPanel) "TransitionValue" 0.0 :!class /Script/Engine.MaterialInstanceDynamic))))

(event EventInFocus
  (if (Variables|Default|GetAssignToTL_Dispatcher?)
    _
    (else
      (|AssignToTeleLumenDispatcher)))
  (if (not (Variables|Default|GetButtonCompleted?))
    (CallFunction|StorePlayerCharacterRef)
    (Variables|Default|SetInFocus? true)
    (if (not (Variables|Default|GetButtonFull?))
      (Variables|Default|SetHasBeenInteracted? true)
      (Utilities|Time|SetTimerbyFunctionName 0 "Increment Focus Progress" 0.01))))

(event EventInteracted
  (bind _asbp_first_person_character (Utilities|Casting|CastToBP_FirstPersonCharacter (Game|GetPlayerCharacter 0)))
  (Variables|Default|SetAs%20BP%20First%20Person%20Character _asbp_first_person_character)
  (Variables|Default|SetHasBeenInteracted? true)
  (Utilities|Time|SetTimerbyFunctionName 0 "Increment Button Progress" 0.01))

(event EventOutFocus
  (if (not (Variables|Default|GetButtonCompleted?))
    (CallFunction|StorePlayerCharacterRef)
    (Variables|Default|SetInFocus? false)
    (if (not (Variables|Default|GetButtonFull?))
      (Variables|Default|SetHasBeenInteracted? false)
      (Utilities|Time|SetTimerbyFunctionName 0 "Increment Focus Progress" 0.01))))

(fn ConstructionScript
  (bind _dmi_buttonemissive (Variables|Default|GetDMI_ButtonEmissive))
  (bind _buttonfull_ (Variables|Default|GetButtonFull?))
  (|CallParentFunction)
  (CallFunction|CheckDMIIsValid)
  (Rendering|Material|SetMaterial (Variables|Default|GetInteractableMesh) 0 _dmi_buttonemissive)
  (Rendering|Material|SetVectorParameterValue _dmi_buttonemissive "ButtonColor" (Math|Color|SelectColor (Variables|Default|GetOnColor) (Variables|Default|GetOffColor) _buttonfull_) :!class /Script/Engine.MaterialInstanceDynamic)
  (Rendering|Material|SetScalarParameterValue (Variables|Default|GetDMI_ThermalPanel) "TransitionValue" (Math|Float|SelectFloat 1.0 0.0 _buttonfull_) :!class /Script/Engine.MaterialInstanceDynamic))

(fn IncrementButtonProgress
  (if (Variables|Default|GetHasBeenInteracted?)
    (bind _output_get (Variables|Default|SetLookingAtButton? (>= (Class|KismetMathLibrary|DegAcos (Math|Vector|DotProduct (Math|Vector|GetForwardVector (Variables|/Script/PSJamJan.PSJamJanCharacter|GetFirstPersonCameraComponent (Variables|Default|GetAs%20BP%20First%20Person%20Character))) (Math|Vector|GetForwardVector (Variables|Default|GetArrow)))) (Variables|Default|GetMaxAngle))))
    (if _output_get
      (if (Math|Float|NearlyEqual(Float) (Variables|Default|GetButtonProgress) 1.0 (LocalVariables|GetTolerance))
        (CallFunction|ButtonFull)
        (return)
        (else
          (Variables|Default|SetButtonProgress (Math|Interpolation|FInterptoConstant (Variables|Default|GetButtonProgress) 1.0 (Utilities|Time|GetWorldDeltaSeconds) (LocalVariables|GetInterpSpeed)))
          (Rendering|Material|SetVectorParameterValue (Variables|Default|GetDMI_ButtonEmissive) "ButtonColor" (Math|Color|Lerp(LinearColor) (Variables|Default|GetOffColor) (Variables|Default|GetOnColor) (Variables|Default|GetButtonProgress)) :!class /Script/Engine.MaterialInstanceDynamic)
          (Rendering|Material|SetScalarParameterValue (Variables|Default|GetDMI_ThermalPanel) "TransitionValue" (Variables|Default|GetButtonProgress) :!class /Script/Engine.MaterialInstanceDynamic)))
      (else
        (Variables|Default|SetButtonFull? false :!label _label)
        (Variables|Default|SetHasBeenInteracted? false)
        (if (Math|Float|NearlyEqual(Float) (Variables|Default|GetButtonProgress) 0.0 (LocalVariables|GetTolerance))
          (return)
          (else
            (Variables|Default|SetButtonProgress (Math|Interpolation|FInterptoConstant (Variables|Default|GetButtonProgress) 0.0 (Utilities|Time|GetWorldDeltaSeconds) (LocalVariables|GetInterpSpeed)))
            (Rendering|Material|SetVectorParameterValue (Variables|Default|GetDMI_ButtonEmissive) "ButtonColor" (Math|Color|Lerp(LinearColor) (Variables|Default|GetOffColor) (Variables|Default|GetOnColor) (Variables|Default|GetButtonProgress)) :!class /Script/Engine.MaterialInstanceDynamic)
            (Rendering|Material|SetScalarParameterValue (Variables|Default|GetDMI_ThermalPanel) "TransitionValue" (Variables|Default|GetButtonProgress) :!class /Script/Engine.MaterialInstanceDynamic)))))
    (else
      (goto _label)))
  (bind _returnvalue (Utilities|Time|SetTimerbyFunctionName 0 "Increment Button Progress" 0.01))
  (Variables|Default|SetIncrementButtonProgress _returnvalue))

(fn IncrementFocusProgress
  (bind _output_get (Variables|Default|SetLookingAtButton? (>= (Class|KismetMathLibrary|DegAcos (Math|Vector|DotProduct (Math|Vector|GetForwardVector (Variables|/Script/PSJamJan.PSJamJanCharacter|GetFirstPersonCameraComponent (Variables|Default|GetAs%20BP%20First%20Person%20Character))) (Math|Vector|GetForwardVector (Variables|Default|GetArrow)))) (Variables|Default|GetMaxAngle))))
  (if _output_get
    (bind _telelumenref (CallFunction|StoreTelelumenRef))
    (if (>= (Variables|/Game/Interactables/EquipmentPickups/Lights/TeleLumen/BP_TeleLumenPickup.BP_TeleLumenPickup_C|GetDynamicIntensity _telelumenref) (Variables|Default|GetMinDynamicIntensity))
      (if (Math|Float|NearlyEqual(Float) (Variables|Default|GetButtonProgress) 1.0 (LocalVariables|GetTolerance))
        (CallFunction|ButtonFull)
        (return)
        (else
          (Variables|Default|SetButtonProgress (Math|Interpolation|FInterptoConstant (Variables|Default|GetButtonProgress) 1.0 (Utilities|Time|GetWorldDeltaSeconds) (LocalVariables|GetInterpSpeed)))
          (Rendering|Material|SetVectorParameterValue (Variables|Default|GetDMI_ButtonEmissive) "ButtonColor" (Math|Color|Lerp(LinearColor) (Variables|Default|GetOffColor) (Variables|Default|GetOnColor) (Variables|Default|GetButtonProgress)) :!class /Script/Engine.MaterialInstanceDynamic)
          (Rendering|Material|SetScalarParameterValue (Variables|Default|GetDMI_ThermalPanel) "TransitionValue" (Variables|Default|GetButtonProgress) :!class /Script/Engine.MaterialInstanceDynamic)))
      (else
        (Variables|Default|SetButtonFull? false :!label _label)
        (if (Math|Float|NearlyEqual(Float) (Variables|Default|GetButtonProgress) 0.0 (LocalVariables|GetTolerance))
          (return)
          (else
            (Variables|Default|SetButtonProgress (Math|Interpolation|FInterptoConstant (Variables|Default|GetButtonProgress) 0.0 (Utilities|Time|GetWorldDeltaSeconds) (LocalVariables|GetInterpSpeed)))
            (Rendering|Material|SetVectorParameterValue (Variables|Default|GetDMI_ButtonEmissive) "ButtonColor" (Math|Color|Lerp(LinearColor) (Variables|Default|GetOffColor) (Variables|Default|GetOnColor) (Variables|Default|GetButtonProgress)) :!class /Script/Engine.MaterialInstanceDynamic)
            (Rendering|Material|SetScalarParameterValue (Variables|Default|GetDMI_ThermalPanel) "TransitionValue" (Variables|Default|GetButtonProgress) :!class /Script/Engine.MaterialInstanceDynamic)))))
    (else
      (goto _label)))
  (bind _returnvalue (Utilities|Time|SetTimerbyFunctionName 0 "Increment Focus Progress" 0.01))
  (Variables|Default|SetIncrementFocusProgress _returnvalue))

(fn StoreTelelumenRef
  (Variables|Default|GetTeleLumenRef
    (:then
      _)
    (:else
      (bind _returnvalue (Actor|GetActorOfClass "/Game/Interactables/EquipmentPickups/Lights/TeleLumen/BP_TeleLumenPickup.BP_TeleLumenPickup_C"))
      (Utilities|IsValid _returnvalue
        (:Is%20Valid
          (Variables|Default|SetTeleLumenRef _returnvalue)))))
  (return (Variables|Default|GetTeleLumenRef)))

(fn StorePlayerCharacterRef
  (Variables|Default|GetAs%20BP%20First%20Person%20Character
    (:then
      _)
    (:else
      (bind _asbp_first_person_character (Utilities|Casting|CastToBP_FirstPersonCharacter (Game|GetPlayerCharacter 0)))
      (Variables|Default|SetAs%20BP%20First%20Person%20Character _asbp_first_person_character)))
  (return (Variables|Default|GetAs%20BP%20First%20Person%20Character)))

(fn CheckforFocus
  (bind _buttoncompleted_ (Variables|Default|GetButtonCompleted?))
  (bind _buttonfull_ (Variables|Default|GetButtonFull?))
  (bind _infocus_ (Variables|Default|GetInFocus?))
  (bind _returnvalue (not _buttoncompleted_))
  (Development|PrintString (Utilities|String|Append "CheckForFocus:" "   " (Utilities|String|ToString(Boolean) _returnvalue) "   " (Utilities|String|ToString(Boolean) _buttonfull_) "   " (Utilities|String|ToString(Boolean) _infocus_)))
  (if _returnvalue
    (if _buttonfull_
      (if _infocus_
        (Utilities|Time|SetTimerbyFunctionName 0 "CheckForFocus" 0.5)
        (else
          (CallFunction|ButtonUncompleted)
          (return))))))

(fn CheckDMIIsValid
  (Variables|Default|GetDMI_ButtonEmissive
    (:then
      _)
    (:else
      (bind _returnvalue (Rendering|Material|CreateDynamicMaterialInstance (Rendering|Material|GetMaterial (Variables|Default|GetInteractableMesh) 0) "None" "None" :!class /Script/Engine.KismetMaterialLibrary))
      (Variables|Default|SetDMI_ButtonEmissive _returnvalue)
      (Rendering|Material|SetMaterial (Variables|Default|GetInteractableMesh) 0 (Variables|Default|GetDMI_ButtonEmissive))))
  (Variables|Default|GetDMI_ThermalPanel
    (:then
      _)
    (:else
      (bind _returnvalue_2 (Rendering|Material|CreateDynamicMaterialInstance (Rendering|Material|GetMaterial (Variables|Default|GetPanel_thermalbar) 0) "None" "None" :!class /Script/Engine.KismetMaterialLibrary))
      (Variables|Default|SetDMI_ThermalPanel _returnvalue_2)
      (Rendering|Material|SetMaterial (Variables|Default|GetPanel_thermalbar) 0 (Variables|Default|GetDMI_ThermalPanel))))
  (return))

(event Custom|RemoteDoorID_Completed_Event
  (params (RemoteDoorID :type Integer))
  (if (== RemoteDoorID (Variables|Default|GetRemoteDoorID))
    (Variables|Default|SetButtonCompleted? true)
    (Variables|Default|SetHasBeenInteracted? true)
    (Variables|Default|SetButtonFull? true)
    (Variables|Default|SetButtonDecrements? false)
    (Rendering|Material|SetVectorParameterValue (Variables|Default|GetDMI_ButtonEmissive) "ButtonColor" (Variables|Default|GetCompletedColor) :!class /Script/Engine.MaterialInstanceDynamic)
    (Rendering|Material|SetScalarParameterValue (Variables|Default|GetDMI_ThermalPanel) "TransitionValue" 1.0 :!class /Script/Engine.MaterialInstanceDynamic)))

(event Custom|DynamicIntensityChanged_Event
  (params (NewDynamicIntensity :type Float%20%28double-precision%29))
  (if (not (Variables|Default|GetButtonCompleted?))
    (if (Variables|Default|GetInFocus?)
      (Utilities|Time|SetTimerbyFunctionName 0 "Increment Focus Progress" 0.01))))

(fn ReturnFocusCenter
  (return (Transformation|GetWorldLocation (Variables|Default|GetInteractableMesh))))