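; BP_RadomeControlPanel is an interactable radome control panel that plays a timed radar start-up audio sequence when used.
; On interaction it runs the parent logic, plays calibrating then radar-on sounds at the mesh location, and after a further delay plays the Boss 3 sound in 2D.
; BeginPlay caches a reference to the walkie-talkie actor, though this graph never uses it afterwards.
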(event EventBeginPlay
  (bind _returnvalue (Actor|GetActorOfClass "/Game/Interactables/EquipmentPickups/BP_WalkieTalkie.BP_WalkieTalkie_C"))
  (Variables|Default|Setwalkietalkie _returnvalue))

(event Collision|EventActorBeginOverlap
  (params (OtherActor :type Actor%20Object%20Reference)))

(event EventTick
  (params (DeltaSeconds :type Float%20%28single-precision%29)))

(event EventInteracted
  (|CallParentFunction)
  (Audio|PlaySoundatLocation "/Game/Sounds/General_SFX/Radar/S_calibrating_Cue.S_calibrating_Cue" (Transformation|GetWorldLocation (Variables|Default|GetInteractableMesh)) "0, 0, 0" 1.0 1.0 0.0 0 0 0 0)
  (Utilities|FlowControl|Delay 1.639)
  (Audio|PlaySoundatLocation "/Game/Sounds/General_SFX/Radar/S_radar_on_Cue.S_radar_on_Cue" (Transformation|GetWorldLocation (Variables|Default|GetInteractableMesh)) "0, 0, 0" 1.0 1.0 0.0 0 0 0 0)
  (Utilities|FlowControl|Delay 5.0)
  (Audio|PlaySound2D "/Game/Sounds/VoiceActing/Boss/S_Boss_3.S_Boss_3" 1.0 1.0 0.0 0 0))

(fn ConstructionScript
  (|CallParentFunction))