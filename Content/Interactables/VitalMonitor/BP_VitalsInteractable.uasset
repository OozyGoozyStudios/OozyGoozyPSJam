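; BP_VitalsInteractable is an interactable that plays a timed vitals scan on the player when used.
; It starts with the Scanning and ThumbsUp components hidden.
; On interaction it runs the parent logic, hides StencilMesh, freezes first-person character movement and shows Scanning for a short delay.
; It then swaps to ThumbsUp, plays a radio beep at the Plane's location and restores movement.
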(event EventBeginPlay
  (Rendering|SetVisibility (Variables|Default|GetScanning) false false)
  (Rendering|SetVisibility (Variables|Default|GetThumbsUp) false false))

(event EventInteracted
  (|CallParentFunction)
  (Rendering|SetVisibility (Variables|Default|GetStencilMesh) false false)
  (bind _asbp_first_person_character (Utilities|Casting|CastToBP_FirstPersonCharacter (Game|GetPlayerCharacter 0)))
  (Default|DisableMovement _asbp_first_person_character)
  (Rendering|SetVisibility (Variables|Default|GetScanning) true false)
  (Utilities|FlowControl|Delay 3.0)
  (Rendering|SetVisibility (Variables|Default|GetScanning) false false)
  (Rendering|SetVisibility (Variables|Default|GetThumbsUp) true false)
  (Audio|PlaySoundatLocation "/Game/Sounds/General_SFX/Radio_Beeps/S_radio_beep_G.S_radio_beep_G" (Transformation|GetWorldLocation (Variables|Default|GetPlane)) "0, 0, 0" 1.0 1.0 0.0 0 0 0 0)
  (Default|EnableMovement _asbp_first_person_character))

(fn ConstructionScript
  (|CallParentFunction))