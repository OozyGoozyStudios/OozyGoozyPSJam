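; BP_TapeCassette is a collectable interactable cassette tape that displays its name on a widget component.
; BeginPlay flags it for whole-object pickup and writes TapeName into its WBP_TapeText widget.
; On Interacted, it runs the parent logic, adds the tape name to the first-person character and shows a WBP_CollectableAdded notification with the name and collectable type.
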(event EventInteracted
  (|CallParentFunction)
  (bind _asbp_first_person_character (Utilities|Casting|CastToBP_FirstPersonCharacter (Game|GetPlayerCharacter 0))
    (:then
      (Default|AddTapeCassette _asbp_first_person_character (Variables|Default|GetTapeName))
      (bind _returnvalue (UserInterface|CreateWidget "/Game/Sounds/Collectables/WBP_CollectableAdded.WBP_CollectableAdded_C" 0 (Variables|Default|GetTapeName) (Variables|Default|GetCollectableType)))
      (UserInterface|Viewport|AddtoViewport _returnvalue 0))
    (:CastFailed
      (Development|PrintString "Failed to Cast to BP_FirstPersonCharacter --BP_TapeCassette--Interacted"))))

(event EventBeginPlay
  (|CallParentFunction)
  (Variables|Default|SetPickUpWholeObject? true)
  (bind _aswbp_tape_text (Utilities|Casting|CastToWBP_TapeText (UserInterface|GetWidget (Variables|Default|GetTapeText))))
  (Variables|/Game/Interactables/TapeCasettes/WBP_TapeText.WBP_TapeText_C|SetTapeName _aswbp_tape_text (Utilities|Text|ToText(Name) (Variables|Default|GetTapeName)))
  (Rendering|Components|TextRender|SetText (Variables|/Game/Interactables/TapeCasettes/WBP_TapeText.WBP_TapeText_C|GetTXT_TapeText _aswbp_tape_text) (Utilities|Text|ToText(Name) (Variables|Default|GetTapeName))))

(fn ConstructionScript)