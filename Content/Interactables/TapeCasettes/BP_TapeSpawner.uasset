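; BP_TapeSpawner places a collectible tape cassette in the level, unless the player already has that tape.
; On BeginPlay it waits briefly, then checks the first-person character's CollectedTapes for its TapeName.
; If the name is absent, it spawns a BP_TapeCassette at its root transform and passes the TapeName to it.
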(event EventBeginPlay
  (Utilities|FlowControl|Delay 0.2)
  (bind _asbp_first_person_character (Utilities|Casting|CastToBP_FirstPersonCharacter (Game|GetPlayerCharacter 0)))
  (if (not (Utilities|Array|ContainsItem (Variables|/Game/FirstPerson/Blueprints/BP_FirstPersonCharacter.BP_FirstPersonCharacter_C|GetCollectedTapes _asbp_first_person_character) (Variables|Default|GetTapeName)))
    (Game|SpawnActorfromClass "/Game/Interactables/TapeCasettes/BP_TapeCassette.BP_TapeCassette_C" (Transformation|GetWorldTransform (Variables|Default|GetDefaultSceneRoot)) "Undefined" "MultiplyWithRoot" 0 (Variables|Default|GetTapeName) 0)))

(fn ConstructionScript)