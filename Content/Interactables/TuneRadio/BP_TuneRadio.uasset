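; Interactable tuning radio that sends the player into a map view and signal-scrubbing sequence tied to task-list objectives.
; Interacting snaps BP_RadioCam to the player's view, moves it to the map and locks movement.
; On the camera's return event, BP_TuneRadioComputer starts scrubbing, or plays a timed tune attempt if the radome is offline, completing that task.
; The construction script duplicates the radio mesh as a hidden highlight outline.
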(event Custom|SetNewAssociatedTask
  (params (NewTaskWidget :type WBP%20Individual%20Task%20Class%20Reference))
  (Variables|Default|SetAssociatedTask NewTaskWidget)
  (CallFunction|InvalidateScrubFreq)
  (Variables|Default|SetCompleted? false)
  (Variables|Default|SetHasBeenInteracted? false)
  (Variables|Default|SetMinigameCompleted? false))

(event Custom|InvalidateScrubFreq
  (Variables|Default|SetWBP_ScrubSignal 0)
  (Variables|/Game/FirstPerson/Blueprints/BP_FirstPersonCharacter.BP_FirstPersonCharacter_C|SetTuningRadio? (Variables|Default|GetPlayerCharacterRef) false))

(event Custom|EnablePlayerMovement
  (Default|EnableMovement (Variables|Default|GetPlayerCharacterRef)))

(event Custom|Returned_Event
  (bind _playercharacterref (Variables|Default|GetPlayerCharacterRef))
  (bind _bp_tuneradiocomputer (Variables|Default|GetBP_TuneRadioComputer))
  (if (Variables|Default|GetRadomeOnline?)
    (Utilities|FlowControl|DoOnce false :!label _label
      (:Completed
        (Utilities|FlowControl|Sequence
          (:then_0
            (Default|ScrubEventStart _bp_tuneradiocomputer self)
            (EventDispatchers|AssignScrubCompleted _bp_tuneradiocomputer (delegate Custom|ScrubCompleted_Event)))
          (:then_1
            (Utilities|FlowControl|Delay 1.0)
            (goto _label Reset)))))
    (else
      (Default|StartTuneAttempt (Variables|Default|GetBP_TuneRadioComputer))
      (Default|DisableMovement _playercharacterref)
      (Variables|/Game/FirstPerson/Blueprints/BP_FirstPersonCharacter.BP_FirstPersonCharacter_C|SetTuningRadio? _playercharacterref false)
      (CallFunction|ChangeStencilVisibility false)
      (Utilities|FlowControl|Delay 3.0)
      (Game|Player|SetViewTargetwithBlend (Game|GetPlayerController 0) (Variables|Default|GetPlayerCharacterRef) 1.5 "VTBlend_EaseInOut" 1.0 false)
      (Default|TuneAttemptEnd (Variables|Default|GetBP_TuneRadioComputer))
      (CallFunction|EnablePlayerMovement)
      (Default|CompleteTask (Variables|/Game/FirstPerson/Blueprints/BP_FirstPersonCharacter.BP_FirstPersonCharacter_C|GetWBP_TaskList (Variables|Default|GetPlayerCharacterRef)) "/Game/TaskSystem/TaskWidgets/TW_AttemptTuneRadio.TW_AttemptTuneRadio_C"))))

(event Custom|ScrubCompleted_Event
  (Utilities|FlowControl|Delay 0.5)
  (Game|Player|SetViewTargetwithBlend (Game|GetPlayerController 0) (Variables|Default|GetPlayerCharacterRef) 1.5 "VTBlend_Linear" 0.0 false))

(event Custom|RadomeOffline
  (Variables|Default|SetAssociatedTask "/Game/TaskSystem/TaskWidgets/TW_AttemptTuneRadio.TW_AttemptTuneRadio_C")
  (Variables|Default|SetRadomeOnline? false))

(event EventBeginPlay
  (bind _returnvalue (Actor|GetActorOfClass "/Game/LevelPrototyping/Blueprints/Lights/BP_TuneRadioComputer.BP_TuneRadioComputer_C"))
  (Variables|Default|SetBP_TuneRadioComputer _returnvalue)
  (bind _returnvalue_2 (Actor|GetActorOfClass "/Game/FirstPerson/Blueprints/BP_FirstPersonCharacter.BP_FirstPersonCharacter_C"))
  (Variables|Default|SetPlayerCharacterRef _returnvalue_2)
  (bind _returnvalue_3 (Actor|GetActorOfClass "/Game/Interactables/TuneRadio/MapSelector/BP_RadioCam.BP_RadioCam_C"))
  (Utilities|IsValid _returnvalue_3
    (:Is%20Valid
      (bind _output_get (Variables|Default|SetRadioCamRef _returnvalue_3))
      (EventDispatchers|AssignReturned _output_get (delegate Custom|Returned_Event)))))

(event EventInteracted
  (bind _playercharacterref (Variables|Default|GetPlayerCharacterRef))
  (|CallParentFunction)
  (Utilities|FlowControl|DoOnce false :!label _label
    (:Completed
      (Utilities|FlowControl|Sequence
        (:then_0
          (bind _hastask_ (CallFunction|EnsureHasTask))
          (if _hastask_
            (Variables|Default|SetHasBeenInteracted? true)
            (CallFunction|InitRadioCam)
            (Utilities|FlowControl|Delay 0.2)
            (Default|MovetoMap (Variables|Default|GetRadioCamRef))
            (Default|DisableMovement _playercharacterref)
            (Variables|/Game/FirstPerson/Blueprints/BP_FirstPersonCharacter.BP_FirstPersonCharacter_C|SetTuningRadio? _playercharacterref true)
            (CallFunction|ChangeStencilVisibility false)))
        (:then_1
          (Utilities|FlowControl|Delay 1.0)
          (goto _label Reset))))))

(event EventTaskUpdated
  (bind _associatedtask (Variables|Default|GetAssociatedTask))
  (if (Variables|Default|GetMinigameCompleted?)
    (if (Utilities|IsValidClass _associatedtask)
      (if (.IsIncrementalTask? (Utilities|GetClassDefaults _associatedtask))
        (bind _asbp_first_person_character (Utilities|Casting|CastToBP_FirstPersonCharacter (Game|GetPlayerCharacter 0)))
        (Default|IncrementTask (Variables|/Game/FirstPerson/Blueprints/BP_FirstPersonCharacter.BP_FirstPersonCharacter_C|GetWBP_TaskList _asbp_first_person_character) (Variables|Default|GetAssociatedTask))
        (else
          (Variables|Default|SetCompleted? true)
          (bind _asbp_first_person_character_2 (Utilities|Casting|CastToBP_FirstPersonCharacter (Game|GetPlayerCharacter 0)))
          (Default|CompleteTask (Variables|/Game/FirstPerson/Blueprints/BP_FirstPersonCharacter.BP_FirstPersonCharacter_C|GetWBP_TaskList _asbp_first_person_character_2) (Variables|Default|GetAssociatedTask)))))))

(fn ConstructionScript
  (bind _ra_801_low (Variables|Default|GetRA_801_Low))
  (|CallParentFunction)
  (bind _returnvalue (AddComponent|AddStaticMeshComponent false (Transformation|GetRelativeTransform _ra_801_low)))
  (bind _output_get (Variables|Default|SetSecondStencil _returnvalue))
  (Components|StaticMesh|SetStaticMesh _output_get (Variables|/Script/Engine.StaticMeshComponent|GetStaticMesh _ra_801_low))
  (for _array_element (Rendering|Material|GetMaterials (Variables|Default|GetSecondStencil))
    (Rendering|Material|SetMaterial (Variables|Default|GetSecondStencil) 0 "/Game/Interactables/MI_InteractableOutline.MI_InteractableOutline")
    (Rendering|SetVisibility _output_get false false)))

(fn ChangeStencilVisibility
  (params (Visible? :type Boolean))
  (|CallParentFunction Visible?)
  (bind _secondstencil (Variables|Default|GetSecondStencil)
    (:then
      (Rendering|SetVisibility _secondstencil Visible? false))
    (:else)))

(fn CreateScrubSignalMinigame
  (Variables|Default|GetWBP_ScrubSignal
    (:then)
    (:else
      (bind _returnvalue (UserInterface|CreateWidget "/Game/Interactables/TuneRadio/UI/WBP_ScrubSignal.WBP_ScrubSignal_C" 0 self))
      (Variables|Default|SetWBP_ScrubSignal _returnvalue)
      (UserInterface|Viewport|AddtoViewport _returnvalue 0))))

(fn InitRadioCam
  (bind _radiocamref (Variables|Default|GetRadioCamRef))
  (Transformation|SetWorldTransform (Variables|/Game/Interactables/TuneRadio/MapSelector/BP_RadioCam.BP_RadioCam_C|GetCamera _radiocamref) (Transformation|GetWorldTransform (Variables|/Script/PSJamJan.PSJamJanCharacter|GetFirstPersonCameraComponent (Variables|Default|GetPlayerCharacterRef))) false true)
  (Game|Player|SetViewTargetwithBlend (Game|GetPlayerController 0) _radiocamref 0.0 "VTBlend_Linear" 0.0 false))