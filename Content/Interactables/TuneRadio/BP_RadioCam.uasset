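; BP_RadioCam is the camera for the tune-radio interactable, with a radio view and a map view.
; MoveToMap starts InterpToTransform, which re-runs on a short timer, easing the camera until it nearly matches the target; nothing here switches back to radio view.
; Once the camera arrives in map mode, Tick spawns a BP_MapSelector if needed and moves it to the Camera-channel trace hit under the cursor.
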(event Custom|MoveToMap
  (Variables|Default|SetCurrentlyViewed? true)
  (Variables|Default|SetOnMapMode? true)
  (Variables|Default|SetCurrentTransform (Transformation|GetWorldTransform (Variables|Default|GetCamera)))
  (Variables|Default|SetMapView (Transformation|GetWorldTransform (Variables|Default|GetMapTransform)))
  (Variables|Default|SetRadioView (Transformation|GetWorldTransform (Variables|Default|GetRadioTransform)))
  (CallFunction|InterptoTransform))

(event EventTick
  (params (DeltaSeconds :type Float%20%28single-precision%29))
  (bind _returnvalue (Game|GetPlayerController 0))
  (if (Math|Boolean|ANDBoolean (Variables|Default|GetCurrentlyViewed?) (Variables|Default|GetArrivedAtLocation?) (Variables|Default|GetOnMapMode?))
    (Variables|Default|GetBP_MapSelector
      (:then
        _)
      (:else
        (bind _returnvalue_2 (Game|SpawnActorfromClass "/Game/Interactables/TuneRadio/BP_MapSelector.BP_MapSelector_C" (Math|Transform|MakeTransform (.WorldLocation (Game|Player|ConvertMouseLocationToWorldSpace _returnvalue)) "0, 0, 0" "1.000000,1.000000,1.000000") "Undefined" 0 0))
        (Variables|Default|SetBP_MapSelector _returnvalue_2)))
    (Transformation|SetWorldLocation (Variables|/Game/Interactables/TuneRadio/BP_MapSelector.BP_MapSelector_C|GetDefaultSceneRoot (Variables|Default|GetBP_MapSelector)) (.impactpoint (.HitResult (Game|Player|GetHitResultUnderCursorbyChannel _returnvalue "TraceTypeQuery2" true))) false false)))

(fn ConstructionScript)

(fn InterptoTransform
  (bind _tolerance (LocalVariables|GetTolerance))
  (bind _tolerance_2 (LocalVariables|GetTolerance))
  (bind _mapview (Variables|Default|GetMapView))
  (bind _radioview (Variables|Default|GetRadioView))
  (Variables|Default|SetArrivedAtLocation? false)
  (if (Variables|Default|GetOnMapMode?)
    (if (Class|KismetMathLibrary|NearlyEqualTransformTransform (Variables|Default|GetCurrentTransform) _mapview _tolerance _tolerance _tolerance)
      (Variables|Default|SetArrivedAtLocation? true)
      (return)
      (else
        (Variables|Default|SetCurrentTransform (Class|KismetMathLibrary|TInterpto (Variables|Default|GetCurrentTransform) _mapview (Utilities|Time|GetWorldDeltaSeconds) (LocalVariables|GetInterpSpeed)))
        (Transformation|SetWorldTransform (Variables|Default|GetCamera) (Class|KismetMathLibrary|TInterpto (Variables|Default|GetCurrentTransform) _mapview (Utilities|Time|GetWorldDeltaSeconds) (LocalVariables|GetInterpSpeed)) false false)
        (Utilities|Time|SetTimerbyFunctionName 0 "InterpToTransform" 0.01)))
    (elif (Class|KismetMathLibrary|NearlyEqualTransformTransform (Variables|Default|GetCurrentTransform) _radioview _tolerance_2 _tolerance_2 _tolerance_2)
      (Variables|Default|SetArrivedAtLocation? true)
      (return)
      (else
        (Variables|Default|SetCurrentTransform (Class|KismetMathLibrary|TInterpto (Variables|Default|GetCurrentTransform) _radioview (Utilities|Time|GetWorldDeltaSeconds) (LocalVariables|GetInterpSpeed)))
        (Transformation|SetWorldTransform (Variables|Default|GetCamera) (Class|KismetMathLibrary|TInterpto (Variables|Default|GetCurrentTransform) _radioview (Utilities|Time|GetWorldDeltaSeconds) (LocalVariables|GetInterpSpeed)) false false)
        (Utilities|Time|SetTimerbyFunctionName 0 "InterpToTransform" 0.01)))))