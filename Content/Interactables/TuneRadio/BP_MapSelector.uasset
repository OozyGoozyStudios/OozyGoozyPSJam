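; BP_MapSelector is a map cursor sphere in the TuneRadio interactable, built to blink while it overlaps a BP_BoardLight.
; The construction script gives the sphere mesh a dynamic instance of M_MapSelector, and collider overlaps set the BlinkCursor flag.
; The Blink Cursor function alternates material opacity on a self-renewing short timer, restoring it when the flag clears.
; Nothing in this file makes the initial call to that function.
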(event OnComponentBeginOverlap(SphereCollider)
  (params (OverlappedComponent :type Primitive%20Component%20Object%20Reference) (OtherActor :type Actor%20Object%20Reference) (OtherComp :type Primitive%20Component%20Object%20Reference) (OtherBodyIndex :type Integer) (bFromSweep :type Boolean) (SweepResult :type Hit%20Result%20Structure%20%28by%20ref%29))
  (Utilities|Casting|CastToBP_BoardLight OtherActor)
  (Variables|Default|SetBlinkCursor? true))

(event OnComponentEndOverlap(SphereCollider)
  (params (OverlappedComponent :type Primitive%20Component%20Object%20Reference) (OtherActor :type Actor%20Object%20Reference) (OtherComp :type Primitive%20Component%20Object%20Reference) (OtherBodyIndex :type Integer))
  (Utilities|Casting|CastToBP_BoardLight OtherActor)
  (Variables|Default|SetBlinkCursor? false))

(fn ConstructionScript
  (bind _returnvalue (Rendering|Material|CreateDynamicMaterialInstance "/Game/Interactables/TuneRadio/M_MapSelector.M_MapSelector" "None" "None" :!class /Script/Engine.KismetMaterialLibrary))
  (Variables|Default|SetDMI_MapSelector _returnvalue)
  (Rendering|Material|SetMaterial (Variables|Default|GetSphereMesh) 0 _returnvalue))

(fn BlinkCursor
  (if (Variables|Default|GetBlinkCursor?)
    (if (Variables|Default|GetCursorOn?)
      (Rendering|Material|SetScalarParameterValue (Variables|Default|GetDMI_MapSelector) "Opacity" 0.1 :!class /Script/Engine.MaterialInstanceDynamic)
      (Variables|Default|SetCursorOn? false)
      (Utilities|Time|SetTimerbyFunctionName 0 "Blink Cursor" 0.01)
      (else
        (Rendering|Material|SetScalarParameterValue (Variables|Default|GetDMI_MapSelector) "Opacity" 0.5 :!class /Script/Engine.MaterialInstanceDynamic)
        (Variables|Default|SetCursorOn? true)
        (Utilities|Time|SetTimerbyFunctionName 0 "Blink Cursor" 0.01)))
    (else
      (Rendering|Material|SetScalarParameterValue (Variables|Default|GetDMI_MapSelector) "Opacity" 0.5 :!class /Script/Engine.MaterialInstanceDynamic)
      (Variables|Default|SetCursorOn? true)
      (return))))