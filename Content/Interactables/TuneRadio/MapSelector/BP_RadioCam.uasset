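; Radio camera that glides between a radio view and an interactive world board map for selecting board lights.
; InterpToTransform re-arms itself by timer, easing the camera until it is within tolerance of the target.
; On arrival at the map, Tick spawns a BP_MapSelector and keeps it under the cursor.
; Selector hover and click events feed WBP_BoardScreen, found through a retrying BP_WorldBoard lookup, and a click returns to the radio.
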(event Custom|MonitorScaled_Event
  (params (ScaledUp? :type Boolean))
  (if ScaledUp?
    (bind _as_wbp_board_screen (Variables|Default|GetAs%20WBP%20Board%20Screen)
      (:then
        _)
      (:else
        (CallFunction|StoreWorldBoardRef)))
    (Default|StartSelector _as_wbp_board_screen)))

(event Custom|ReturnToRadio
  (Variables|Default|SetOnMapMode? false)
  (CallFunction|InterptoTransform)
  (Default|MapSelectorChange (Variables|Default|GetWorldBoardRef) false))

(event Custom|UnhoveredLight_Event
  (params (BoardLightRef :type BP%20Board%20Light%20Object%20Reference))
  (bind _as_wbp_board_screen (Variables|Default|GetAs%20WBP%20Board%20Screen)
    (:then
      (Default|CursorLeftRange _as_wbp_board_screen))
    (:else
      _))
  (Variables|Default|SetWBP_HoveredBoardLight 0))

(event Custom|ClickedLight_Event
  (params (ClickedBoardLight :type BP%20Board%20Light%20Object%20Reference))
  (CallFunction|ReturntoRadio)
  (Actor|DestroyActor (Variables|Default|GetBP_MapSelector))
  (Default|LightClicked (Variables|Default|GetAs%20WBP%20Board%20Screen)))

(event Custom|MoveToMap
  (Audio|PlaySound2D "/Game/Sounds/General_SFX/MapBoard/S_interactivemap_startup.S_interactivemap_startup" 1.0 1.0 0.0 0 0)
  (Variables|Default|SetCurrentlyViewed? true)
  (Variables|Default|SetOnMapMode? true)
  (Variables|Default|SetCurrentTransform (Transformation|GetWorldTransform (Variables|Default|GetCamera)))
  (Variables|Default|SetMapView (Transformation|GetWorldTransform (Variables|Default|GetMapTransform)))
  (Variables|Default|SetRadioView (Transformation|GetWorldTransform (Variables|Default|GetRadioTransform)))
  (CallFunction|InterptoTransform))

(event Custom|CreateMapSelector
  (params (SpawnLocation :type Vector))
  (Default|MapSelectorChange (Variables|Default|GetWorldBoardRef) true)
  (bind _returnvalue (Game|SpawnActorfromClass "/Game/Interactables/TuneRadio/MapSelector/BP_MapSelector.BP_MapSelector_C" (Math|Transform|MakeTransform SpawnLocation "0, 0, 0" "1.000000,1.000000,1.000000") "Undefined" 0 0))
  (bind _output_get (Variables|Default|SetBP_MapSelector _returnvalue))
  (EventDispatchers|AssignClickedLight _output_get (delegate Custom|ClickedLight_Event))
  (EventDispatchers|AssignHoveredLight _output_get (delegate Custom|HoveredLight_Event))
  (EventDispatchers|AssignUnhoveredLight _output_get (delegate Custom|UnhoveredLight_Event)))

(event Custom|HoveredLight_Event
  (params (BoardLightRef :type BP%20Board%20Light%20Object%20Reference))
  (bind _as_wbp_board_screen (Variables|Default|GetAs%20WBP%20Board%20Screen)
    (:then
      (Default|LightHovered _as_wbp_board_screen BoardLightRef))
    (:else)))

(event EventTick
  (params (DeltaSeconds :type Float%20%28single-precision%29))
  (bind _returnvalue (Game|GetPlayerController 0))
  (if (Math|Boolean|ANDBoolean (Variables|Default|GetCurrentlyViewed?) (Variables|Default|GetArrivedAtLocation?) (Variables|Default|GetOnMapMode?))
    (Variables|Default|GetBP_MapSelector
      (:then
        _)
      (:else
        (CallFunction|CreateMapSelector (.WorldLocation (Game|Player|ConvertMouseLocationToWorldSpace _returnvalue)))))
    (Transformation|SetWorldLocation (Variables|/Game/Interactables/TuneRadio/MapSelector/BP_MapSelector.BP_MapSelector_C|GetDefaultSceneRoot (Variables|Default|GetBP_MapSelector)) (.impactpoint (.HitResult (Game|Player|GetHitResultUnderCursorbyChannel _returnvalue "TraceTypeQuery2" true))) false false)))

(event EventBeginPlay
  (CallFunction|StoreWorldBoardRef)
  (EventDispatchers|AssignMonitorScaled (Variables|Default|GetWorldBoardRef) (delegate Custom|MonitorScaled_Event)))

(fn ConstructionScript)

(fn InterptoTransform
  (bind _tolerance (LocalVariables|GetTolerance))
  (bind _tolerance_2 (LocalVariables|GetTolerance))
  (bind _mapview (Variables|Default|GetMapView))
  (bind _radioview (Variables|Default|GetRadioView))
  (Variables|Default|SetArrivedAtLocation? false)
  (if (Variables|Default|GetOnMapMode?)
    (if (Class|KismetMathLibrary|NearlyEqualTransformTransform (Variables|Default|GetCurrentTransform) _mapview _tolerance _tolerance _tolerance)
      (Variables|Default|SetArrivedAtLocation? true)
      (return)
      (else
        (Variables|Default|SetCurrentTransform (Class|KismetMathLibrary|TInterpto (Variables|Default|GetCurrentTransform) _mapview (Utilities|Time|GetWorldDeltaSeconds) (LocalVariables|GetInterpSpeed)))
        (Transformation|SetWorldTransform (Variables|Default|GetCamera) (Class|KismetMathLibrary|TInterpto (Variables|Default|GetCurrentTransform) _mapview (Utilities|Time|GetWorldDeltaSeconds) (LocalVariables|GetInterpSpeed)) false false)
        (Utilities|Time|SetTimerbyFunctionName 0 "InterpToTransform" 0.01)))
    (elif (Class|KismetMathLibrary|NearlyEqualTransformTransform (Variables|Default|GetCurrentTransform) _radioview _tolerance_2 _tolerance_2 _tolerance_2)
      (Variables|Default|SetArrivedAtLocation? true)
      (Default|CallReturned)
      (return)
      (else
        (Variables|Default|SetCurrentTransform (Class|KismetMathLibrary|TInterpto (Variables|Default|GetCurrentTransform) _radioview (Utilities|Time|GetWorldDeltaSeconds) (LocalVariables|GetInterpSpeed)))
        (Transformation|SetWorldTransform (Variables|Default|GetCamera) (Class|KismetMathLibrary|TInterpto (Variables|Default|GetCurrentTransform) _radioview (Utilities|Time|GetWorldDeltaSeconds) (LocalVariables|GetInterpSpeed)) false false)
        (Utilities|Time|SetTimerbyFunctionName 0 "InterpToTransform" 0.01)))))

(fn SetWidgetScreenPosition
  (bind _returnvalue (Game|GetPlayerController 0))
  (bind (_locationx _locationy) (Game|Player|GetMousePosition _returnvalue))
  (Class|UserWidget|SetPositioninViewport (Variables|Default|GetWBP_HoveredBoardLight) (Math|Vector2D|MakeVector2D (Math|Float|Clamp(Float) _locationx 0.0 1.5e+03) (Math|Float|Clamp(Float) _locationy 0.0 7.5e+02)) true))

(fn StoreWorldBoardRef
  (bind _returnvalue (Actor|GetActorOfClass "/Game/LevelPrototyping/Blueprints/MapBoard/BP_WorldBoard.BP_WorldBoard_C"))
  (bind _output_get (Variables|Default|SetWorldBoardRef _returnvalue))
  (Utilities|IsValid _output_get
    (:Is%20Valid
      (bind _aswbp_board_screen (Utilities|Casting|CastToWBP_BoardScreen (UserInterface|GetWidget (Variables|/Game/LevelPrototyping/Blueprints/MapBoard/BP_WorldBoard.BP_WorldBoard_C|GetBoardScreen _output_get))))
      (bind _output_get_2 (Variables|Default|SetAs%20WBP%20Board%20Screen _aswbp_board_screen))
      (Utilities|IsValid _output_get_2
        (:Is%20Valid
          (return))
        (:Is%20Not%20Valid
          _)))
    (:Is%20Not%20Valid
      _))
  (Utilities|Time|SetTimerbyFunctionName 0 "Store World Board Ref" 0.5))