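; BP_MapSelector is the cursor that hovers and selects board lights on the tune radio's world map board.
; Its sphere overlaps track the current BP_BoardLight, broadcast hover and unhover, and switch a dynamic material between on and off opacity.
; Releasing or canceling UseEquipment over a light with the required tune status, while the board screen is scaled, disables the selector's input and broadcasts the click.
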(event OnComponentBeginOverlap(SphereCollider)
  (params (OverlappedComponent :type Primitive%20Component%20Object%20Reference) (OtherActor :type Actor%20Object%20Reference) (OtherComp :type Primitive%20Component%20Object%20Reference) (OtherBodyIndex :type Integer) (bFromSweep :type Boolean) (SweepResult :type Hit%20Result%20Structure%20%28by%20ref%29))
  (bind _asbp_board_light (Utilities|Casting|CastToBP_BoardLight OtherActor))
  (Variables|Default|SetCurrentBoardLight _asbp_board_light)
  (Variables|Default|SetOnBoardLight? true)
  (CallFunction|BlinkCursor)
  (Default|CallHoveredLight _asbp_board_light))

(event OnComponentEndOverlap(SphereCollider)
  (params (OverlappedComponent :type Primitive%20Component%20Object%20Reference) (OtherActor :type Actor%20Object%20Reference) (OtherComp :type Primitive%20Component%20Object%20Reference) (OtherBodyIndex :type Integer))
  (bind _asbp_board_light (Utilities|Casting|CastToBP_BoardLight OtherActor))
  (Variables|Default|SetCurrentBoardLight 0)
  (Variables|Default|SetOnBoardLight? false)
  (CallFunction|BlinkCursor)
  (Default|CallUnhoveredLight _asbp_board_light))

(event Input|EnhancedActionEvents|EnhancedInputActionIA_UseEquipment
  (params (ActionValue :type Boolean) (ElapsedSeconds :type Float%20%28double-precision%29) (TriggeredSeconds :type Float%20%28double-precision%29) (InputAction :type Input%20Action%20Object%20Reference :default "/Game/FirstPerson/Input/Actions/IA_UseEquipment.IA_UseEquipment"))
  (:Canceled
    (if (Variables|Default|GetOnBoardLight?) :!label _label
      (if (Variables|/Game/LevelPrototyping/Blueprints/MapBoard/MapMonitor/WBP_BoardScreen.WBP_BoardScreen_C|GetScaled? (Variables|Default|GetAs%20WBP%20Board%20Screen))
        (if (Utilities|Enum|Equal(Enum) (Variables|/Game/LevelPrototyping/Blueprints/MapBoard/BP_BoardLight.BP_BoardLight_C|GetTuneStatus (Variables|Default|GetCurrentBoardLight)) "NewEnumerator1")
          (Input|DisableInput (Game|GetPlayerController 0))
          (Default|CallClickedLight (Variables|Default|GetCurrentBoardLight))))))
  (:Completed
    (goto _label)))

(event EventBeginPlay
  (Variables|Default|SetOnBoardLight? false)
  (CallFunction|BlinkCursor)
  (Input|EnableInput (Game|GetPlayerController 0))
  (bind _returnvalue (Actor|GetActorOfClass "/Game/LevelPrototyping/Blueprints/MapBoard/BP_WorldBoard.BP_WorldBoard_C"))
  (Utilities|IsValid _returnvalue
    (:Is%20Valid
      (Variables|Default|SetAs%20WBP%20Board%20Screen (Variables|/Game/LevelPrototyping/Blueprints/MapBoard/BP_WorldBoard.BP_WorldBoard_C|GetAs%20WBP%20Board%20Screen _returnvalue)))))

(fn ConstructionScript
  (bind _returnvalue (Rendering|Material|CreateDynamicMaterialInstance "/Game/Interactables/TuneRadio/MapSelector/M_MapSelector.M_MapSelector" "None" "None" :!class /Script/Engine.KismetMaterialLibrary))
  (bind _output_get (Variables|Default|SetDMI_MapSelector _returnvalue))
  (Rendering|Material|SetScalarParameterValue _output_get "None" (Variables|Default|GetOffOpacity) :!class /Script/Engine.MaterialInstanceDynamic)
  (Rendering|Material|SetMaterial (Variables|Default|GetSphereMesh) 0 _returnvalue))

(fn BlinkCursor
  (if (Variables|Default|GetOnBoardLight?)
    (Rendering|Material|SetScalarParameterValue (Variables|Default|GetDMI_MapSelector) "Opacity" (Variables|Default|GetOnOpacity) :!class /Script/Engine.MaterialInstanceDynamic)
    (return)
    (else
      (Rendering|Material|SetScalarParameterValue (Variables|Default|GetDMI_MapSelector) "Opacity" (Variables|Default|GetOffOpacity) :!class /Script/Engine.MaterialInstanceDynamic)
      (return))))