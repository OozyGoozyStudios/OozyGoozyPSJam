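; BP_BoilerDoor is an interactable boiler door that players open and close, and that can start locked until equipment is consumed on it.
; Interacting runs the parent logic, then, if unlocked, toggles the door via ChangeDoorState, resets completion and clears its associated task after a short delay.
; ChangeDoorState snaps the mesh rotation, updates the prompt and plays a sound.
; Consuming equipment unlocks the door and resets its interacted flag.
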(event EventInteracted
  (|CallParentFunction)
  (if (not (Variables|Default|GetbLocked?))
    (CallFunction|ChangeDoorState)
    (Variables|Default|SetCompleted? false)
    (Utilities|FlowControl|Delay 1.5)
    (Variables|Default|SetAssociatedTask 0)))

(event EventEquipmentConsumed
  (Variables|Default|SetbLocked? false)
  (Variables|Default|SetHasBeenInteracted? false)
  (Variables|Default|SetUnlocked? true))

(fn ConstructionScript
  (|CallParentFunction))

(fn ChangeDoorState
  (if (Variables|Default|GetbOpen?)
    (Variables|Default|SetbOpen? false)
    (Transformation|SetRelativeRotation (Variables|Default|GetInteractableMesh) (Variables|Default|GetClosed) false false)
    (Variables|Default|SetInteractionPrompt "Open Door")
    (Audio|PlaySoundatLocation "/Game/Sounds/General_SFX/S_close_door.S_close_door" (Transformation|GetWorldLocation (Variables|Default|GetInteractableMesh)) "0, 0, 0" 1.0 1.0 0.0 0 0 0 0)
    (else
      (Variables|Default|SetbOpen? true)
      (Transformation|SetRelativeRotation (Variables|Default|GetInteractableMesh) (Variables|Default|GetOpen) false false)
      (Variables|Default|SetInteractionPrompt "Close Door")
      (Audio|PlaySoundatLocation "/Game/Sounds/General_SFX/S_open_door.S_open_door" (Transformation|GetWorldLocation (Variables|Default|GetInteractableMesh)) "0, 0, 0" 1.0 1.0 0.0 0 0 0 0))))