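; Interactable door that toggles open and closed with rotation, prompt and sound, and can be locked until remotely opened.
; In remote mode it binds to BP_TaskManager dispatchers, counting completed buttons up or down.
; Reaching the required count opens and unlocks it, then reports the ID as completed.
; An optional trigger closes it when the player capsule overlaps, and its state is reapplied silently on BeginPlay and load.
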(event OnComponentBeginOverlap(AutoCloseTrigger)
  (params (OverlappedComponent :type Primitive%20Component%20Object%20Reference) (OtherActor :type Actor%20Object%20Reference) (OtherComp :type Primitive%20Component%20Object%20Reference) (OtherBodyIndex :type Integer) (bFromSweep :type Boolean) (SweepResult :type Hit%20Result%20Structure%20%28by%20ref%29))
  (bind _asbp_first_person_character (Utilities|Casting|CastToBP_FirstPersonCharacter OtherActor))
  (if (== OtherComp (Variables|/Script/Engine.Character|GetCapsuleComponent _asbp_first_person_character))
    (if (Variables|Default|GetbAutoClose?)
      (if (Variables|Default|GetbOpen?)
        (CallFunction|Interacted)))))

(event EventMakeDoorOpen
  (params (PlaySound? :type Boolean))
  (Variables|Default|SetbOpen? true)
  (Transformation|SetRelativeRotation (Variables|Default|GetInteractableMesh) (Variables|Default|GetOpen) false false)
  (Variables|Default|SetInteractionPrompt "Close Door")
  (if PlaySound?
    (Audio|PlaySoundatLocation "/Game/Sounds/General_SFX/S_open_door.S_open_door" (Transformation|GetWorldLocation (Variables|Default|GetInteractableMesh)) "0, 0, 0" 1.0 1.0 0.0 0 0 0 0)))

(event EventMakeDoorClosed
  (params (PlaySound? :type Boolean))
  (Variables|Default|SetbOpen? false)
  (Transformation|SetRelativeRotation (Variables|Default|GetInteractableMesh) (Variables|Default|GetClose) false false)
  (Variables|Default|SetInteractionPrompt "Open Door")
  (if PlaySound?
    (Audio|PlaySoundatLocation "/Game/Sounds/General_SFX/S_close_door.S_close_door" (Transformation|GetWorldLocation (Variables|Default|GetInteractableMesh)) "0, 0, 0" 1.0 1.0 0.0 0 0 0 0)))

(event EventActorLoaded
  (CallFunction|InitializeDoorState))

(event EventInteracted
  (if (Variables|Default|GetbCanBeOpened?)
    (Variables|Default|SetHasBeenInteracted? false)
    (CallFunction|ChangeDoorState)))

(event EventBeginPlay
  (CallFunction|InitializeDoorState)
  (if (Variables|Default|GetIsRemotelyOpened?)
    (Variables|Default|SetbCanBeOpened? false)
    (Variables|Default|SetHasBeenInteracted? true)
    (Variables|Default|SetInteractionPrompt "")
    (bind _returnvalue (Actor|GetActorOfClass "/Game/TaskSystem/BP_TaskManager.BP_TaskManager_C"))
    (Variables|Default|SetTaskManagerRef _returnvalue)
    (|AssignRemoteDoorOpenDispatcher _returnvalue)
    (|AssignRemoteDoorCloseDispatcher _returnvalue)
    (|AssignRemoteDoorCompletedDIspatcher _returnvalue)
    (elif (not (Variables|Default|GetbCanBeOpened?))
      (Variables|Default|SetHasBeenInteracted? true)
      (Variables|Default|SetInteractionPrompt ""))))

(fn ConstructionScript)

(fn ChangeDoorState
  (if (Variables|Default|GetbOpen?)
    (CallFunction|MakeDoorClosed true)
    (else
      (CallFunction|MakeDoorOpen true))))

(fn InitializeDoorState
  (if (Variables|Default|GetbOpen?)
    (CallFunction|MakeDoorOpen false)
    (else
      (CallFunction|MakeDoorClosed false))))

(event Custom|RemoteDoorOpen_Event
  (params (RemoteOpenID :type Integer))
  (bind _currentbuttonscompleted (Variables|Default|GetCurrentButtonsCompleted))
  (if (== RemoteOpenID (Variables|Default|GetRemoteOpenID))
    (if (< (Variables|Default|GetCurrentButtonsCompleted) (Variables|Default|GetRequiredButtonsCompleted))
      (Math|Integer|IncrementInt _currentbuttonscompleted
        (:%20%20
          (if (>= _currentbuttonscompleted (Variables|Default|GetRequiredButtonsCompleted))
            (CallFunction|MakeDoorOpen true)
            (Variables|Default|SetbCanBeOpened? true)
            (Default|RemoteDoorIDCompleted (Variables|Default|GetTaskManagerRef) (Variables|Default|GetRemoteOpenID))))))))

(event Custom|RemoteDoorClose_Event
  (params (RemoteDoorID :type Integer))
  (if (== RemoteDoorID (Variables|Default|GetRemoteOpenID))
    (if (> (Variables|Default|GetCurrentButtonsCompleted) 0)
      (Math|Integer|DecrementInt (Variables|Default|GetCurrentButtonsCompleted)))))

(event Custom|RemoteDoorID_Completed_Event
  (params (RemoteDoorID :type Integer))
  (if (== RemoteDoorID (Variables|Default|GetRemoteOpenID))
    _))

(fn GetDoorCurrentState
  (return (Variables|Default|GetbOpen?)))

(fn GetIsMonsterOpen?
  (return (Variables|Default|GetIsMonsterOpen?)))