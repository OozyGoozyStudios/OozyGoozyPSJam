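; Interactable radar room door, a child of a base door Blueprint, that can be shut and hard-locked.
; ShutRadarDoor closes the door and hard-locks it, which also marks it as already interacted.
; Interacting toggles the door only while it is not hard-locked, clearing the interacted flag first so it can be reused.
; ActorLoaded restores the open or closed pose from the Open state.
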(event Custom|ShutRadarDoor
  (CallFunction|MakeDoorClosed true)
  (CallFunction|SetHardLocked true))

(event EventBeginPlay
  (|CallParentFunction))

(event Collision|EventActorBeginOverlap
  (params (OtherActor :type Actor%20Object%20Reference)))

(event EventTick
  (params (DeltaSeconds :type Float%20%28single-precision%29)))

(event EventInteracted
  (if (not (Variables|Default|GetHardLocked?))
    (Variables|Default|SetHasBeenInteracted? false)
    (CallFunction|ChangeDoorState)))

(event EventActorLoaded
  (if (Variables|Default|GetbOpen?)
    (CallFunction|MakeDoorOpen false)
    (else
      (CallFunction|MakeDoorClosed false))))

(fn ConstructionScript
  (|CallParentFunction))

(fn SetHardLocked
  (params (HardLocked? :type Boolean))
  (Variables|Default|SetHardLocked? HardLocked?)
  (Variables|Default|SetHasBeenInteracted? HardLocked?))