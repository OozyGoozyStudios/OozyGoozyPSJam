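; BP_AntarticaScareDoor is an interactable door that triggers a scripted glass-break scare and then sends the player home.
; On BeginPlay it caches the task manager and first-person character through GetActorOfClass.
; When interacted with, it flags itself as used, disables player movement, and plays the GlassBreakSequence after a short delay.
; A second delay later, it calls ReturnPlayerHome on the task manager, re-fetching that reference if invalid.
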(event EventBeginPlay
  (|CallParentFunction)
  (bind _returnvalue (Actor|GetActorOfClass "/Game/TaskSystem/BP_TaskManager.BP_TaskManager_C"))
  (Variables|Default|SetTaskManagerRef_0 _returnvalue)
  (bind _returnvalue_2 (Actor|GetActorOfClass "/Game/FirstPerson/Blueprints/BP_FirstPersonCharacter.BP_FirstPersonCharacter_C"))
  (Variables|Default|SetCharacterRef _returnvalue_2))

(event Collision|EventActorBeginOverlap
  (params (OtherActor :type Actor%20Object%20Reference)))

(event EventTick
  (params (DeltaSeconds :type Float%20%28single-precision%29)))

(event EventInteracted
  (Variables|Default|SetHasBeenInteracted? true)
  (Default|DisableMovement (Variables|Default|GetCharacterRef))
  (Utilities|FlowControl|Delay 0.25)
  (Sequencer|Player|Play (Variables|/Script/LevelSequence.LevelSequenceActor|GetSequencePlayer (Variables|Default|GetGlassBreakSequence)) :!class /Script/MovieScene.MovieSceneSequencePlayer)
  (Utilities|FlowControl|Delay 1.0)
  (Variables|Default|GetTaskManagerRef_0
    (:then
      _)
    (:else
      (bind _returnvalue (Actor|GetActorOfClass "/Game/TaskSystem/BP_TaskManager.BP_TaskManager_C"))
      (Variables|Default|SetTaskManagerRef_0 _returnvalue)))
  (Default|ReturnPlayerHome (Variables|Default|GetTaskManagerRef_0)))

(fn ConstructionScript
  (|CallParentFunction))