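; Interactable sublevels door that toggles open and closed by snapping mesh rotation, updating its prompt and optionally playing a sound.
; Interaction toggles it only when unlocked, then clears task state after a delay; consuming equipment unlocks it.
; BeginPlay and save loading silently reapply the Open state, while EstablishPrologueDoor and RecloseAndLock force it closed and locked.
; Door-state and monster-open queries are stubs returning false.
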(event Custom|RecloseAndLock
  (CallFunction|MakeDoorClosed false)
  (Variables|Default|SetbLocked? true)
  (Variables|Default|SetHasBeenInteracted? false)
  (Variables|Default|SetUnlocked? false))

(event Custom|EstablishPrologueDoor
  (CallFunction|MakeDoorClosed false)
  (Variables|Default|SetbLocked? true)
  (Variables|Default|SetHasBeenInteracted? false)
  (Variables|Default|SetUnlocked? false))

(event EventBeginPlay
  (if (Variables|Default|GetbOpen?)
    (CallFunction|MakeDoorOpen false)
    (else
      (CallFunction|MakeDoorClosed false))))

(event EventMakeDoorOpen
  (params (PlaySound? :type Boolean))
  (Variables|Default|SetbOpen? true)
  (Transformation|SetRelativeRotation (Variables|Default|GetInteractableMesh) (Variables|Default|GetOpen) false false)
  (Variables|Default|SetInteractionPrompt "Close Sublevels Door")
  (if PlaySound?
    (Audio|PlaySoundatLocation "/Game/Sounds/General_SFX/S_open_door.S_open_door" (Transformation|GetWorldLocation (Variables|Default|GetInteractableMesh)) "0, 0, 0" 1.0 1.0 0.0 0 0 0 0)))

(event EventMakeDoorClosed
  (params (PlaySound? :type Boolean))
  (Variables|Default|SetbOpen? false)
  (Transformation|SetRelativeRotation (Variables|Default|GetInteractableMesh) (Variables|Default|GetClosed) false false)
  (Variables|Default|SetInteractionPrompt "Open Sublevels Door")
  (if PlaySound?
    (Audio|PlaySoundatLocation "/Game/Sounds/General_SFX/S_close_door.S_close_door" (Transformation|GetWorldLocation (Variables|Default|GetInteractableMesh)) "0, 0, 0" 1.0 1.0 0.0 0 0 0 0)))

(event EventInteracted
  (|CallParentFunction)
  (if (not (Variables|Default|GetbLocked?))
    (CallFunction|ChangeDoorState)
    (Utilities|FlowControl|Delay 1.5)
    (Variables|Default|SetCompleted? false)
    (Variables|Default|SetAssociatedTask 0)))

(event EventEquipmentConsumed
  (Variables|Default|SetbLocked? false)
  (Variables|Default|SetHasBeenInteracted? false)
  (Variables|Default|SetUnlocked? true))

(event EventActorLoaded
  (if (Variables|Default|GetbOpen?)
    (CallFunction|MakeDoorOpen false)
    (else
      (CallFunction|MakeDoorClosed false))))

(fn ConstructionScript
  (|CallParentFunction))

(fn ChangeDoorState
  (if (Variables|Default|GetbOpen?)
    (CallFunction|MakeDoorClosed true)
    (else
      (CallFunction|MakeDoorOpen true))))

(fn ComponentstoSave
  (return 0))

(fn GetDoorCurrentState
  (return false))

(fn GetIsMonsterOpen?
  (return false))