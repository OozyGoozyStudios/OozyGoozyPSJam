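; Interactable radome door that the player opens and closes, with optional auto-close and lock support.
; Interaction runs the parent logic, then, if unlocked, toggles the door by snapping mesh rotation, swapping the prompt and playing a sound.
; It then resets completion and clears its associated task after a short delay.
; Consuming equipment unlocks it; the player capsule entering AutoCloseTrigger reuses the interaction to close an open door.
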(event OnComponentBeginOverlap(AutoCloseTrigger)
  (params (OverlappedComponent :type Primitive%20Component%20Object%20Reference) (OtherActor :type Actor%20Object%20Reference) (OtherComp :type Primitive%20Component%20Object%20Reference) (OtherBodyIndex :type Integer) (bFromSweep :type Boolean) (SweepResult :type Hit%20Result%20Structure%20%28by%20ref%29))
  (bind _asbp_first_person_character (Utilities|Casting|CastToBP_FirstPersonCharacter OtherActor))
  (if (== OtherComp (Variables|/Script/Engine.Character|GetCapsuleComponent _asbp_first_person_character))
    (if (Variables|Default|GetbAutoClose?)
      (if (Variables|Default|GetbOpen?)
        (CallFunction|Interacted)))))

(event EventInteracted
  (|CallParentFunction)
  (if (not (Variables|Default|GetbLocked?))
    (CallFunction|ChangeDoorState)
    (Variables|Default|SetCompleted? false)
    (Utilities|FlowControl|Delay 1.5)
    (Variables|Default|SetAssociatedTask 0)))

(event EventEquipmentConsumed
  (Variables|Default|SetbLocked? false)
  (Variables|Default|SetHasBeenInteracted? false)
  (Variables|Default|SetUnlocked? true))

(fn ConstructionScript
  (|CallParentFunction))

(fn ChangeDoorState
  (if (Variables|Default|GetbOpen?)
    (Variables|Default|SetbOpen? false)
    (Transformation|SetRelativeRotation (Variables|Default|GetInteractableMesh) (Variables|Default|GetClosed) false false)
    (Variables|Default|SetInteractionPrompt "Open Door")
    (Audio|PlaySoundatLocation "/Game/Sounds/General_SFX/S_close_door.S_close_door" (Transformation|GetWorldLocation (Variables|Default|GetInteractableMesh)) "0, 0, 0" 1.0 1.0 0.0 0 0 0 0)
    (else
      (Variables|Default|SetbOpen? true)
      (Transformation|SetRelativeRotation (Variables|Default|GetInteractableMesh) (Variables|Default|GetOpen) false false)
      (Variables|Default|SetInteractionPrompt "Close Door")
      (Audio|PlaySoundatLocation "/Game/Sounds/General_SFX/S_open_door.S_open_door" (Transformation|GetWorldLocation (Variables|Default|GetInteractableMesh)) "0, 0, 0" 1.0 1.0 0.0 0 0 0 0))))