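; BP_BunkerDoor is an interactable bunker door that responds to remote-open broadcasts and reports its opening as a task.
; On BeginPlay it finds BP_TaskManager and binds to its RemoteDoorOpen dispatcher.
; When the RemoteOpenID check passes, it completes the OpenBunkerDoor task with autosave, then reports that ID as completed to the manager.
; The graph contains no door movement or animation, only task bookkeeping.
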(event Custom|RemoteDoorOpen_Event
  (params (RemoteOpenID :type Integer))
  (if (== RemoteOpenID (Variables|Default|GetRemoteOpenID))
    (CallFunction|BunkerDoorOpened)
    (Default|RemoteDoorIDCompleted (Variables|Default|GetTaskManagerRef) (Variables|Default|GetRemoteOpenID))))

(event Custom|BunkerDoorOpened
  (Default|TaskCompleted (Variables|Default|GetTaskManagerRef) "OpenBunkerDoor" true true))

(event EventBeginPlay
  (bind _returnvalue (Actor|GetActorOfClass "/Game/TaskSystem/BP_TaskManager.BP_TaskManager_C"))
  (Variables|Default|SetTaskManagerRef _returnvalue)
  (EventDispatchers|AssignRemoteDoorOpen _returnvalue (delegate Custom|RemoteDoorOpen_Event)))

(fn ConstructionScript)