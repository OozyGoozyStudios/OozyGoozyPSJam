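; BP_BunkerDoor2 is an interactable bunker door built on a skeletal mesh that opens and closes on demand.
; The BunkerDoorOpened event plays the open montage, plays an opening sound at the door's location and disables the mesh collision.
; The CloseBunkerDoor event plays the close montage and restores query and physics collision, with no sound.
; Both collision changes happen immediately rather than waiting for the animation to finish.
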(event Custom|BunkerDoorOpened
  (Components|Animation|PlayAnimation (Variables|Default|GetSKM_BunkerDoor) "/Game/Interactables/BunkerDoor/BunkerOpen_Montage.BunkerOpen_Montage" false)
  (Audio|PlaySoundatLocation "/Game/Sounds/General_SFX/S_Bunker_Open.S_Bunker_Open" (Transformation|GetWorldLocation (Variables|Default|GetSKM_BunkerDoor)) "0, 0, 0" 1.0 1.0 0.0 0 0 0 0)
  (Collision|SetCollisionEnabled (Variables|Default|GetSKM_BunkerDoor) "NoCollision"))

(event Custom|CloseBunkerDoor
  (Components|Animation|PlayAnimation (Variables|Default|GetSKM_BunkerDoor) "/Game/Interactables/BunkerDoor/BunkerClose_Montage.BunkerClose_Montage" false)
  (Collision|SetCollisionEnabled (Variables|Default|GetSKM_BunkerDoor) "QueryAndPhysics"))

(fn ConstructionScript)