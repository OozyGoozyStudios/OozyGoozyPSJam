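; BP_KitchenDoor is an interactable kitchen door in the Old Brick House that triggers a one-time banging sound at the house's final door.
; It extends its parent's Interacted event, calling the parent logic on every interaction.
; On the first interaction only, it sets a HasBeenOpened flag, waits briefly, then finds BP_BrickHouseFinalDoor by class and plays the door-banging cue at that actor's location.
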(event EventBeginPlay
  (|CallParentFunction) ; This node is disabled and will not be called.\nDrag off pins to build functionality.
)

(event EventInteracted
  (|CallParentFunction)
  (if (not (Variables|Default|GetHasBeenOpened?))
    (Variables|Default|SetHasBeenOpened? true)
    (Utilities|FlowControl|Delay 1.5)
    (bind _returnvalue (Actor|GetActorOfClass "/Game/Interactables/Door/BP_BrickHouseFinalDoor.BP_BrickHouseFinalDoor_C"))
    (Audio|PlaySoundatLocation "/Game/Sounds/Spooky_Sounds/S_door_banging_Cue.S_door_banging_Cue" (Transformation|GetWorldLocation (Variables|/Game/Interactables/BP_ParentInteractable.BP_ParentInteractable_C|GetDefaultSceneRoot _returnvalue)) "0, 0, 0" 1.0 1.0 0.0 0 0 0 0)))

(fn ConstructionScript
  (|CallParentFunction))