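; BP_ParentInteractable is a base actor for task objects the first-person player can interact with once.
; Its OverlapBox reacts only to the BP_FirstPersonCharacter capsule, setting the character's NearInteractable flag on entry, then clearing it and removing the interaction widget on exit.
; The Interacted event sets HasBeenInteracted, after which both overlap handlers ignore the player.
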(event OnComponentBeginOverlap(OverlapBox)
  (params (OverlappedComponent :type Primitive%20Component%20Object%20Reference) (OtherActor :type Actor%20Object%20Reference) (OtherComp :type Primitive%20Component%20Object%20Reference) (OtherBodyIndex :type Integer) (bFromSweep :type Boolean) (SweepResult :type Hit%20Result%20Structure%20%28by%20ref%29))
  (if (not (Variables|Default|GetHasBeenInteracted?))
    (bind _asbp_first_person_character (Utilities|Casting|CastToBP_FirstPersonCharacter OtherActor))
    (if (== OtherComp (Variables|/Script/Engine.Character|GetCapsuleComponent _asbp_first_person_character))
      (Variables|/Game/FirstPerson/Blueprints/BP_FirstPersonCharacter.BP_FirstPersonCharacter_C|SetNearInteractable? _asbp_first_person_character true))))

(event OnComponentEndOverlap(OverlapBox)
  (params (OverlappedComponent :type Primitive%20Component%20Object%20Reference) (OtherActor :type Actor%20Object%20Reference) (OtherComp :type Primitive%20Component%20Object%20Reference) (OtherBodyIndex :type Integer))
  (if (not (Variables|Default|GetHasBeenInteracted?))
    (bind _asbp_first_person_character (Utilities|Casting|CastToBP_FirstPersonCharacter OtherActor))
    (if (== OtherComp (Variables|/Script/Engine.Character|GetCapsuleComponent _asbp_first_person_character))
      (Variables|/Game/FirstPerson/Blueprints/BP_FirstPersonCharacter.BP_FirstPersonCharacter_C|SetNearInteractable? _asbp_first_person_character false)
      (Default|RemoveInteractionWidget _asbp_first_person_character))))

(event Custom|Interacted
  (Variables|Default|SetHasBeenInteracted? true))

(fn ConstructionScript)