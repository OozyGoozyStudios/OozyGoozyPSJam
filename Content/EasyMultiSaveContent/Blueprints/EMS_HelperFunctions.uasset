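; Helper function Blueprint for Easy Multi Save that formats save dates and exports save slot thumbnail images.
; DateToString builds a year/month/day-hour:minute string, using DateStringPrefix to zero-pad single-digit values.
; SaveThumbnailImage gets the player pawn, or the controller as fallback, and checks its SceneCaptureComponent2D for the ScreenshotThumbnailCapture tag.
; It then captures the scene and exports the render target under the slot info's save game name.
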(fn DatetoString
  (params (InDateTime :type Date%20Time%20Structure))
  (bind (_year _month _day _hour _minute) (Math|DateTime|BreakDateTime InDateTime))
  (return (Utilities|String|BuildString(Integer) (Utilities|String|BuildString(Integer) (Utilities|String|BuildString(Integer) (Utilities|String|BuildString(Integer) (Utilities|String|BuildString(Integer) "" "" _year "/") (EasyMultiSave|TimeandDate|DateStringPrefix _month) _month "/") (EasyMultiSave|TimeandDate|DateStringPrefix _day) _day " - ") (EasyMultiSave|TimeandDate|DateStringPrefix _hour) _hour ":") (EasyMultiSave|TimeandDate|DateStringPrefix _minute) _minute)))

(fn DateStringPrefix
  (params (A :type Integer))
  (return (select (< A 10) "0" "")))

(fn SaveThumbnailImage
  (bind _returnvalue (Game|Player|GetPlayerPawn 0))
  (bind _returnvalue_2 (Game|GetPlayerController 0))
  (Utilities|FlowControl|Sequence
    (:then_0
      (Utilities|IsValid _returnvalue
        (:Is%20Valid
          (LocalVariables|SetTempActor _returnvalue))
        (:Is%20Not%20Valid
          (Utilities|IsValid _returnvalue_2
            (:Is%20Valid
              (LocalVariables|SetTempActor _returnvalue_2))))))
    (:then_1
      (Utilities|IsValid (LocalVariables|GetTempActor)
        (:Is%20Valid
          (if (Components|ComponentHasTag (Actor|GetComponentbyClass (LocalVariables|GetTempActor) "/Script/Engine.SceneCaptureComponent2D") "ScreenshotThumbnailCapture")
            (bind _output_get (LocalVariables|SetCaptureComp (Actor|GetComponentbyClass (LocalVariables|GetTempActor) "/Script/Engine.SceneCaptureComponent2D")))
            (Utilities|IsValid _output_get
              (:Is%20Valid
                (Rendering|SceneCapture|CaptureScene (LocalVariables|GetCaptureComp) :!class /Script/Engine.SceneCaptureComponent2D)
                (CallFunction|ExportSaveThumbnail 0 (Variables|/Script/Engine.SceneCaptureComponent2D|GetTextureTarget (LocalVariables|GetCaptureComp)) (.SaveGameName (CallFunction|GetSlotInfoSaveGame)))))))))))