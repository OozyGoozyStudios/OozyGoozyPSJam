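; BP_Snowfall is a snowfall effect actor whose particle component is tuned through Blueprint variables.
; The construction script pushes velocity range, spawn rate, box extent and lifetime range into the Snowfall component as named parameters, so the effect is configured at construction.
; The event graph holds only disabled placeholder events, so the Blueprint adds no runtime logic.
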(event EventBeginPlay)

(event Collision|EventActorBeginOverlap
  (params (OtherActor :type Actor%20Object%20Reference)))

(event EventTick
  (params (DeltaSeconds :type Float%20%28single-precision%29)))

(fn ConstructionScript
  (bind _snowfall (Variables|Default|GetSnowfall))
  (Effects|Components|ParticleSystem|SetFloatParameter _snowfall "MaxVelocity" (Variables|Default|GetMaxVelocity))
  (Effects|Components|ParticleSystem|SetFloatParameter _snowfall "MinVelocity" (Variables|Default|GetMinVelocity))
  (Effects|Components|ParticleSystem|SetFloatParameter _snowfall "SpawnRate" (Variables|Default|GetSpawnRate))
  (Effects|Components|ParticleSystem|SetVectorParameter _snowfall "BoxExtent" (Variables|Default|GetBoxExtent))
  (Effects|Components|ParticleSystem|SetFloatParameter _snowfall "LifetimeMin" (Variables|Default|GetMinLifetime))
  (Effects|Components|ParticleSystem|SetFloatParameter _snowfall "LifetimeMax" (Variables|Default|GetMaxLifetime)))