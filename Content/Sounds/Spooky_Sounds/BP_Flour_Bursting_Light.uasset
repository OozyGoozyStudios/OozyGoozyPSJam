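; BP_Flour_Bursting_Light is a light actor that can blow out on demand.
; Its BlowOut event calls PowerOff, spawns the NS_BlowoutSparks effect at the Scene component's world location and stops the Audio component.
; BeginPlay, overlap and Tick are disabled stubs, and the construction script only calls its parent, so nothing in this graph triggers the blowout itself.
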(event Custom|BlowOut
  (CallFunction|PowerOff)
  (Niagara|SpawnSystematLocation "/Game/MaterialsTexturesVFX/VFX/Blowout/NS_BlowoutSparks.NS_BlowoutSparks" (Transformation|GetWorldLocation (Variables|Default|GetScene)))
  (Audio|Components|Audio|Stop (Variables|Default|GetAudio)))

(event EventBeginPlay
  (|CallParentFunction) ; This node is disabled and will not be called.\nDrag off pins to build functionality.
)

(event Collision|EventActorBeginOverlap
  (params (OtherActor :type Actor%20Object%20Reference))
  (|CallParentFunction OtherActor) ; This node is disabled and will not be called.\nDrag off pins to build functionality.
)

(event EventTick
  (params (DeltaSeconds :type Float%20%28single-precision%29))
  (|CallParentFunction DeltaSeconds) ; This node is disabled and will not be called.\nDrag off pins to build functionality.
)

(fn ConstructionScript
  (|CallParentFunction))