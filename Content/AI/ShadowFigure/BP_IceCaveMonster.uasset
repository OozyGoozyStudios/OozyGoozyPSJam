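; BP_IceCaveMonster is a shadow figure monster for the ice cave that starts hidden and without collision.
; BeginPlay caches its ABP_ShadowMan anim instance, then calls MakeEnableDisabled, which toggles mesh visibility and switches capsule collision between physics-only and none.
; FacePlayer turns the capsule toward the first-person character and re-arms itself on a 0.1-second timer; nothing in this Blueprint starts it or sets the player reference.
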(event EventBeginPlay
  (bind _asabp_shadow_man (Utilities|Casting|CastToABP_ShadowMan (Components|SkeletalMesh|GetAnimInstance (Variables|Character|GetMesh)))
    (:then
      (Variables|Default|SetAs%20ABP%20Shadow%20Man _asabp_shadow_man))
    (:CastFailed
      _))
  (CallFunction|MakeEnableDisabled false))

(fn ConstructionScript)

(fn FacePlayer
  (bind _capsulecomponent (Variables|Collision|GetCapsuleComponent))
  (Transformation|SetWorldRotation _capsulecomponent (Math|Rotator|FindLookatRotation (Transformation|GetWorldLocation _capsulecomponent) (Transformation|GetWorldLocation (Variables|/Script/Engine.Character|GetCapsuleComponent (Variables|Default|GetAs%20BP%20First%20Person%20Character)))) false false)
  (Utilities|Time|SetTimerbyFunctionName 0 "FacePlayer" 0.1))

(fn MakeEnableDisabled
  (params (Enabled? :type Boolean))
  (if Enabled?
    (Rendering|SetVisibility (Variables|Character|GetMesh) true true)
    (Collision|SetCollisionEnabled (Variables|Collision|GetCapsuleComponent) "PhysicsOnly")
    (else
      (Rendering|SetVisibility (Variables|Character|GetMesh) false true)
      (Collision|SetCollisionEnabled (Variables|Collision|GetCapsuleComponent) "NoCollision"))))