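; Shadow figure actor that can watch the player and vanish when they get close.
; When stationary, it turns its capsule toward the first-person player through a self-rescheduling timer.
; If set to vanish, player overlap with its sphere starts a timeline that fades dynamic jeans, jacket and face materials plus Niagara shadow particles.
; The actor destroys itself after a short delay once the fade ends.
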(event OnComponentBeginOverlap(VanishSphere)
  (params (OverlappedComponent :type Primitive%20Component%20Object%20Reference) (OtherActor :type Actor%20Object%20Reference) (OtherComp :type Primitive%20Component%20Object%20Reference) (OtherBodyIndex :type Integer) (bFromSweep :type Boolean) (SweepResult :type Hit%20Result%20Structure%20%28by%20ref%29))
  (if (Variables|Default|GetVanishes?)
    (Utilities|Casting|CastToBP_FirstPersonCharacter OtherActor)
    (CallFunction|FadeOut)))

(event Custom|FadeOut
  (bind _opacitycurve (Timeline|TL_FadeOut PlayFromStart)
    (:Update
      (Rendering|Material|SetScalarParameterValue (Variables|Default|GetDMI_Jeans) "Opacity" _opacitycurve :!class /Script/Engine.MaterialInstanceDynamic)
      (Rendering|Material|SetScalarParameterValue (Variables|Default|GetDMI_Jacket) "Opacity" _opacitycurve :!class /Script/Engine.MaterialInstanceDynamic)
      (Rendering|Material|SetScalarParameterValue (Variables|Default|GetDMI_Face) "Opacity" _opacitycurve :!class /Script/Engine.MaterialInstanceDynamic)
      (Effects|Components|ParticleSystem|SetFloatParameter (Variables|Default|GetNS_Shadow) "SpawnRate" (* _opacitycurve 1e+01))
      (Effects|Components|ParticleSystem|SetFloatParameter (Variables|Default|GetNS_Shadow) "AlphaScale" _opacitycurve))
    (:Finished
      (Utilities|FlowControl|Delay 4.0)
      (Actor|DestroyActor))))

(event EventBeginPlay
  (CallFunction|SetupDMIs)
  (bind _asabp_shadow_man (Utilities|Casting|CastToABP_ShadowMan (Components|SkeletalMesh|GetAnimInstance (Variables|Character|GetMesh))))
  (Variables|Default|SetAs%20ABP%20Shadow%20Man _asabp_shadow_man)
  (bind _returnvalue (Actor|GetActorOfClass "/Game/FirstPerson/Blueprints/BP_FirstPersonCharacter.BP_FirstPersonCharacter_C"))
  (Variables|Default|SetAs%20BP%20First%20Person%20Character _returnvalue)
  (if (Variables|Default|GetStationary?)
    (CallFunction|FacePlayer)))

(fn ConstructionScript)

(fn SetupDMIs
  (bind _mesh (Variables|Character|GetMesh))
  (bind _mesh_2 (Variables|Character|GetMesh))
  (bind _returnvalue (Rendering|Material|CreateDynamicMaterialInstance _mesh 0 "/Game/AI/ShadowFigure/Textures/M_Jeans.M_Jeans" "None" :!class /Script/Engine.PrimitiveComponent))
  (bind _output_get (Variables|Default|SetDMI_Jeans _returnvalue))
  (Rendering|Material|SetMaterial _mesh 0 _output_get)
  (Rendering|Material|SetMaterial _mesh 2 _output_get)
  (Rendering|Material|SetMaterial _mesh 4 _output_get)
  (bind _returnvalue_2 (Rendering|Material|CreateDynamicMaterialInstance _mesh 1 "/Game/AI/ShadowFigure/Textures/M_Jacket.M_Jacket" "None" :!class /Script/Engine.PrimitiveComponent))
  (bind _output_get_2 (Variables|Default|SetDMI_Jacket _returnvalue_2))
  (Rendering|Material|SetMaterial (Variables|Character|GetMesh) 1 _output_get_2)
  (bind _returnvalue_3 (Rendering|Material|CreateDynamicMaterialInstance _mesh_2 3 "/Game/AI/ShadowFigure/Textures/M_Face.M_Face" "None" :!class /Script/Engine.PrimitiveComponent))
  (bind _output_get_3 (Variables|Default|SetDMI_Face _returnvalue_3))
  (Rendering|Material|SetMaterial _mesh_2 0 _output_get_3))

(fn FacePlayer
  (bind _capsulecomponent (Variables|Collision|GetCapsuleComponent))
  (Transformation|SetWorldRotation _capsulecomponent (Math|Rotator|FindLookatRotation (Transformation|GetWorldLocation _capsulecomponent) (Transformation|GetWorldLocation (Variables|/Script/Engine.Character|GetCapsuleComponent (Variables|Default|GetAs%20BP%20First%20Person%20Character)))) false false)
  (Utilities|Time|SetTimerbyFunctionName 0 "FacePlayer" 0.1))