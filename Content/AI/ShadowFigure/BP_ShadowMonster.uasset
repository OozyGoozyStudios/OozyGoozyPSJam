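; Shadow figure monster that fades away when the player gets close or when it receives an InFocus event.
; If stationary, it starts at a set opacity and re-aims at the player on a repeating timer.
; VanishSphere overlap, when vanishing is enabled, or InFocus runs a timeline that drives body material opacity and Niagara shadow particles, then destroys the actor after a delay.
; ReturnFocusCenter exposes the sphere's location as the focus point.
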(event OnComponentBeginOverlap(VanishSphere)
  (params (OverlappedComponent :type Primitive%20Component%20Object%20Reference) (OtherActor :type Actor%20Object%20Reference) (OtherComp :type Primitive%20Component%20Object%20Reference) (OtherBodyIndex :type Integer) (bFromSweep :type Boolean) (SweepResult :type Hit%20Result%20Structure%20%28by%20ref%29))
  (if (Variables|Default|GetVanishes?)
    (Utilities|Casting|CastToBP_FirstPersonCharacter OtherActor)
    (CallFunction|FadeOut)))

(event Custom|FadeOut
  (if (not (Variables|Default|GetIsFadingOut?))
    (bind _opacitycurve (Timeline|TL_FadeOut PlayFromStart)
      (:Update
        (Rendering|Material|SetScalarParameterValue (Variables|Default|GetDMI_MonsterBody) "Opacity" _opacitycurve :!class /Script/Engine.MaterialInstanceDynamic)
        (Effects|Components|ParticleSystem|SetFloatParameter (Variables|Default|GetNS_Shadow) "SpawnRate" (* _opacitycurve 1e+01))
        (Effects|Components|ParticleSystem|SetFloatParameter (Variables|Default|GetNS_Shadow) "AlphaScale" _opacitycurve)
        (Variables|Default|SetIsFadingOut? true))
      (:Finished
        (Utilities|FlowControl|Delay 3.0)
        (Actor|DestroyActor)))))

(event EventBeginPlay
  (bind _asabp_shadow_man (Utilities|Casting|CastToABP_ShadowMan (Components|SkeletalMesh|GetAnimInstance (Variables|Character|GetMesh))))
  (Variables|Default|SetAs%20ABP%20Shadow%20Man _asabp_shadow_man)
  (Components|Sphere|SetSphereRadius (Variables|Default|GetVanishSphere) (Variables|Default|GetVanishRadius) true)
  (bind _returnvalue (Actor|GetActorOfClass "/Game/FirstPerson/Blueprints/BP_FirstPersonCharacter.BP_FirstPersonCharacter_C"))
  (Variables|Default|SetAs%20BP%20First%20Person%20Character _returnvalue)
  (if (Variables|Default|GetStationary?)
    (CallFunction|FacePlayer)
    (Rendering|Material|SetScalarParameterValue (Variables|Default|GetDMI_MonsterBody) "Opacity" (Variables|Default|GetStartingOpacity) :!class /Script/Engine.MaterialInstanceDynamic)))

(event EventInFocus
  (CallFunction|FadeOut))

(fn ConstructionScript
  (CallFunction|SetupDMIs))

(fn SetupDMIs
  (bind _mesh (Variables|Character|GetMesh))
  (bind _returnvalue (Rendering|Material|CreateDynamicMaterialInstance _mesh 2 "/Game/AI/Jessica/Materials/ShadowMats/Shadow_Body1.Shadow_Body1" "None" :!class /Script/Engine.PrimitiveComponent))
  (Variables|Default|SetDMI_MonsterBody _returnvalue)
  (Rendering|Material|SetMaterial _mesh 2 (Variables|Default|GetDMI_MonsterBody)))

(fn FacePlayer
  (bind _capsulecomponent (Variables|Collision|GetCapsuleComponent))
  (Transformation|SetWorldRotation _capsulecomponent (Math|Rotator|FindLookatRotation (Transformation|GetWorldLocation _capsulecomponent) (Transformation|GetWorldLocation (Variables|/Script/Engine.Character|GetCapsuleComponent (Variables|Default|GetAs%20BP%20First%20Person%20Character)))) false false)
  (Utilities|Time|SetTimerbyFunctionName 0 "FacePlayer" 0.1))

(fn ReturnFocusCenter
  (return (Transformation|GetWorldLocation (Variables|Default|GetVanishSphere))))