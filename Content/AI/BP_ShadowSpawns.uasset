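; BP_ShadowSpawns is a trigger volume that spawns a BP_ShadowMan at its SpawnLocation when the first-person player overlaps it.
; An optional prerequisite task gates the spawn by checking its row name against the player's task list widget's completed tasks.
; Exposed variables control one-shot or repeat triggering and pass stationary and vanish behavior to the shadow.
; An optional lifetime timer fades out the last spawned shadow.
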(event OnComponentBeginOverlap(BoxTrigger)
  (params (OverlappedComponent :type Primitive%20Component%20Object%20Reference) (OtherActor :type Actor%20Object%20Reference) (OtherComp :type Primitive%20Component%20Object%20Reference) (OtherBodyIndex :type Integer) (bFromSweep :type Boolean) (SweepResult :type Hit%20Result%20Structure%20%28by%20ref%29))
  (bind _asbp_first_person_character (Utilities|Casting|CastToBP_FirstPersonCharacter OtherActor))
  (if (Variables|Default|GetDoesOnce?)
    (if (not (Variables|Default|GetHasSpawned?))
      (bind _prerequisitetask (Variables|Default|GetPrerequisiteTask :!label _label)
        (:then
          (if (Utilities|Array|ContainsItem (Variables|/Game/TaskSystem/WBP_TaskList.WBP_TaskList_C|GetCompletedTasks (Variables|/Game/FirstPerson/Blueprints/BP_FirstPersonCharacter.BP_FirstPersonCharacter_C|GetWBP_TaskList _asbp_first_person_character)) (.TaskRowName (Utilities|GetClassDefaults _prerequisitetask)))
            (Variables|Default|SetHasCompletedTask? true)
            (bind _returnvalue (Game|SpawnActorfromClass "/Game/AI/ShadowFigure/BP_ShadowMan.BP_ShadowMan_C" (Transformation|GetWorldTransform (Variables|Default|GetSpawnLocation)) "Undefined" "MultiplyWithRoot" 0 (Variables|Default|GetSummonStationary?) (Variables|Default|GetSummonVanishes?) (Variables|Default|GetVanishRadius) 0 :!label _label_2))
            (Variables|Default|SetSpawnedShadow _returnvalue)
            (Variables|Default|SetHasSpawned? true)
            (if (Variables|Default|GetUseDuration?)
              (Utilities|Time|SetTimerbyEvent (delegate Custom|DespawnSummon) (Variables|Default|GetSummonLifetime)))))
        (:else
          (goto _label_2))))
    (else
      (goto _label))))

(event Custom|DespawnSummon
  (bind _spawnedshadow (Variables|Default|GetSpawnedShadow)
    (:then
      (Default|FadeOut _spawnedshadow))
    (:else)))

(event EventBeginPlay)

(event Collision|EventActorBeginOverlap
  (params (OtherActor :type Actor%20Object%20Reference)))

(event EventTick
  (params (DeltaSeconds :type Float%20%28single-precision%29)))

(fn ConstructionScript)