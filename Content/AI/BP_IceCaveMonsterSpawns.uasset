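; Spawn point actor that creates a stationary BP_IceCaveMonster slightly above its SpawnLocation when SpawnMonster is called.
; It marks itself as spawned, optionally plays a sound at that location, and can start a lifetime timer for DespawnSummon.
; DespawnSummon fades out SpawnedShadow if valid, but SpawnMonster sets that reference to None, so the new monster is not faded by it.
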(event Custom|DespawnSummon
  (bind _spawnedshadow (Variables|Default|GetSpawnedShadow)
    (:then
      (Default|FadeOut _spawnedshadow))
    (:else)))

(event Custom|SpawnMonster
  (bind _spawnlocation (Variables|Default|GetSpawnLocation))
  (bind _returnvalue (Transformation|GetWorldTransform _spawnlocation))
  (bind (_x _y _z) (Math|Vector|BreakVector (.location _returnvalue)))
  (Game|SpawnActorfromClass "/Game/AI/ShadowFigure/BP_IceCaveMonster.BP_IceCaveMonster_C" (Math|Transform|MakeTransform (Math|Vector|MakeVector _x _y (+ _z 1e+02)) (.rotation _returnvalue) "1.000000,1.000000,1.000000") "AlwaysSpawn" "MultiplyWithRoot" 0 true 0)
  (Variables|Default|SetSpawnedShadow 0)
  (Variables|Default|SetHasSpawned? true)
  (Utilities|FlowControl|Sequence
    (:then_0
      (if (Variables|Default|GetPlaySpawnSound?)
        (bind _spawnsoundtoplay (Variables|Default|GetSpawnSoundToPlay)
          (:then
            (Audio|PlaySoundatLocation _spawnsoundtoplay (.location (Transformation|GetWorldTransform (Variables|Default|GetSpawnLocation))) "0, 0, 0" 3.0 1.0 0.0 "/Game/Sounds/SA_TapeRecorder.SA_TapeRecorder" 0 0 0))
          (:else))))
    (:then_1
      (if (Variables|Default|GetUseDuration?)
        (Utilities|Time|SetTimerbyEvent (delegate Custom|DespawnSummon) (Variables|Default|GetSummonLifetime))))))

(event EventBeginPlay)

(event Collision|EventActorBeginOverlap
  (params (OtherActor :type Actor%20Object%20Reference)))

(event EventTick
  (params (DeltaSeconds :type Float%20%28single-precision%29)))

(fn ConstructionScript)