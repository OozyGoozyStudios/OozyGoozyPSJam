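; BP_JessicaAntarctica is the Jessica monster for Antarctica, which watches for the first-person player and sends them back to Greenland on sight.
; From BeginPlay, PeepDoorway sphere-traces from the EyeSocket to the player on a 0.2-second timer until it hits them.
; A hit calls the still-empty Scare event, then ReturnToGreenland on the player after a short delay.
; A self-repeating CrawlForward timer function nudges the capsule forward, but nothing here starts it.
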(event Custom|Scare
  ;[1 1 1] Put logic hear to rotate monster head and open mouth brefore cutting to black
)

(event Custom|ReturnPlayerHome
  (Utilities|FlowControl|Delay 0.5)
  (Default|ReturntoGreenland (Variables|Default|GetPlayerRef)))

(event EventBeginPlay
  (bind _returnvalue (Actor|GetActorOfClass "/Game/FirstPerson/Blueprints/BP_FirstPersonCharacter.BP_FirstPersonCharacter_C"))
  (Variables|Default|SetPlayerRef _returnvalue)
  (CallFunction|PeepDoorway))

(fn ConstructionScript)

(fn PeepDoorway
  (bind _playerref (Variables|Default|GetPlayerRef)
    (:then
      (bind _outhit (Collision|SphereTraceByChannel (Transformation|GetSocketLocation (Variables|Character|GetMesh) "EyeSocket") (Transformation|GetWorldLocation (Variables|/Script/Engine.Character|GetCapsuleComponent _playerref)) 25.0 "TraceTypeQuery2" false 0 "None" true "(R=1.000000,G=0.000000,B=0.000000,A=1.000000)" "(R=0.000000,G=1.000000,B=0.000000,A=1.000000)" 1.0))
      (if (== (.HitActor (Collision|BreakHitResult _outhit)) (Variables|Default|GetPlayerRef))
        (Development|PrintString "Hit Player!")
        (CallFunction|Scare)
        (CallFunction|ReturnPlayerHome)
        (return)
        (else
          (Utilities|Time|SetTimerbyFunctionName 0 "PeepDoorway" 0.2))))
    (:else
      (Development|PrintString "PlayerRef Is Not Valid --PeepDoorway-- BP_JessicaAntarctica"))))

(fn CrawlForward
  (bind _capsulecomponent (Variables|Collision|GetCapsuleComponent))
  (Transformation|SetWorldLocation _capsulecomponent (+ (Transformation|GetWorldLocation _capsulecomponent) (* (Math|Vector|GetForwardVector _capsulecomponent) 6.0)) false false)
  (Utilities|Time|SetTimerbyFunctionName 0 "Crawl Forward" 0.01))