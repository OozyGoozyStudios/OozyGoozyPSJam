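; BP_StaticMonsterSpawn is a static monster sighting, visible on BeginPlay only if the task manager lists GoToBed as completed.
; The first InFocus event flags the player character as having seen the monster and awards the WhatWasThat achievement, with delayed, capped retries if caching achievements fails.
; ReturnFocusCenter supplies the Scene component's location as the focus point, and Despawn destroys the actor.
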(event Custom|Despawn
  (Actor|DestroyActor))

(event EventBeginPlay
  (bind _returnvalue (Actor|GetActorOfClass "/Game/TaskSystem/BP_TaskManager.BP_TaskManager_C"))
  (Rendering|SetVisibility (Variables|Default|GetStaticMesh) (Utilities|Array|ContainsItem (Variables|/Game/TaskSystem/BP_TaskManager.BP_TaskManager_C|GetTasksCompleted _returnvalue) "GoToBed") true))

(event EventInFocus
  (bind _returnvalue (Game|GetPlayerController 0))
  (if (not (Variables|Default|GetHasBeenFocused?))
    (Variables|Default|SetHasBeenFocused? true)
    (bind _asbp_first_person_character (Utilities|Casting|CastToBP_FirstPersonCharacter (Game|GetPlayerCharacter 0))
      (:then
        (Variables|/Game/FirstPerson/Blueprints/BP_FirstPersonCharacter.BP_FirstPersonCharacter_C|SetHasSeenTheMonster? _asbp_first_person_character true))
      (:CastFailed
        _))
    (|CacheAchievements _returnvalue :!label _label
      (:OnSuccess
        (|WriteAchievementProgress _returnvalue "WhatWasThat" 1.0
          (:OnSuccess
            (Development|PrintString "Achievement Write Success!" true true "(R=0.000000,G=1.000000,B=0.107318,A=1.000000)" 5.0))
          (:OnFailure
            (Development|PrintString "Achievement Write Failed!" true true "(R=1.000000,G=0.000000,B=0.034709,A=1.000000)" 5.0))))
      (:OnFailure
        (Utilities|FlowControl|Delay 0.2)
        (Utilities|FlowControl|DoN 5
          (:Exit
            (goto _label)))))))

(fn ConstructionScript)

(fn ComponentstoSave
  (return 0))

(fn ReturnFocusCenter
  (return (Transformation|GetWorldLocation (Variables|Default|GetScene))))