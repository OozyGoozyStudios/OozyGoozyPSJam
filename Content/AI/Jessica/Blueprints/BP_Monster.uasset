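; BP_Monster is the hostile AI monster that makes a scripted entrance, chases the player and attacks with a swipe.
; Being seen or a door trigger, whichever fires first, starts the timed AnimState entrance and capsule move, then a timer-looped check that opens overlapping doors.
; Sphere overlap drives look-at and AIMoveTo chasing, while a toggled hand hitbox deals hits.
; Shadow dynamic materials, an elevator-button fade and a datamosh toggle handle its visuals.
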(event OnComponentEndOverlap(Sphere)
  (params (OverlappedComponent :type Primitive%20Component%20Object%20Reference) (OtherActor :type Actor%20Object%20Reference) (OtherComp :type Primitive%20Component%20Object%20Reference) (OtherBodyIndex :type Integer))
  ;[1 1 1] Overlap events
  (Utilities|Casting|CastToBP_FirstPersonCharacter OtherActor)
  (Variables|Default|SetIsLookAt false))

(event OnComponentBeginOverlap(Sphere)
  (params (OverlappedComponent :type Primitive%20Component%20Object%20Reference) (OtherActor :type Actor%20Object%20Reference) (OtherComp :type Primitive%20Component%20Object%20Reference) (OtherBodyIndex :type Integer) (bFromSweep :type Boolean) (SweepResult :type Hit%20Result%20Structure%20%28by%20ref%29))
  ;[1 1 1] Overlap events
  (Utilities|Casting|CastToBP_FirstPersonCharacter OtherActor)
  (Variables|Default|SetIsLookAt true))

(event OnComponentBeginOverlap(DoorOpeningCapsule)
  (params (OverlappedComponent :type Primitive%20Component%20Object%20Reference) (OtherActor :type Actor%20Object%20Reference) (OtherComp :type Primitive%20Component%20Object%20Reference) (OtherBodyIndex :type Integer) (bFromSweep :type Boolean) (SweepResult :type Hit%20Result%20Structure%20%28by%20ref%29))
  ;[1 1 1] Overlap events
  (bind _ismonsterreturn_ (Class|BPIDoors|GetIsMonsterOpen?(Message) OtherActor))
  (if _ismonsterreturn_
    (Class|BPIDoors|MakeDoorOpen(Message) OtherActor true)))

(event OnComponentBeginOverlap(HandHitbox)
  (params (OverlappedComponent :type Primitive%20Component%20Object%20Reference) (OtherActor :type Actor%20Object%20Reference) (OtherComp :type Primitive%20Component%20Object%20Reference) (OtherBodyIndex :type Integer) (bFromSweep :type Boolean) (SweepResult :type Hit%20Result%20Structure%20%28by%20ref%29))
  (bind _as_bp_first_person_character (Variables|Default|GetAs%20BP%20First%20Person%20Character))
  (Utilities|Casting|CastToBP_FirstPersonCharacter OtherActor)
  (Utilities|FlowControl|DoOnce false :!label _label
    (:Completed
      (Default|GetHitbyMonster _as_bp_first_person_character)
      (Utilities|FlowControl|Delay 1.0)
      (if (not (Variables|/Game/FirstPerson/Blueprints/BP_FirstPersonCharacter.BP_FirstPersonCharacter_C|GetIsDead? _as_bp_first_person_character))
        (goto _label Reset)))))

(event Custom|FollowPlayer
  ;[1 1 1] movement
  (if (Variables|Default|GetIsSeeingPlayer)
    (AI|AIMoveTo self "0, 0, 0" (Game|GetPlayerCharacter 0) 1e+02 false
      (:OnSuccess
        (Utilities|FlowControl|DoOnce false :!label _label
          (:Completed
            (Animation|Montage|PlayMontage (Variables|Character|GetMesh) "/Game/AI/Jessica/Anims/Monster_AttackSwipe_Montage.Monster_AttackSwipe_Montage"
              (:OnCompleted
                (goto _label Reset)))))))))

(event Custom|Spawn%20event
  (bind _capsulecomponent (Variables|Collision|GetCapsuleComponent))
  ;[1 1 1] Spawn/Scripted sequence
  (Utilities|FlowControl|Sequence
    (:then_0
      (bind _asbp_first_person_character (Utilities|Casting|CastToBP_FirstPersonCharacter (Game|GetPlayerCharacter 0)))
      (Variables|Default|SetAs%20BP%20First%20Person%20Character _asbp_first_person_character)
      (bind _returnvalue (Actor|GetActorOfClass "/Game/AI/Jessica/Blueprints/BP_StaticMonsterSpawn.BP_StaticMonsterSpawn_C"))
      (Default|Despawn _returnvalue)
      (Collision|SetCollisionEnabled (Variables|Default|GetHandHitbox) "NoCollision"))
    (:then_1
      (Audio|PlaySoundatLocation "/Game/AI/Jessica/sounds/M_intro.M_intro" (Transformation|GetWorldLocation _capsulecomponent) "0, 0, 0" 1.0 1.0 0.0 0 0 (Components|GetOwner _capsulecomponent) 0))))

(event Custom|TriggerMovement
  ;[1 1 1] Spawn/Scripted sequence
  (Utilities|FlowControl|Delay 0.2)
  (Variables|Default|SetAnimState 1.0)
  (Utilities|FlowControl|Delay 0.8666)
  (Variables|Default|SetAnimState 2.0)
  (Utilities|FlowControl|Delay 0.76666)
  (Components|MoveComponentTo (Variables|Collision|GetCapsuleComponent) "-3600.252862,6986.107220,61.586971" "0.000000,-90.000000,0.000000" false false 0.55 false)
  (Variables|Default|SetAnimState 3.0)
  (Utilities|FlowControl|Delay 1.5)
  (bind _returnvalue (Actor|GetActorOfClass "/Game/FirstPerson/Blueprints/BP_FirstPersonCharacter.BP_FirstPersonCharacter_C"))
  (Default|CreateSprintTutorial _returnvalue)
  (CallFunction|CheckOverlappingDoor))

(event Custom|Door%20Trigger
  ;[1 1 1] Monster Focus Triggers
  (if (not (Variables|Default|GetSightTriggered))
    (Variables|Default|SetDoorTriggered true)
    (Utilities|FlowControl|DoOnce false
      (:Completed
        (CallFunction|TriggerMovement)))))

(event Custom|SpawnHitbox
  (Collision|SetCollisionEnabled (Variables|Default|GetHandHitbox) "QueryOnly"))

(event Custom|DespawnHitbox
  (Collision|SetCollisionEnabled (Variables|Default|GetHandHitbox) "NoCollision"))

(event Custom|ToggleDatamosh
  (params (Active? :type Boolean))
  (Variables|Default|SetDatamoshActive? Active?)
  (Class|DatamoshLibrary|ToggleDatamosh Active?)
  (if Active?
    (Class|DatamoshLibrary|SetDatamoshNoise 1)
    (Rendering|SetRenderCustomDepth (Variables|Character|GetMesh) true)
    (Class|DatamoshLibrary|SetDatamoshFactor 0.93)))

(event Custom|ElevatorButtonsPressed
  (CallFunction|MakeShadowMaterials)
  (bind _fadeaway (Timeline|FadeAwayOpacity Play)
    (:Update
      (Rendering|Material|SetScalarParameterValue (Variables|Materials|GetDMI_ShadowBody) "Opacity" _fadeaway :!class /Script/Engine.MaterialInstanceDynamic))))

(event EventBeginPlay
  (bind _returnvalue (Actor|GetActorOfClass "/Game/LevelPrototyping/Blueprints/Elevator/BP_ElevatorButtons.BP_ElevatorButtons_C"))
  (EventDispatchers|AssignButtonsPressed _returnvalue (delegate Custom|ElevatorButtonsPressed)))

(event EventInFocus
  ;[1 1 1] Monster Focus Triggers
  (if (not (Variables|Default|GetDoorTriggered))
    (Variables|Default|SetSightTriggered true)
    (Utilities|FlowControl|DoOnce false
      (:Completed
        (CallFunction|TriggerMovement)))))

(event EventOutFocus
  ;[1 1 1] light beam debug
)

(event EventTick
  (params (DeltaSeconds :type Float%20%28single-precision%29))
  ;[1 1 1] targeting
  (if (Variables|Default|GetIsLookAt)
    (Utilities|FlowControl|Sequence
      (:then_0
        (bind _output_get (Variables|Default|SetIsSeeingPlayer true))
        (if (and _output_get (== (Variables|Default|GetAnimState) 3.0))
          (CallFunction|FollowPlayer)))
      (:then_1
        (bind _as_bp_first_person_character (Variables|Default|GetAs%20BP%20First%20Person%20Character)
          (:then
            (Variables|Default|SetLookAtLocation (Transformation|GetWorldLocation (Variables|/Game/FirstPerson/Blueprints/BP_FirstPersonCharacter.BP_FirstPersonCharacter_C|GetFadeToBlackPlane _as_bp_first_person_character))))
          (:else))))))

(fn ConstructionScript
  (Components|Activation|SetAutoActivate (Variables|Default|GetNS_ShadowMonsterClouds) (Variables|Materials|GetIsShadow?))
  (if (Variables|Materials|GetIsShadow?)
    (bind _returnvalue (Rendering|Material|CreateDynamicMaterialInstance "/Game/AI/Jessica/Materials/ShadowMats/Shadow_Eyes1.Shadow_Eyes1" "None" "None" :!class /Script/Engine.KismetMaterialLibrary))
    (bind _output_get (Variables|Materials|SetDMI_ShadowEyes _returnvalue))
    (Utilities|Array|Add (Variables|Materials|GetShadowDMIs) _output_get)
    (bind _returnvalue_2 (Rendering|Material|CreateDynamicMaterialInstance "/Game/AI/Jessica/Materials/ShadowMats/Shadow_Teeth1.Shadow_Teeth1" "None" "None" :!class /Script/Engine.KismetMaterialLibrary))
    (bind _output_get_2 (Variables|Materials|SetDMI_ShadowTeeth _returnvalue_2))
    (Utilities|Array|Add (Variables|Materials|GetShadowDMIs) _output_get_2)
    (bind _returnvalue_3 (Rendering|Material|CreateDynamicMaterialInstance "/Game/AI/Jessica/Materials/ShadowMats/Shadow_Body1.Shadow_Body1" "None" "None" :!class /Script/Engine.KismetMaterialLibrary))
    (bind _output_get_3 (Variables|Materials|SetDMI_ShadowBody _returnvalue_3))
    (Utilities|Array|Add (Variables|Materials|GetShadowDMIs) _output_get_3)
    (Rendering|Material|SetMaterial (Variables|Character|GetMesh) 0 (Variables|Materials|GetDMI_ShadowEyes))
    (Rendering|Material|SetMaterial (Variables|Character|GetMesh) 1 (Variables|Materials|GetDMI_ShadowTeeth))
    (Rendering|Material|SetMaterial (Variables|Character|GetMesh) 2 (Variables|Materials|GetDMI_ShadowBody))
    (for _array_element (Variables|Materials|GetShadowDMIs)
      (Rendering|Material|SetScalarParameterValue _array_element "Opacity" 0.7 :!class /Script/Engine.MaterialInstanceDynamic))
    (else
      (Rendering|Material|SetMaterial (Variables|Character|GetMesh) 0 "/Game/AI/Jessica/Materials/RegularMats/Monster_Eyes.Monster_Eyes")
      (Rendering|Material|SetMaterial (Variables|Character|GetMesh) 1 "/Game/AI/Jessica/Materials/RegularMats/Monster_Teeth.Monster_Teeth")
      (Rendering|Material|SetMaterial (Variables|Character|GetMesh) 2 "/Game/AI/Jessica/Materials/RegularMats/Monster_Body.Monster_Body"))))

(fn CheckOverlappingDoor
  (for _array_element (Collision|GetOverlappingActors (Variables|Default|GetDoorOpeningCapsule) "/Game/Interactables/Door/BP_Door.BP_Door_C" :!class /Script/Engine.PrimitiveComponent)
    (bind _dooropen_ (Class|BPIDoors|GetDoorCurrentState(Message) _array_element))
    (if (not _dooropen_)
      (Class|BPIDoors|MakeDoorOpen(Message) _array_element true)))
  (Utilities|Time|SetTimerbyFunctionName 0 "Check Overlapping Door" 0.5))

(fn MakeShadowMaterials
  (bind _returnvalue (Rendering|Material|CreateDynamicMaterialInstance "/Game/AI/Jessica/Materials/ShadowMats/Shadow_Eyes1.Shadow_Eyes1" "None" "None" :!class /Script/Engine.KismetMaterialLibrary))
  (bind _output_get (Variables|Materials|SetDMI_ShadowEyes _returnvalue))
  (Utilities|Array|Add (Variables|Materials|GetShadowDMIs) _output_get)
  (bind _returnvalue_2 (Rendering|Material|CreateDynamicMaterialInstance "/Game/AI/Jessica/Materials/ShadowMats/Shadow_Teeth1.Shadow_Teeth1" "None" "None" :!class /Script/Engine.KismetMaterialLibrary))
  (bind _output_get_2 (Variables|Materials|SetDMI_ShadowTeeth _returnvalue_2))
  (Utilities|Array|Add (Variables|Materials|GetShadowDMIs) _output_get_2)
  (bind _returnvalue_3 (Rendering|Material|CreateDynamicMaterialInstance "/Game/AI/Jessica/Materials/ShadowMats/Shadow_Body1.Shadow_Body1" "None" "None" :!class /Script/Engine.KismetMaterialLibrary))
  (bind _output_get_3 (Variables|Materials|SetDMI_ShadowBody _returnvalue_3))
  (Utilities|Array|Add (Variables|Materials|GetShadowDMIs) _output_get_3)
  (Rendering|Material|SetMaterial (Variables|Character|GetMesh) 0 (Variables|Materials|GetDMI_ShadowEyes))
  (Rendering|Material|SetMaterial (Variables|Character|GetMesh) 1 (Variables|Materials|GetDMI_ShadowTeeth))
  (Rendering|Material|SetMaterial (Variables|Character|GetMesh) 2 (Variables|Materials|GetDMI_ShadowBody))
  (for _array_element (Variables|Materials|GetShadowDMIs)
    (Rendering|Material|SetScalarParameterValue _array_element "Opacity" 1.0 :!class /Script/Engine.MaterialInstanceDynamic)))

(fn ReturnFocusCenter
  (return (Transformation|GetWorldLocation (Variables|Default|GetFocusCenter))))