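; BP_IndustrialLight_01 is an industrial light prop for the Nuclear Launch Bunker environment, configured entirely in the construction script.
; The Lit flag sets the light component's intensity to LightIntensity or zero and swaps the mesh material between lit and unlit instances.
; A DebugCastShadows flag controls whether the light casts shadows.
; The event graph holds only disabled placeholder events, so the Blueprint has no runtime logic.
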(event EventBeginPlay)

(event Collision|EventActorBeginOverlap
  (params (OtherActor :type Actor%20Object%20Reference)))

(event EventTick
  (params (DeltaSeconds :type Float%20%28single-precision%29)))

(fn ConstructionScript
  (bind _lit (Variables|Default|GetLit))
  (bind _staticmeshcomponent0 (Variables|Default|GetStaticMeshComponent0))
  (bind _lightintensity (Variables|Default|GetLightIntensity))
  (Rendering|Components|Light|SetCastShadows (Variables|Default|GetLightComponent0) (Variables|Default|Get%28Debug%29%20Cast%20Shadows))
  (if _lit
    (Variables|Default|SetLightInt _lightintensity)
    (else
      (Variables|Default|SetLightInt (* _lightintensity 0.0))))
  (Rendering|Components|Light|SetIntensity (Variables|Default|GetLightComponent0) (Variables|Default|GetLightInt))
  (if _lit
    (Rendering|Material|SetMaterial _staticmeshcomponent0 0 "/Game/NuclearLaunchBunker/Assets/Props/Materials/MI_IndustrialLight_01_Lit.MI_IndustrialLight_01_Lit")
    (else
      (Rendering|Material|SetMaterial _staticmeshcomponent0 0 "/Game/NuclearLaunchBunker/Assets/Props/Materials/MI_IndustrialLight_01.MI_IndustrialLight_01"))))